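; Ship-builder part Blueprint for cuboid pieces, providing their build slots and overlap collision.
; On BeginPlay it generates two horizontal build-slot sets when the ship-builder game mode is valid, then creates collision and adds tags.
; A query-only overlap box is attached to the mesh, positioned and sized from slot counts, plate height and GameInstance grid spacing.
; Its extents fall just short of the full grid footprint.
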(event EventBeginPlay
  ;[1 1 1] BEGIN play
  (|CallParentFunction)
  (Utilities|IsValid (Variables|Default|GetShipBuilderGameMode)
    (:Is%20Valid
      (CallFunction|GenerateBuildSlots))
    (:Is%20Not%20Valid
      _))
  (CallFunction|GenerateBoxCollision)
  (CallFunction|AddTags))

(event Collision|EventActorBeginOverlap
  (params (OtherActor :type Actor%20Object%20Reference)))

(event EventTick
  (params (DeltaSeconds :type Float%20%28single-precision%29))
  (|CallParentFunction DeltaSeconds) ; This node is disabled and will not be called.\nDrag off pins to build functionality.
)

(fn ConstructionScript
  (|CallParentFunction))

(fn GenerateBoxCollision
  (bind _gameinstance (Variables|Default|GetGameInstance))
  (bind _returnvalue (AddComponent|AddBoxComponent true (Math|Transform|MakeTransform "0, 0, 0")))
  (bind _output_get (Variables|Default|SetCollisionBox _returnvalue))
  (Transformation|AttachComponentToComponent _output_get (Variables|Default|GetStaticMesh) "None" "KeepRelative" "KeepRelative" "KeepRelative" true)
  (Transformation|SetRelativeLocation _returnvalue (- (Variables|Default|GetRelative%20Euclidean%20Origin) (Math|Vector|MakeVector (* (Variables|/Game/Blueprints/AllLevels/BP_GameInstance.BP_GameInstance_C|GetBuild%20Distance%20X _gameinstance) (/ (Math|Conversions|ToFloat(Integer) (- (Variables|Default|GetSlots%20X) 1)) 2.0)) (* (Variables|/Game/Blueprints/AllLevels/BP_GameInstance.BP_GameInstance_C|GetBuild%20Distance%20Y _gameinstance) (/ (Math|Conversions|ToFloat(Integer) (- (Variables|Default|GetSlots%20Y) 1)) 2.0)) (* (Variables|/Game/Blueprints/AllLevels/BP_GameInstance.BP_GameInstance_C|GetBuild%20Distance%20Z _gameinstance) (/ (Math|Conversions|ToFloat(Integer) (Variables|Default|GetPlate%20Height)) -2.0)))) false false)
  (Components|Box|SetBoxExtent _returnvalue (* (Math|Vector|MakeVector (* (Variables|Default|GetSlots%20X) (Variables|/Game/Blueprints/AllLevels/BP_GameInstance.BP_GameInstance_C|GetBuild%20Distance%20X _gameinstance)) (* (Variables|Default|GetSlots%20Y) (Variables|/Game/Blueprints/AllLevels/BP_GameInstance.BP_GameInstance_C|GetBuild%20Distance%20Y _gameinstance)) (* (Variables|Default|GetPlate%20Height) (Variables|/Game/Blueprints/AllLevels/BP_GameInstance.BP_GameInstance_C|GetBuild%20Distance%20Z _gameinstance))) 0.49) true)
  (Collision|SetCollisionEnabled _returnvalue "QueryOnly")
  (Variables|/Script/Engine.PrimitiveComponent|SetbGenerateOverlapEvents _returnvalue true)
  (return true))

(fn GenerateBuildSlots
  (CallFunction|AddBuildSlotsHorizontal "NewEnumerator0")
  (CallFunction|AddBuildSlotsHorizontal "NewEnumerator1"))