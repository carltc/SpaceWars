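; Ship builder part actor that snaps to others through male and female BP_ConnectionSlot child actors, laid out on grids scaled by GameInstance build distances.
; Functions cycle highlighted slots, find the nearest free slot and link slots whose spheres overlap.
; Collision box overlaps swap in an invalid material, while custom depth stencils mark hovered, selected and moving states.
; Destroying any part removes every selected-slot visual in the world.
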(event EventDestroyed
  ;[1 1 1] On DESTROY
  (CallFunction|SPDestroyConnectionSlotVisuals))

(event EventTick
  (params (DeltaSeconds :type Float%20%28single-precision%29))
  ;[1 1 1] EVENT tick
)

(fn ConstructionScript
  (bind _material (Variables|Appearance|GetMaterial))
  ;[1 1 1] SET clickable-ness of actor
  (Variables|/Game/Blueprints/ShipBuilder/BP_ClickableShipPartComponent.BP_ClickableShipPartComponent_C|SetIsClickable (Variables|Default|GetBP_ClickableShipPartComponent) (Variables|Selecting|GetIsClickable))
  ;[1 1 1] SET game instance
  (bind _asbp_game_instance (Utilities|Casting|CastToBP_GameInstance (Game|GetGameInstance)))
  (Variables|Game|SetGameInstance _asbp_game_instance)
  ;[1 1 1] SET game mode
  (bind _asbp_ship_builder_game_mode (Utilities|Casting|CastToBP_ShipBuilderGameMode (Game|GetGameMode))
    (:then
      (Variables|Game|SetShipBuilderGameMode _asbp_ship_builder_game_mode)
      (CallFunction|SetupSlotsOrigin))
    (:CastFailed
      _))
  ;[1 1 1] ADD tags to part
  (CallFunction|AddTags)
  ;[1 1 1] SETUP Material
  (Utilities|IsValid _material
    (:Is%20Valid
      (CallFunction|SetPieceMaterial _material true))))

(fn AddBuildSlotsHorizontal
  (params (Build%20Slot%20Type :type BuildSlotType%20Enum :default "NewEnumerator0"))
  (bind _visualisation_scale (Variables|Appearance|GetVisualisation%20Scale))
  (bind _gameinstance (Variables|Game|GetGameInstance))
  (bind _gameinstance_2 (Variables|Game|GetGameInstance))
  (bind _visualisation_scale_2 (Variables|Appearance|GetVisualisation%20Scale))
  (for _index (range 0 (- (Variables|SlotOrigin|GetSlots%20X) 1))
    (for _index_2 (range 0 (- (Variables|SlotOrigin|GetSlots%20Y) 1))
      (if (Utilities|Enum|Equal(Enum) Build%20Slot%20Type "NewEnumerator0")
        (bind _returnvalue (AddComponent|AddChildActorComponent false (Math|Transform|MakeTransform (- (Variables|SlotOrigin|GetRelative%20Euclidean%20Origin) (Math|Vector|MakeVector (* _index (Variables|/Game/Blueprints/AllLevels/BP_GameInstance.BP_GameInstance_C|GetBuild%20Distance%20X _gameinstance)) (* _index_2 (Variables|/Game/Blueprints/AllLevels/BP_GameInstance.BP_GameInstance_C|GetBuild%20Distance%20Y _gameinstance)) (* (Variables|SlotOrigin|GetPlate%20Height) (* (Variables|/Game/Blueprints/AllLevels/BP_GameInstance.BP_GameInstance_C|GetBuild%20Distance%20Z _gameinstance) -1.0)))) "0, 0, 0" (Math|Vector|MakeVector _visualisation_scale _visualisation_scale _visualisation_scale))))
        (ChildActorComponent|SetChildActorClass _returnvalue "/Game/Blueprints/ShipBuilder/BP_ConnectionSlot.BP_ConnectionSlot_C")
        (bind _asbp_connection_slot (Utilities|Casting|CastToBP_ConnectionSlot (Variables|/Script/Engine.ChildActorComponent|GetChildActor _returnvalue)))
        (Variables|/Game/Blueprints/ShipBuilder/BP_ConnectionSlot.BP_ConnectionSlot_C|SetRelativeLocation _asbp_connection_slot (- (Variables|SlotOrigin|GetRelative%20Euclidean%20Origin) (Math|Vector|MakeVector (* _index (Variables|/Game/Blueprints/AllLevels/BP_GameInstance.BP_GameInstance_C|GetBuild%20Distance%20X _gameinstance)) (* _index_2 (Variables|/Game/Blueprints/AllLevels/BP_GameInstance.BP_GameInstance_C|GetBuild%20Distance%20Y _gameinstance)) (* (Variables|SlotOrigin|GetPlate%20Height) (* (Variables|/Game/Blueprints/AllLevels/BP_GameInstance.BP_GameInstance_C|GetBuild%20Distance%20Z _gameinstance) -1.0)))))
        (Variables|/Game/Blueprints/ShipBuilder/BP_ConnectionSlot.BP_ConnectionSlot_C|SetSlot%20Type _asbp_connection_slot "NewEnumerator0")
        (Utilities|Array|Add (Variables|BuildSlots|GetBuildSlots_Male) _asbp_connection_slot)
        (else
          (bind _returnvalue_2 (AddComponent|AddChildActorComponent false (Math|Transform|MakeTransform (- (Variables|SlotOrigin|GetRelative%20Euclidean%20Origin) (Math|Vector|MakeVector (* _index (Variables|/Game/Blueprints/AllLevels/BP_GameInstance.BP_GameInstance_C|GetBuild%20Distance%20X _gameinstance_2)) (* _index_2 (Variables|/Game/Blueprints/AllLevels/BP_GameInstance.BP_GameInstance_C|GetBuild%20Distance%20Y _gameinstance_2)) 0.0)) "0, 0, 0" (Math|Vector|MakeVector _visualisation_scale_2 _visualisation_scale_2 _visualisation_scale_2))))
          (ChildActorComponent|SetChildActorClass _returnvalue_2 "/Game/Blueprints/ShipBuilder/BP_ConnectionSlot.BP_ConnectionSlot_C")
          (bind _asbp_connection_slot_2 (Utilities|Casting|CastToBP_ConnectionSlot (Variables|/Script/Engine.ChildActorComponent|GetChildActor _returnvalue_2)))
          (Variables|/Game/Blueprints/ShipBuilder/BP_ConnectionSlot.BP_ConnectionSlot_C|SetRelativeLocation _asbp_connection_slot_2 (- (Variables|SlotOrigin|GetRelative%20Euclidean%20Origin) (Math|Vector|MakeVector (* _index (Variables|/Game/Blueprints/AllLevels/BP_GameInstance.BP_GameInstance_C|GetBuild%20Distance%20X _gameinstance_2)) (* _index_2 (Variables|/Game/Blueprints/AllLevels/BP_GameInstance.BP_GameInstance_C|GetBuild%20Distance%20Y _gameinstance_2)) 0.0)))
          (Variables|/Game/Blueprints/ShipBuilder/BP_ConnectionSlot.BP_ConnectionSlot_C|SetSlot%20Type _asbp_connection_slot_2 "NewEnumerator1")
          (Utilities|Array|Add (Variables|BuildSlots|GetBuildSlots_Female) _asbp_connection_slot_2))))))

(fn SetPieceMaterial
  (params (Material :type Material%20Instance%20Object%20Reference) (IsOverlay :type Boolean))
  (Utilities|IsValid Material
    (:Is%20Valid
      (if IsOverlay
        _
        (else
          (Variables|Appearance|SetMaterial Material)))
      (Rendering|Material|SetMaterial (Variables|Default|GetStaticMesh) 0 Material))))

(fn SetHovered
  (params (SetHovered :type Boolean))
  (bind _staticmesh (Variables|Default|GetStaticMesh))
  (if (and (.CanBuildWith (Utilities|Struct|BreakShipPartInfo (Variables|Default|GetShipPartInfo))) (not (Variables|Selecting|GetIsSelected)))
    (bind _output_get (Variables|Selecting|SetIsHovered SetHovered))
    (Rendering|SetRenderCustomDepth _staticmesh _output_get)
    (Rendering|SetCustomDepthStencilValue _staticmesh 2)))

(fn AddTags
  (bind _shipbuildergamemode (Variables|Game|GetShipBuilderGameMode))
  (Utilities|IsValid _shipbuildergamemode
    (:Is%20Valid
      (Utilities|Array|Add (Variables|Actor|GetTags) (Variables|/Game/Blueprints/ShipBuilder/BP_ShipBuilderGameMode.BP_ShipBuilderGameMode_C|GetShipPartTag _shipbuildergamemode)))))

(fn SetupSlotsOrigin
  (bind _gameinstance (Variables|Game|GetGameInstance))
  (bind _relative_slots_origin (Variables|SlotOrigin|GetRelative%20Slots%20Origin))
  (bind (_x _y _z) (Math|Vector|BreakVector _relative_slots_origin))
  (Variables|SlotOrigin|SetRelative%20Euclidean%20Origin (Math|Vector|MakeVector (* (Variables|/Game/Blueprints/AllLevels/BP_GameInstance.BP_GameInstance_C|GetBuild%20Distance%20X _gameinstance) _x) (* (Variables|/Game/Blueprints/AllLevels/BP_GameInstance.BP_GameInstance_C|GetBuild%20Distance%20Y _gameinstance) _y) (* (Variables|/Game/Blueprints/AllLevels/BP_GameInstance.BP_GameInstance_C|GetBuild%20Distance%20Z _gameinstance) _z))))

(fn GetBuildDistances
  (bind _gameinstance (Variables|Game|GetGameInstance))
  (return (Variables|/Game/Blueprints/AllLevels/BP_GameInstance.BP_GameInstance_C|GetBuild%20Distance%20X _gameinstance) (Variables|/Game/Blueprints/AllLevels/BP_GameInstance.BP_GameInstance_C|GetBuild%20Distance%20Y _gameinstance) (Variables|/Game/Blueprints/AllLevels/BP_GameInstance.BP_GameInstance_C|GetBuild%20Distance%20Z _gameinstance)))

(fn MakeBuildDistanceVector
  (params (X :type Float%20%28single-precision%29) (Y :type Float%20%28single-precision%29) (Z :type Float%20%28single-precision%29))
  (bind (_x _y _z) (CallFunction|GetBuildDistances))
  (return (Math|Vector|MakeVector (* X _x) (* Y _y) (* Z _z))))

(fn CycleThroughBuildSlots
  (params (Slot%20Type :type BuildSlotType%20Enum :default "NewEnumerator0") (Cycle%20Amount :type Integer))
  (bind _buildslots_male (Variables|BuildSlots|GetBuildSlots_Male))
  (bind _buildslots_female (Variables|BuildSlots|GetBuildSlots_Female))
  (bind _returnvalue (Utilities|Array|Length _buildslots_male))
  (bind _returnvalue_2 (Utilities|Array|Length _buildslots_female))
  (Utilities|FlowControl|Sequence
    (:then_0
      (switch Utilities|FlowControl|Switch|SwitchonBuildSlotType Slot%20Type
        (:NewEnumerator0
          (if (>= (+ (Variables|BuildSlots|GetCurrentBuildSlotIndex_Male) Cycle%20Amount) _returnvalue)
            (Variables|BuildSlots|SetCurrentBuildSlotIndex_Male 0)
            (elif (< (+ (Variables|BuildSlots|GetCurrentBuildSlotIndex_Male) Cycle%20Amount) 0)
              (Variables|BuildSlots|SetCurrentBuildSlotIndex_Male (- _returnvalue 1))
              (else
                (Variables|BuildSlots|SetCurrentBuildSlotIndex_Male (+ (Variables|BuildSlots|GetCurrentBuildSlotIndex_Male) Cycle%20Amount))))))
        (:NewEnumerator1
          (if (>= (+ (Variables|BuildSlots|GetCurrentBuildSlotIndex_Female) Cycle%20Amount) _returnvalue_2)
            (Variables|BuildSlots|SetCurrentBuildSlotIndex_Female 0)
            (elif (< (+ (Variables|BuildSlots|GetCurrentBuildSlotIndex_Female) Cycle%20Amount) 0)
              (Variables|BuildSlots|SetCurrentBuildSlotIndex_Female (- _returnvalue_2 1))
              (else
                (Variables|BuildSlots|SetCurrentBuildSlotIndex_Female (+ (Variables|BuildSlots|GetCurrentBuildSlotIndex_Female) Cycle%20Amount))))))))
    (:then_1
      (CallFunction|MoveSelectedConnectionSlotVisual Slot%20Type))))

(fn GetCurrentBuildSlot
  (params (Slot%20Type :type BuildSlotType%20Enum :default "NewEnumerator0"))
  (switch Utilities|FlowControl|Switch|SwitchonBuildSlotType Slot%20Type
    (:NewEnumerator0
      (return (Utilities|Array|Get(acopy) (Variables|BuildSlots|GetBuildSlots_Male) (Variables|BuildSlots|GetCurrentBuildSlotIndex_Male))))
    (:NewEnumerator1
      (return (Utilities|Array|Get(acopy) (Variables|BuildSlots|GetBuildSlots_Female) (Variables|BuildSlots|GetCurrentBuildSlotIndex_Female))))))

(fn MoveSelectedConnectionSlotVisual
  (params (Slot%20Type :type BuildSlotType%20Enum :default "NewEnumerator0"))
  (bind _build_slot (CallFunction|GetCurrentBuildSlot Slot%20Type))
  (Utilities|IsValid _build_slot
    (:Is%20Valid
      (Transformation|AttachActorToActor (CallFunction|GetSelectedConnectionSlotVisual Slot%20Type) _build_slot "None" "KeepRelative" "KeepRelative" "KeepRelative" true))))

(fn GetSelectedConnectionSlotVisual
  (params (Slot%20Type :type BuildSlotType%20Enum :default "NewEnumerator0"))
  (switch Utilities|FlowControl|Switch|SwitchonBuildSlotType Slot%20Type
    (:NewEnumerator0
      (Utilities|IsValid (Variables|BuildSlots|GetSelectedConnectionSlotVisual_Male)
        (:Is%20Valid
          _)
        (:Is%20Not%20Valid
          (bind _returnvalue (Game|SpawnActorfromClass "/Game/Blueprints/ShipBuilder/BP_SelectedConnectionSlotVisual.BP_SelectedConnectionSlotVisual_C" (Math|Transform|MakeTransform "0, 0, 0") "Undefined" 0 0))
          (bind _output_get (Variables|BuildSlots|SetSelectedConnectionSlotVisual_Male _returnvalue))))
      (return _output_get))
    (:NewEnumerator1
      (Utilities|IsValid (Variables|BuildSlots|GetSelectedConnectionSlotVisual_Female)
        (:Is%20Valid
          _)
        (:Is%20Not%20Valid
          (bind _returnvalue_2 (Game|SpawnActorfromClass "/Game/Blueprints/ShipBuilder/BP_SelectedConnectionSlotVisual.BP_SelectedConnectionSlotVisual_C" (Math|Transform|MakeTransform "0, 0, 0") "Undefined" 0 0))
          (bind _output_get_2 (Variables|BuildSlots|SetSelectedConnectionSlotVisual_Female _returnvalue_2))))
      (return _output_get_2))))

(fn SPDestroyConnectionSlotVisuals
  (bind _outactors (Actor|GetAllActorsOfClass "/Game/Blueprints/ShipBuilder/BP_SelectedConnectionSlotVisual.BP_SelectedConnectionSlotVisual_C"))
  (for _array_element _outactors
    (Actor|DestroyActor _array_element)))

(fn UnsetAllConnectionSlots
  (for _array_element (Actor|GetAllChildActors false)
    (bind _asbp_connection_slot (Utilities|Casting|CastToBP_ConnectionSlot _array_element))
    (Default|UnsetConnectionSlot _asbp_connection_slot)))

(fn SPConnectAllConnectedConnectionSlots
  ;[1 1 1] FIND all connection slots of this part
  (for _array_element (Actor|GetAllChildActors false)
    (bind _asbp_connection_slot (Utilities|Casting|CastToBP_ConnectionSlot _array_element)
      (:then
        ;[1 1 1] CHECK if this slot overlaps any other slots
        (LocalVariables|SetThisPartConnectionSlot _asbp_connection_slot)
        (if (== (Utilities|Array|Length (Collision|GetOverlappingActors (Variables|/Game/Blueprints/ShipBuilder/BP_ConnectionSlot.BP_ConnectionSlot_C|GetCollision%20Sphere _asbp_connection_slot) "/Game/Blueprints/ShipBuilder/BP_ConnectionSlot.BP_ConnectionSlot_C" :!class /Script/Engine.PrimitiveComponent)) 1)
          ;[1 1 1] SET connection between the 2 slots that overlap
          (for _array_element_2 (Collision|GetOverlappingActors (Variables|/Game/Blueprints/ShipBuilder/BP_ConnectionSlot.BP_ConnectionSlot_C|GetCollision%20Sphere _asbp_connection_slot) "/Game/Blueprints/ShipBuilder/BP_ConnectionSlot.BP_ConnectionSlot_C" :!class /Script/Engine.PrimitiveComponent)
            (bind _asbp_connection_slot_2 (Utilities|Casting|CastToBP_ConnectionSlot _array_element_2)
              (:then
                (LocalVariables|SetOtherPartConnectionSlot _asbp_connection_slot_2)
                (Default|SetConnectionSlot (LocalVariables|GetThisPartConnectionSlot) (LocalVariables|GetOtherPartConnectionSlot)))
              (:CastFailed
                ;[1 1 1] OVERLAP not another slot
                (Development|PrintString "ERROR: Failed to cast overlapped part to connection slot" true true "(R=1.000000,G=0.000000,B=0.000000,A=1.000000)" 1e+01))))
          (else
            ;[1 1 1] TOO MANY OVERLAPS
            (if (> (Utilities|Array|Length (Collision|GetOverlappingActors (Variables|/Game/Blueprints/ShipBuilder/BP_ConnectionSlot.BP_ConnectionSlot_C|GetCollision%20Sphere _asbp_connection_slot) "/Game/Blueprints/ShipBuilder/BP_ConnectionSlot.BP_ConnectionSlot_C" :!class /Script/Engine.PrimitiveComponent)) 0)
              (Development|PrintString "ERROR: Connection Slot overlapped more than 1 other connection slot." true true "(R=1.000000,G=0.000000,B=0.000000,A=1.000000)" 1e+01)))))
      (:CastFailed
        (Development|PrintString "ERROR: Failed to cast THIS part connection slot" true true "(R=1.000000,G=0.000000,B=0.000000,A=1.000000)" 1e+01)))))

(fn PositionCustomConnectionSlot
  (params (Custom%20Connection%20Slot :type BP%20Connection%20Slot%20Object%20Reference) (Relative%20Location :type Vector) (Relative%20Rotation :type Rotator))
  (bind (_x _y _z) (Math|Vector|BreakVector Relative%20Location))
  (bind _build_location (CallFunction|MakeBuildDistanceVector _x _y _z))
  (Transformation|SetRelativeLocationAndRotation (Variables|/Script/Engine.Actor|GetRootComponent Custom%20Connection%20Slot) _build_location Relative%20Rotation false false)
  (if (Utilities|Enum|Equal(Enum) (Variables|/Game/Blueprints/ShipBuilder/BP_ConnectionSlot.BP_ConnectionSlot_C|GetSlot%20Type Custom%20Connection%20Slot) "NewEnumerator0")
    (Utilities|Array|Add (Variables|BuildSlots|GetBuildSlots_Male) Custom%20Connection%20Slot)
    (else
      (Utilities|Array|Add (Variables|BuildSlots|GetBuildSlots_Female) Custom%20Connection%20Slot)))
  (Variables|/Game/Blueprints/ShipBuilder/BP_ConnectionSlot.BP_ConnectionSlot_C|SetRelativeLocation Custom%20Connection%20Slot _build_location)
  (Variables|/Game/Blueprints/ShipBuilder/BP_ConnectionSlot.BP_ConnectionSlot_C|SetRelativeRotation Custom%20Connection%20Slot Relative%20Rotation))

(fn AddCustomConnectionSlotsHorizontal
  (params (Build%20Slot%20Type :type BuildSlotType%20Enum :default "NewEnumerator0") (Slots%20X :type Integer) (Slots%20Y :type Integer) (Plate%20Height :type Integer) (Relative%20Slot%20Origin :type Vector))
  (bind _visualisation_scale (Variables|Appearance|GetVisualisation%20Scale))
  (bind _gameinstance (Variables|Game|GetGameInstance))
  (bind _gameinstance_2 (Variables|Game|GetGameInstance))
  (bind _visualisation_scale_2 (Variables|Appearance|GetVisualisation%20Scale))
  (for _index (range 0 (- Slots%20X 1))
    (for _index_2 (range 0 (- Slots%20Y 1))
      (if (Utilities|Enum|Equal(Enum) Build%20Slot%20Type "NewEnumerator0")
        (bind _returnvalue (AddComponent|AddChildActorComponent false (Math|Transform|MakeTransform (- (CallFunction|SlotVectortoEuclideanVector Relative%20Slot%20Origin) (Math|Vector|MakeVector (* _index (Variables|/Game/Blueprints/AllLevels/BP_GameInstance.BP_GameInstance_C|GetBuild%20Distance%20X _gameinstance)) (* _index_2 (Variables|/Game/Blueprints/AllLevels/BP_GameInstance.BP_GameInstance_C|GetBuild%20Distance%20Y _gameinstance)) (* Plate%20Height (* (Variables|/Game/Blueprints/AllLevels/BP_GameInstance.BP_GameInstance_C|GetBuild%20Distance%20Z _gameinstance) -1.0)))) "0, 0, 0" (Math|Vector|MakeVector _visualisation_scale _visualisation_scale _visualisation_scale))))
        (ChildActorComponent|SetChildActorClass _returnvalue "/Game/Blueprints/ShipBuilder/BP_ConnectionSlot.BP_ConnectionSlot_C")
        (bind _asbp_connection_slot (Utilities|Casting|CastToBP_ConnectionSlot (Variables|/Script/Engine.ChildActorComponent|GetChildActor _returnvalue)))
        (Variables|/Game/Blueprints/ShipBuilder/BP_ConnectionSlot.BP_ConnectionSlot_C|SetRelativeLocation _asbp_connection_slot (- (CallFunction|SlotVectortoEuclideanVector Relative%20Slot%20Origin) (Math|Vector|MakeVector (* _index (Variables|/Game/Blueprints/AllLevels/BP_GameInstance.BP_GameInstance_C|GetBuild%20Distance%20X _gameinstance)) (* _index_2 (Variables|/Game/Blueprints/AllLevels/BP_GameInstance.BP_GameInstance_C|GetBuild%20Distance%20Y _gameinstance)) (* Plate%20Height (* (Variables|/Game/Blueprints/AllLevels/BP_GameInstance.BP_GameInstance_C|GetBuild%20Distance%20Z _gameinstance) -1.0)))))
        (Variables|/Game/Blueprints/ShipBuilder/BP_ConnectionSlot.BP_ConnectionSlot_C|SetSlot%20Type _asbp_connection_slot "NewEnumerator0")
        (Utilities|Array|Add (Variables|BuildSlots|GetBuildSlots_Male) _asbp_connection_slot)
        (else
          (bind _returnvalue_2 (AddComponent|AddChildActorComponent false (Math|Transform|MakeTransform (- (CallFunction|SlotVectortoEuclideanVector Relative%20Slot%20Origin) (Math|Vector|MakeVector (* _index (Variables|/Game/Blueprints/AllLevels/BP_GameInstance.BP_GameInstance_C|GetBuild%20Distance%20X _gameinstance_2)) (* _index_2 (Variables|/Game/Blueprints/AllLevels/BP_GameInstance.BP_GameInstance_C|GetBuild%20Distance%20Y _gameinstance_2)) 0.0)) "0, 0, 0" (Math|Vector|MakeVector _visualisation_scale_2 _visualisation_scale_2 _visualisation_scale_2))))
          (ChildActorComponent|SetChildActorClass _returnvalue_2 "/Game/Blueprints/ShipBuilder/BP_ConnectionSlot.BP_ConnectionSlot_C")
          (bind _asbp_connection_slot_2 (Utilities|Casting|CastToBP_ConnectionSlot (Variables|/Script/Engine.ChildActorComponent|GetChildActor _returnvalue_2)))
          (Variables|/Game/Blueprints/ShipBuilder/BP_ConnectionSlot.BP_ConnectionSlot_C|SetRelativeLocation _asbp_connection_slot_2 (- (CallFunction|SlotVectortoEuclideanVector Relative%20Slot%20Origin) (Math|Vector|MakeVector (* _index (Variables|/Game/Blueprints/AllLevels/BP_GameInstance.BP_GameInstance_C|GetBuild%20Distance%20X _gameinstance_2)) (* _index_2 (Variables|/Game/Blueprints/AllLevels/BP_GameInstance.BP_GameInstance_C|GetBuild%20Distance%20Y _gameinstance_2)) 0.0)))
          (Variables|/Game/Blueprints/ShipBuilder/BP_ConnectionSlot.BP_ConnectionSlot_C|SetSlot%20Type _asbp_connection_slot_2 "NewEnumerator1")
          (Utilities|Array|Add (Variables|BuildSlots|GetBuildSlots_Female) _asbp_connection_slot_2))))))

(fn SlotVectortoEuclideanVector
  (params (Slot%20Vector :type Vector))
  (bind (_x _y _z) (Math|Vector|BreakVector Slot%20Vector))
  (bind _gameinstance (Variables|Game|GetGameInstance))
  (return (Math|Vector|MakeVector (* _x (Variables|/Game/Blueprints/AllLevels/BP_GameInstance.BP_GameInstance_C|GetBuild%20Distance%20X _gameinstance)) (* _y (Variables|/Game/Blueprints/AllLevels/BP_GameInstance.BP_GameInstance_C|GetBuild%20Distance%20Y _gameinstance)) (* _z (Variables|/Game/Blueprints/AllLevels/BP_GameInstance.BP_GameInstance_C|GetBuild%20Distance%20Z _gameinstance)))))

(fn CheckforOverlap
  (bind _collisionbox (Variables|Default|GetCollisionBox))
  (bind _overlappingactors (Collision|GetOverlappingActors _collisionbox "BP_ShipPart_C" :!class /Script/Engine.PrimitiveComponent))
  ;[1 1 1] Check for any overlapping ship pieces
  (Utilities|IsValid _collisionbox
    (:Is%20Valid
      ;[1 1 1] LOOP through all overlapping pieces and set overlap
      (for _array_element _overlappingactors
        (bind _asbp_ship_part (Utilities|Casting|CastToBP_ShipPart _array_element))
        (CallFunction|SetOverlap _asbp_ship_part true))
      ;[1 1 1] FINALLY set this piece overlap
      (if (> (Utilities|Array|Length _overlappingactors) 0)
        (CallFunction|SetOverlap true)
        (else
          (bind _didchange_ (CallFunction|SetOverlap false))
          ;[1 1 1] IF there is no overlap and this was changed (meaning it was the first time of no overlap) then set all other pieces to no overlap
          (if _didchange_
            (Default|UnsetAllOverlaps (Variables|Game|GetShipBuilderGameMode))))))))

(fn SetOverlap
  (params (Overlapping :type Boolean))
  (if Overlapping
    (if (Variables|Selecting|GetIsOverlapping)
      (return false)
      (else
        (Variables|Selecting|SetIsOverlapping true)
        (CallFunction|SetPieceMaterial (Variables|/Game/Blueprints/ShipBuilder/BP_ShipBuilderGameMode.BP_ShipBuilderGameMode_C|GetInvalidMaterial (Variables|Game|GetShipBuilderGameMode)) true)))
    (elif (Variables|Selecting|GetIsOverlapping)
      (Variables|Selecting|SetIsOverlapping false)
      (CallFunction|SetPieceMaterial (Variables|Appearance|GetMaterial) true)
      (else
        (return false))))
  (return true))

(fn GetHoveredSelectionSlot
  (params (World%20Location :type Vector))
  (for _array_element (Actor|GetAllChildActors false)
    (bind _asbp_connection_slot (Utilities|Casting|CastToBP_ConnectionSlot _array_element))
    (if (and (not (Variables|/Game/Blueprints/ShipBuilder/BP_ConnectionSlot.BP_ConnectionSlot_C|GetIsConnected _asbp_connection_slot)) (or (< (Math|Vector|Distance(Vector) (Transformation|GetActorLocation _asbp_connection_slot) World%20Location) (LocalVariables|GetClosestDistance)) (== (LocalVariables|GetClosestDistance) 0.0)))
      (LocalVariables|SetClosestDistance (Math|Vector|Distance(Vector) (Transformation|GetActorLocation _asbp_connection_slot) World%20Location))
      (LocalVariables|SetNearestConnectionSlot _asbp_connection_slot)
      (LocalVariables|SetSlotFound true)))
  (return (LocalVariables|GetSlotFound) (LocalVariables|GetNearestConnectionSlot)))

(fn SetSelected
  (params (IsSelected :type Boolean))
  (bind _staticmesh (Variables|Default|GetStaticMesh))
  (Utilities|FlowControl|Sequence
    (:then_0
      (Variables|Selecting|SetIsSelected IsSelected))
    (:then_1
      (if (not IsSelected)
        (CallFunction|SetIsMoving false)))
    (:then_2
      (Rendering|SetRenderCustomDepth _staticmesh IsSelected)
      (Rendering|SetCustomDepthStencilValue _staticmesh 1))))

(fn SetIsMoving
  (params (IsMoving :type Boolean))
  (bind _staticmesh (Variables|Default|GetStaticMesh))
  (bind _output_get (Variables|Selecting|SetIsMoving IsMoving))
  (if _output_get
    (Rendering|SetRenderCustomDepth _staticmesh _output_get)
    (Rendering|SetCustomDepthStencilValue _staticmesh 3)))

(fn SPSetIsClickable
  (Variables|Selecting|SetIsClickable true)
  (Default|SetIsClickable (Variables|Default|GetBP_ClickableShipPartComponent)))