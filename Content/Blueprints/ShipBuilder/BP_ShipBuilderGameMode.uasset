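; Game mode for the ship builder, where the player assembles a custom ship from parts within a build currency budget.
; BeginPlay loads the selected ship or spawns an empty one, and feeds buildable DataTable parts to the UI.
; Tick traces under the mouse to highlight parts or snap the held piece to the nearest slot, joining male to female connectors.
; Placement checks overlap and cost; saving records the ship in the player profile.
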(event Custom|Place%20Building%20Piece
  (bind _selected_ship_part (Variables|BuildPieces|GetSelected%20Ship%20Part))
  ;[1 1 1] Place Building Piece
  (Utilities|IsValid _selected_ship_part
    (:Is%20Valid
      (if (not (Variables|/Game/Blueprints/ShipBuilder/BP_ShipPart.BP_ShipPart_C|GetIsOverlapping _selected_ship_part))
        (if (>= (Variables|Default|GetBuildCurrency) (.Cost (Utilities|Struct|BreakShipPartInfo (Variables|BuildPieces|GetSelected%20Ship%20Part%20Info))))
          ;;[1 1 1] ADD piece to the ship
          (CallFunction|AddCurrentParttoShip)
          ;;[1 1 1] Detach current build piece which places it
          (CallFunction|SetCurrentShipPart)
          (CallFunction|SpawnNewBuildPiece))))))

(event Custom|Spawn%20New%20Build%20Piece
  (bind _selected_ship_part_info (Variables|BuildPieces|GetSelected%20Ship%20Part%20Info))
  (bind (_canbuildwith _id _category _displayname _class _imagetexture _isvalid _isselected _speedaddition _manueverabilityaddition _armouraddition _firerateaddition _firespeedaddition _cost _defaultmaterial) (Utilities|Struct|BreakShipPartInfo _selected_ship_part_info))
  ;[1 1 1] Spawn new building piece
  (if (and (Utilities|IsValidClass _class) _isvalid)
    ;;[1 1 1] Spawn initial block
    (bind _returnvalue (Game|SpawnActorfromClass _class (Math|Transform|MakeTransform (Variables|BuildSpace|GetCurrent%20Build%20Location) (Variables|BuildSpace|GetCurrent%20Piece%20Rotation)) "Undefined" 0 _defaultmaterial (Variables|BuildPieces|GetSelected%20Ship%20Part%20Info) 0))
    (Utilities|Array|Add (Variables|/Script/Engine.Actor|GetTags _returnvalue) "BuildPiece")
    (CallFunction|SetCurrentShipPart _returnvalue)
    (else
      (CallFunction|Set2DCursor "NewEnumerator2"))))

(event Custom|Rotate%20Building%20Piece
  (params (Relative%20Rotation%20Angles :type Rotator))
  ;[1 1 1] Rotate build piece
  (if (Utilities|Enum|Equal(Enum) (Variables|UI|Get2DCursorMode) "NewEnumerator1")
    (Variables|BuildSpace|SetCurrent%20Piece%20Rotation (Math|Rotator|CombineRotators Relative%20Rotation%20Angles (Variables|BuildSpace|GetCurrent%20Piece%20Rotation)))
    (CallFunction|SetShipPartLocation)))

(event Custom|Respawn%20Build%20Piece
  (bind _selected_ship_part (Variables|BuildPieces|GetSelected%20Ship%20Part))
  ;[1 1 1] RESPAWN build piece
  (if (Utilities|IsValid _selected_ship_part)
    (Actor|DestroyActor _selected_ship_part))
  (CallFunction|SpawnNewBuildPiece))

(event Custom|Unselect%20Build%20Piece
  (bind _selected_ship_part (Variables|BuildPieces|GetSelected%20Ship%20Part))
  ;[1 1 1] UNSELECT build piece
  (Variables|BuildPieces|SetSelected%20Ship%20Part%20Info "")
  (CallFunction|Set2DCursor "NewEnumerator2")
  (if (Utilities|IsValid _selected_ship_part)
    (Actor|DestroyActor _selected_ship_part)))

(event Custom|Select%20Build%20Piece
  ;[1 1 1] SELECT build piece
  (if (Utilities|Enum|Equal(Enum) (Variables|UI|Get2DCursorMode) "NewEnumerator0")
    (Utilities|IsValid (Variables|BuildPieces|GetCurrently%20Hovered%20Part)
      (:Is%20Valid
        (CallFunction|SetCurrentShipPart (Variables|BuildPieces|GetCurrently%20Hovered%20Part))
        (Default|SetHovered (Variables|BuildPieces|GetCurrently%20Hovered%20Part) false)
        (Variables|BuildPieces|SetCurrently%20Hovered%20Part 0)
        (CallFunction|Set2DCursor "NewEnumerator1")
        (Variables|Default|SetBuildCurrency (+ (Variables|Default|GetBuildCurrency) (.Cost (Utilities|Struct|BreakShipPartInfo (Variables|BuildPieces|GetSelected%20Ship%20Part%20Info)))))))))

(event EventBeginPlay
  (bind _returnvalue (Game|GetPlayerController 0))
  (bind _3dcursorscale (Variables|UI|Get3DCursorScale))
  (bind _buildcentre (Variables|BuildSpace|GetBuildCentre))
  (bind _returnvalue_2 (Math|Transform|MakeTransform _buildcentre))
  ;[1 1 1] BEGIN play
  (Utilities|FlowControl|Sequence
    (:then_0
      ;;[1 1 1] Load reference to game instance
      (bind _asbp_game_instance (Utilities|Casting|CastToBP_GameInstance (Game|GetGameInstance)))
      (Variables|Game|SetGameInstance _asbp_game_instance))
    (:then_1
      (CallFunction|Set2DCursor "NewEnumerator2"))
    (:then_2
      ;;[1 1 1] Set starting Build Location
      (Variables|BuildSpace|SetCurrent%20Build%20Location (Variables|BuildSpace|GetBuildCentre)))
    (:then_3
      ;;[1 1 1] Set input mode so mouse is used but not shown
      (Variables|/Script/Engine.PlayerController|SetbShowMouseCursor _returnvalue true)
      (Input|SetInputModeGameandUI _returnvalue 0 "DoNotLock" false))
    (:then_4
      ;;[1 1 1] SPAWN new ship
      (if (Variables|/Game/Blueprints/AllLevels/BP_GameInstance.BP_GameInstance_C|GetShipSelected (Variables|Game|GetGameInstance))
        (bind _returnvalue_3 (Game|SpawnActorfromClass "/Game/Blueprints/Ship/BP_CustomShip.BP_CustomShip_C" _returnvalue_2 "Undefined" 0 (.ShipParts (Utilities|Struct|BreakShipInfo (Variables|/Game/Blueprints/AllLevels/BP_GameInstance.BP_GameInstance_C|GetShipInfo (Variables|Game|GetGameInstance)))) (Utilities|String|ToString(Text) (.ShipName (Utilities|Struct|BreakShipInfo (Variables|/Game/Blueprints/AllLevels/BP_GameInstance.BP_GameInstance_C|GetShipInfo (Variables|Game|GetGameInstance))))) 0))
        (Default|LoadShip _returnvalue_3)
        (Variables|Ship|SetEditorShip _returnvalue_3)
        (else
          (bind _returnvalue_4 (Game|SpawnActorfromClass "/Game/Blueprints/Ship/BP_CustomShip.BP_CustomShip_C" _returnvalue_2 "Undefined" 0 0 "" 0))
          (Variables|Ship|SetEditorShip _returnvalue_4)))
      (CallFunction|CalculateInitialBuildCurrency))
    (:then_5
      ;;[1 1 1] Spawn and Set Cursor
      (bind _returnvalue_5 (Game|SpawnActorfromClass "/Game/Blueprints/ShipBuilder/BP_BuildCursor.BP_BuildCursor_C" (Math|Transform|MakeTransform "0, 0, 0" "0, 0, 0" (Math|Vector|MakeVector _3dcursorscale _3dcursorscale _3dcursorscale)) "Undefined" 0 0))
      (Variables|UI|Set3DCursor _returnvalue_5))
    (:then_6
      ;;[1 1 1] LOAD Build Pieces and Add to UI
      (bind _outrownames (DataTable|GetDataTableRowNames "/Game/Blueprints/ShipBuilder/ShipParts_DataTable.ShipParts_DataTable"))
      (for _array_element _outrownames
        (bind _returnvalue_6 (Utilities|GetDataTableRow "/Game/Blueprints/ShipBuilder/ShipParts_DataTable.ShipParts_DataTable" _array_element)
          (:then
            (if (.CanBuildWith (Utilities|Struct|BreakShipPartInfo _returnvalue_6))
              (Utilities|Array|Add (Variables|BuildPieces|GetShip%20Part%20Infos) _returnvalue_6)))))
      (bind _returnvalue_7 (UserInterface|CreateWidget "/Game/UI/ShipBuilder/ShipBuilderUI.ShipBuilderUI_C" (Game|GetPlayerController 0) (Variables|BuildPieces|GetShip%20Part%20Infos)))
      (UserInterface|Viewport|AddtoViewport _returnvalue_7 0))))

(event EventTick
  (params (DeltaSeconds :type Float%20%28single-precision%29))
  (bind _returnvalue (Game|GetPlayerController 0))
  (bind _selected_ship_part (Variables|BuildPieces|GetSelected%20Ship%20Part))
  (bind (_worldlocation _worlddirection) (Game|Player|ConvertMouseLocationToWorldSpace _returnvalue))
  ;[1 1 1] EVENT tick
  (Utilities|FlowControl|Sequence
    (:then_0
      ;;[1 1 1] GET the mouse pointing location
      (bind _outhit (Collision|LineTraceForObjects _worldlocation (+ _worldlocation (* _worlddirection 1e+02)) (Utilities|Array|MakeArray "ObjectTypeQuery2" "ObjectTypeQuery1") false 0 "None"))
      ;;[1 1 1] SET the cursor position
      (Transformation|SetActorLocation (Variables|UI|Get3DCursor) (.Location (Collision|BreakHitResult _outhit)) false false)
      (if (Utilities|Enum|Equal(Enum) (Variables|UI|Get2DCursorMode) "NewEnumerator1")
        (if (.CanBuildWith (Utilities|Struct|BreakShipPartInfo (Variables|BuildPieces|GetSelected%20Ship%20Part%20Info)))
          ;;[1 1 1] Move the new piece into position
          ;;;[1 1 1] Set the locations and calculate the nearest 'snap' location
          (bind _nearest_build_slot (CallFunction|GetNearestBuildSlot (.Location (Collision|BreakHitResult _outhit))))
          (if (Utilities|IsValid _nearest_build_slot)
            (Variables|BuildSpace|SetCurrent%20Build%20Location (Transformation|GetWorldLocation _nearest_build_slot))
            ;;;[1 1 1] Move build piece if a one has been selected
            (if (Utilities|IsValid (Variables|BuildPieces|GetSelected%20Ship%20Part))
              ;;;;[1 1 1] GET build slot on build piece to connect to (opposite type)
              (if (Utilities|Enum|Equal(Enum) (Variables|/Game/Blueprints/ShipBuilder/ShipPartConnectionSlot.ShipPartConnectionSlot_C|GetSlotType _nearest_build_slot) "NewEnumerator0")
                (Variables|Default|SetCurrent%20Build%20Slot (Variables|/Game/Blueprints/ShipBuilder/BP_ShipPart.BP_ShipPart_C|GetCurrentBuildSlotFemale _selected_ship_part))
                (else
                  (Variables|Default|SetCurrent%20Build%20Slot (Variables|/Game/Blueprints/ShipBuilder/BP_ShipPart.BP_ShipPart_C|GetCurrentBuildSlotMale _selected_ship_part))))
              ;;;;[1 1 1] Move piece to new location and apply rotation transforms
              (CallFunction|SetShipPartLocation)))
          (else
            (CallFunction|Set2DCursor "NewEnumerator2")))
        (else
          ;;[1 1 1] SET the hovered material of the piece that is moused over
          (bind _outactors (Actor|GetAllActorsOfClass "/Game/Blueprints/ShipBuilder/BP_ShipPart.BP_ShipPart_C"))
          (bind _asbp_ship_part (Utilities|Casting|CastToBP_ShipPart (.HitActor (Collision|BreakHitResult _outhit)))
            (:then
              ;;;[1 1 1] LOOP through all pieces and unset unless it is hovered over in which case set if it has not already been
              (for _array_element _outactors
                (if (== _array_element _asbp_ship_part)
                  (Default|SetHovered _array_element true)
                  (else
                    (Default|SetHovered _array_element false)))))
            (:CastFailed
              ;;;[1 1 1] LOOP through all pieces and unset hovered state
              (for _array_element_2 _outactors
                (Default|SetHovered _array_element_2 false)))))))))

(event EventPostLogin
  (params (NewPlayer :type Player%20Controller%20Object%20Reference))
  ;[1 1 1] Setup Player Controller
  (bind _asbp_ship_builder_player_controller (Utilities|Casting|CastToBP_ShipBuilderPlayerController NewPlayer))
  (Variables|Game|SetPlayerController _asbp_ship_builder_player_controller))

(fn ConstructionScript)

(fn CalculatePlaneIntersectionPoint
  (params (Line%20Origin :type Vector) (Line%20Direction :type Vector) (Plane%20Origin :type Vector) (Plane%20Normal :type Vector))
  (bind (_x _y _z) (Math|Vector|BreakVector Line%20Origin))
  (bind (_x_2 _y_2 _z_2) (Math|Vector|BreakVector Line%20Direction))
  (bind _returnvalue (Math|Vector|DotProduct Plane%20Normal Line%20Direction))
  (bind _returnvalue_2 (Math|Vector|DotProduct Plane%20Normal Line%20Origin))
  (bind _returnvalue_3 (Math|Vector|DotProduct Plane%20Normal Plane%20Origin))
  (bind _returnvalue_4 (- _returnvalue_2 _returnvalue_3))
  (bind _returnvalue_5 (* _returnvalue_4 -1.0))
  (bind _returnvalue_6 (/ _returnvalue_5 _returnvalue))
  (return (Math|Vector|MakeVector (+ _x (* _x_2 _returnvalue_6)) (+ _y (* _y_2 _returnvalue_6)) (+ _z (* _z_2 _returnvalue_6)))))

(fn GetNearestSnapLocation
  (params (Exact%20Location :type Vector))
  (bind (_x _y _z) (Math|Vector|BreakVector Exact%20Location))
  (bind _returnvalue (Game|GetGameInstance))
  (bind _asbp_game_instance (Utilities|Casting|CastToBP_GameInstance _returnvalue))
  (return (Math|Vector|MakeVector (CallFunction|SnaptoNearestFloat _x (Variables|/Game/Blueprints/AllLevels/BP_GameInstance.BP_GameInstance_C|GetBuild%20Distance%20X _asbp_game_instance)) (CallFunction|SnaptoNearestFloat _y (Variables|/Game/Blueprints/AllLevels/BP_GameInstance.BP_GameInstance_C|GetBuild%20Distance%20Y _asbp_game_instance)) (CallFunction|SnaptoNearestFloat _z (Variables|/Game/Blueprints/AllLevels/BP_GameInstance.BP_GameInstance_C|GetBuild%20Distance%20Z _asbp_game_instance)))))

(fn SnaptoNearestFloat
  (params (Input%20Number :type Float%20%28single-precision%29) (Snap%20Size :type Float%20%28single-precision%29))
  (bind _returnvalue (Math|Float|%(Float) Input%20Number Snap%20Size))
  (bind _returnvalue_2 (- Input%20Number _returnvalue))
  (if (> _returnvalue (/ Snap%20Size 2.0))
    (return (+ _returnvalue_2 Snap%20Size))
    (else
      (return _returnvalue_2))))

(fn GetNearestBuildSlot
  (params (Build%20Location :type Vector))
  (bind _outactors (Actor|GetAllActorswithTag (Variables|BuildPieces|GetShipPartTag)))
  (for _array_element _outactors
    (if (not (== _array_element (Variables|BuildPieces|GetSelected%20Ship%20Part)))
      (for _array_element_2 (Actor|GetComponentsByClass _array_element "/Game/Blueprints/ShipBuilder/ShipPartConnectionSlot.ShipPartConnectionSlot_C")
        (if (or (< (Math|Vector|Distance(Vector) (Transformation|GetWorldLocation _array_element_2) Build%20Location) (LocalVariables|GetNearest%20Distance)) (== (LocalVariables|GetNearest%20Distance) 0.0))
          (LocalVariables|SetNearest%20Distance (Math|Vector|Distance(Vector) (Transformation|GetWorldLocation _array_element_2) Build%20Location))
          (LocalVariables|SetCurrent%20Nearest%20Build%20Slot _array_element_2)))))
  (return (LocalVariables|GetCurrent%20Nearest%20Build%20Slot)))

(fn SetShipPartLocation
  (bind _current_build_slot (Variables|Default|GetCurrent%20Build%20Slot))
  (bind _current_piece_rotation (Variables|BuildSpace|GetCurrent%20Piece%20Rotation))
  (bind _returnvalue (Transformation|GetRelativeTransform _current_build_slot))
  (bind _returnvalue_2 (Math|Transform|MakeTransform "0, 0, 0" _current_piece_rotation))
  (bind _returnvalue_3 (Math|Transform|ComposeTransforms _returnvalue _returnvalue_2))
  (bind (_location _rotation) (Math|Transform|BreakTransform _returnvalue_3))
  ;[1 1 1] Check if a build piece has been selected
  (Utilities|IsValid (Variables|BuildPieces|GetSelected%20Ship%20Part)
    (:Is%20Valid
      ;[1 1 1] Check if a build slot has been selected
      (Utilities|IsValid (Variables|Default|GetCurrent%20Build%20Slot)
        (:Is%20Valid
          ;[1 1 1] Set build piece location
          (Transformation|SetActorLocationAndRotation (Variables|BuildPieces|GetSelected%20Ship%20Part) (- (Variables|BuildSpace|GetCurrent%20Build%20Location) _location) _rotation))))))

(fn Set2DCursor
  (params (Cursor%20Mode :type BP_CursorModeEnum%20Enum :default "NewEnumerator2"))
  (bind _output_get (Variables|UI|Set2DCursorMode Cursor%20Mode))
  (Default|SetMouseCursor (Variables|Game|GetPlayerController) _output_get))

(fn SetCurrentShipPart
  (params (Ship%20Part :type BP%20Ship%20Part%20Object%20Reference))
  (bind _output_get (Variables|BuildPieces|SetSelected%20Ship%20Part Ship%20Part))
  (Utilities|IsValid _output_get
    (:Is%20Valid
      (Variables|BuildSpace|SetCurrent%20Piece%20Rotation (Transformation|GetWorldRotation (Variables|/Game/Blueprints/ShipBuilder/BP_ShipPart.BP_ShipPart_C|GetStaticMesh _output_get)))
      (bind _output_get_2 (Variables|BuildPieces|SetSelected%20Ship%20Part%20Info (Variables|/Game/Blueprints/ShipBuilder/BP_ShipPart.BP_ShipPart_C|GetShipPartInfo _output_get)))
      (Variables|BuildPieces|SetSelected%20Ship%20Part%20Class (Utilities|GetClass _output_get))
      (Variables|Materials|SetSelectMaterial (.DefaultMaterial (Utilities|Struct|BreakShipPartInfo _output_get_2))))))

(fn CalculateVehicleStats
  (bind _editorship (Variables|Ship|GetEditorShip))
  ;[1 1 1] RESET stats
  (Default|ResetStats (Variables|/Game/Blueprints/Ship/BP_Ship.BP_Ship_C|GetShipStats _editorship))
  (for _array_element (Variables|/Game/Blueprints/Ship/BP_CustomShip.BP_CustomShip_C|GetShipParts _editorship)
    (Default|AddStats (Variables|/Game/Blueprints/Ship/BP_Ship.BP_Ship_C|GetShipStats (Variables|Ship|GetEditorShip)) (.SpeedAddition (Utilities|Struct|BreakShipPartInfo (.ShipPartInfo (Utilities|Struct|BreakShipPart _array_element)))) (.ManueverabilityAddition (Utilities|Struct|BreakShipPartInfo (.ShipPartInfo (Utilities|Struct|BreakShipPart _array_element)))) (.ArmourAddition (Utilities|Struct|BreakShipPartInfo (.ShipPartInfo (Utilities|Struct|BreakShipPart _array_element)))) (.FireRateAddition (Utilities|Struct|BreakShipPartInfo (.ShipPartInfo (Utilities|Struct|BreakShipPart _array_element)))) (.FireSpeedAddition (Utilities|Struct|BreakShipPartInfo (.ShipPartInfo (Utilities|Struct|BreakShipPart _array_element)))))))

(fn AddCurrentParttoShip
  (bind _selected_ship_part_info (Variables|BuildPieces|GetSelected%20Ship%20Part%20Info))
  (Default|AddParttoShip (Variables|Ship|GetEditorShip) (Utilities|Struct|MakeShipPart _selected_ship_part_info (Variables|BuildPieces|GetSelected%20Ship%20Part) "0.000000,0.000000,0.000000|0.000000,0.000000,0.000000|1.000000,1.000000,1.000000" (Variables|Materials|GetSelectMaterial)))
  (Default|CalculateVehicleStats (Variables|Ship|GetEditorShip))
  (Variables|Default|SetBuildCurrency (- (Variables|Default|GetBuildCurrency) (.Cost (Utilities|Struct|BreakShipPartInfo _selected_ship_part_info)))))

(fn SaveShip
  (bind _gameinstance (Variables|Game|GetGameInstance))
  (bind _playerinfo (Variables|/Game/Blueprints/AllLevels/BP_GameInstance.BP_GameInstance_C|GetPlayerInfo _gameinstance))
  (bind _customshipsavegames (Utilities|Struct|BreakPlayerInfo _playerinfo))
  (if (Variables|/Game/Blueprints/AllLevels/BP_GameInstance.BP_GameInstance_C|GetShipSelected (Variables|Game|GetGameInstance))
    ;[1 1 1] Save EXISTING ship
    (bind _savegamename (Default|SaveShip (Variables|Ship|GetEditorShip) (Utilities|String|ToString(Text) (.MyPlayerName (Utilities|Struct|BreakPlayerInfo (Variables|/Game/Blueprints/AllLevels/BP_GameInstance.BP_GameInstance_C|GetPlayerInfo (Variables|Game|GetGameInstance))))) true))
    (Utilities|Array|RemoveItem _customshipsavegames (.ShipSaveGameName (Utilities|Struct|BreakShipInfo (Variables|/Game/Blueprints/AllLevels/BP_GameInstance.BP_GameInstance_C|GetShipInfo (Variables|Game|GetGameInstance)))))
    (Utilities|Array|Add _customshipsavegames _savegamename)
    (CallFunction|SavePlayerInfo)
    (return _savegamename)
    (else
      ;[1 1 1] Save NEW ship
      (bind _savegamename_2 (Default|SaveShip (Variables|Ship|GetEditorShip) (Utilities|String|ToString(Text) (.MyPlayerName (Utilities|Struct|BreakPlayerInfo (Variables|/Game/Blueprints/AllLevels/BP_GameInstance.BP_GameInstance_C|GetPlayerInfo (Variables|Game|GetGameInstance))))) false))
      (Utilities|Array|Add (.CustomShipSaveGames (Utilities|Struct|BreakPlayerInfo (Variables|/Game/Blueprints/AllLevels/BP_GameInstance.BP_GameInstance_C|GetPlayerInfo (Variables|Game|GetGameInstance)))) _savegamename_2)
      (CallFunction|SavePlayerInfo)
      (return _savegamename_2))))

(fn SavePlayerInfo
  (Utilities|IsValid (Variables|Saves|GetSaveGameRef)
    (:Is%20Valid
      _)
    (:Is%20Not%20Valid
      (bind _returnvalue (SaveGame|CreateSaveGameObject "/Game/Blueprints/AllLevels/BP_ProfileSaveGame.BP_ProfileSaveGame_C"))
      (bind _asbp_profile_save_game (Utilities|Casting|CastToBP_ProfileSaveGame _returnvalue))
      (Variables|Saves|SetSaveGameRef _asbp_profile_save_game)))
  (Variables|/Game/Blueprints/AllLevels/BP_ProfileSaveGame.BP_ProfileSaveGame_C|SetS_PlayerInfo (Variables|Saves|GetSaveGameRef) (Variables|/Game/Blueprints/AllLevels/BP_GameInstance.BP_GameInstance_C|GetPlayerInfo (Variables|Game|GetGameInstance)))
  (SaveGame|SaveGametoSlot (Variables|Saves|GetSaveGameRef) (Variables|Saves|GetPlayerSettingsSave)))

(fn CalculateInitialBuildCurrency
  (bind _array_element (Utilities|Array|ForEachLoopwithBreak (Variables|/Game/Blueprints/Ship/BP_CustomShip.BP_CustomShip_C|GetShipParts (Variables|Ship|GetEditorShip)))
    (:LoopBody
      (Variables|Default|SetBuildCurrency (- (Variables|Default|GetBuildCurrency) (.Cost (Utilities|Struct|BreakShipPartInfo (.ShipPartInfo (Utilities|Struct|BreakShipPart _array_element)))))))))