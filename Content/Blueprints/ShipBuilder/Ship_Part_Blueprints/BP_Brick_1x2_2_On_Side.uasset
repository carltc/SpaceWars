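; Ship builder brick part, a 1x2 brick with two extra connection slots on one side.
; Its construction script runs the parent's setup, then casts the two SideConnector child actors to BP_ConnectionSlot.
; Each slot is placed through PositionCustomConnectionSlot at mirrored X offsets, pitched or rotated a quarter turn to sit sideways.
; The event graph holds only disabled default events.
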(event EventBeginPlay
  (|CallParentFunction) ; This node is disabled and will not be called.\nDrag off pins to build functionality.
)

(event Collision|EventActorBeginOverlap
  (params (OtherActor :type Actor%20Object%20Reference))
  (|CallParentFunction OtherActor) ; This node is disabled and will not be called.\nDrag off pins to build functionality.
)

(event EventTick
  (params (DeltaSeconds :type Float%20%28single-precision%29))
  (|CallParentFunction DeltaSeconds) ; This node is disabled and will not be called.\nDrag off pins to build functionality.
)

(fn ConstructionScript
  (|CallParentFunction)
  (CallFunction|PositionCustomConnectionSlot (.AsBP%20Connection%20Slot (Utilities|Casting|CastToBP_ConnectionSlot (Variables|/Script/Engine.ChildActorComponent|GetChildActor (Variables|Default|GetSide%20Connector%201)))) "0.500000,0.500000,1.770000" "0, 0,90.000000")
  (CallFunction|PositionCustomConnectionSlot (.AsBP%20Connection%20Slot (Utilities|Casting|CastToBP_ConnectionSlot (Variables|/Script/Engine.ChildActorComponent|GetChildActor (Variables|Default|GetSide%20Connector%202)))) "-0.500000,0.500000,1.770000" "0, 0,90.000000"))