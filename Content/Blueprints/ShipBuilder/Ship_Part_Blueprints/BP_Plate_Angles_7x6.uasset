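; Ship builder part for a 7x6 angled plate that defines where other parts connect to it.
; The construction script runs the parent's, then fills a stepped, symmetric taper with three nested-loop bands, two, four and six cells wide.
; Each cell gets two single horizontal connection slots offset from RelativeSlotsOrigin: one at plate height 1, one of a second slot type.
; The event graph has no active logic.
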(event EventBeginPlay
  (|CallParentFunction) ; This node is disabled and will not be called.\nDrag off pins to build functionality.
)

(event Collision|EventActorBeginOverlap
  (params (OtherActor :type Actor%20Object%20Reference))
  (|CallParentFunction OtherActor) ; This node is disabled and will not be called.\nDrag off pins to build functionality.
)

(event EventTick
  (params (DeltaSeconds :type Float%20%28single-precision%29))
  (|CallParentFunction DeltaSeconds) ; This node is disabled and will not be called.\nDrag off pins to build functionality.
)

(fn ConstructionScript
  (|CallParentFunction)
  (Utilities|FlowControl|Sequence
    (:then_0
      ;[1 1 1] ADD top row of slots
      (for _index (range 2 3)
        (for _index_2 (range 0 1)
          (CallFunction|AddCustomConnectionSlotsHorizontal "NewEnumerator0" 1 1 1 (- (Variables|Default|GetRelative%20Slots%20Origin) (Math|Vector|MakeVector (Math|Conversions|ToFloat(Integer) _index) (Math|Conversions|ToFloat(Integer) _index_2) 0.0)))
          (CallFunction|AddCustomConnectionSlotsHorizontal "NewEnumerator1" 1 1 0 (- (Variables|Default|GetRelative%20Slots%20Origin) (Math|Vector|MakeVector (Math|Conversions|ToFloat(Integer) _index) (Math|Conversions|ToFloat(Integer) _index_2) 0.0))))))
    (:then_1
      ;[1 1 1] ADD top row of slots
      (for _index_3 (range 1 4)
        (for _index_4 (range 2 4)
          (CallFunction|AddCustomConnectionSlotsHorizontal "NewEnumerator0" 1 1 1 (- (Variables|Default|GetRelative%20Slots%20Origin) (Math|Vector|MakeVector (Math|Conversions|ToFloat(Integer) _index_3) (Math|Conversions|ToFloat(Integer) _index_4) 0.0)))
          (CallFunction|AddCustomConnectionSlotsHorizontal "NewEnumerator1" 1 1 0 (- (Variables|Default|GetRelative%20Slots%20Origin) (Math|Vector|MakeVector (Math|Conversions|ToFloat(Integer) _index_3) (Math|Conversions|ToFloat(Integer) _index_4) 0.0))))))
    (:then_2
      ;[1 1 1] ADD top row of slots
      (for _index_5 (range 0 5)
        (for _index_6 (range 5 6)
          (CallFunction|AddCustomConnectionSlotsHorizontal "NewEnumerator0" 1 1 1 (- (Variables|Default|GetRelative%20Slots%20Origin) (Math|Vector|MakeVector (Math|Conversions|ToFloat(Integer) _index_5) (Math|Conversions|ToFloat(Integer) _index_6) 0.0)))
          (CallFunction|AddCustomConnectionSlotsHorizontal "NewEnumerator1" 1 1 0 (- (Variables|Default|GetRelative%20Slots%20Origin) (Math|Vector|MakeVector (Math|Conversions|ToFloat(Integer) _index_5) (Math|Conversions|ToFloat(Integer) _index_6) 0.0))))))))