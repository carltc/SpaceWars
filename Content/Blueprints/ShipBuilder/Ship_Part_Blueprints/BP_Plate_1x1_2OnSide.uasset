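; BP_Plate_1x1_2OnSide is a ship builder part: a 1x1 plate with two side connectors.
; Its construction script runs the parent's logic, then casts each connector's child actor to BP_ConnectionSlot.
; PositionCustomConnectionSlot places both slots at mirrored X offsets with opposite 90-degree yaws.
; The event graph holds only disabled default events.
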(event EventBeginPlay
  (|CallParentFunction) ; This node is disabled and will not be called.\nDrag off pins to build functionality.
)

(event Collision|EventActorBeginOverlap
  (params (OtherActor :type Actor%20Object%20Reference))
  (|CallParentFunction OtherActor) ; This node is disabled and will not be called.\nDrag off pins to build functionality.
)

(event EventTick
  (params (DeltaSeconds :type Float%20%28single-precision%29))
  (|CallParentFunction DeltaSeconds) ; This node is disabled and will not be called.\nDrag off pins to build functionality.
)

(fn ConstructionScript
  (|CallParentFunction)
  (Utilities|FlowControl|Sequence
    (:then_0
      (bind _asbp_connection_slot (Utilities|Casting|CastToBP_ConnectionSlot (Variables|/Script/Engine.ChildActorComponent|GetChildActor (Variables|Default|GetSide%20Connector%201))))
      (CallFunction|PositionCustomConnectionSlot _asbp_connection_slot "-0.100000,1.000000,0.770000" "90.000000, 0, 0"))
    (:then_1
      (bind _asbp_connection_slot_2 (Utilities|Casting|CastToBP_ConnectionSlot (Variables|/Script/Engine.ChildActorComponent|GetChildActor (Variables|Default|GetSide%20Connector%202))))
      (CallFunction|PositionCustomConnectionSlot _asbp_connection_slot_2 "0.100000,1.000000,0.770000" "-90.000000, 0, 0"))))