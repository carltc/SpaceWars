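; Player controller for the ship builder, translating input into part editing and camera control.
; It caches the builder game mode and pawn, delegating part placement, rotation, deletion, move mode and connection-slot cycling to the game mode and its selected part.
; Slot cycling repositions the part and rechecks overlap.
; Axis inputs pitch the pawn locally and yaw it in world space, while zoom scales the camera's clamped relative X.
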(event EventBeginPlay
  (bind _asbp_ship_builder_game_mode (Utilities|Casting|CastToBP_ShipBuilderGameMode (Game|GetGameMode)))
  (Variables|Default|SetBuildGameMode _asbp_ship_builder_game_mode)
  (bind _asbp_ship_builder_pawn (Utilities|Casting|CastToBP_ShipBuilderPawn (Game|Player|GetPlayerPawn 0)))
  (Variables|Default|SetPlayerPawn _asbp_ship_builder_pawn)
  (CallFunction|SetMouseCursor "NewEnumerator2"))

(event EventTick
  (params (DeltaSeconds :type Float%20%28single-precision%29)))

(event Input|ActionEvents|InputActionBuildZoomIn
  (params (Key :type Key%20Structure :default "None"))
  (bind _playerpawn (Variables|Default|GetPlayerPawn))
  (bind _camera (Variables|/Game/Blueprints/ShipBuilder/BP_ShipBuilderPawn.BP_ShipBuilderPawn_C|GetCamera _playerpawn))
  (bind _relativelocation (Variables|/Script/Engine.SceneComponent|GetRelativeLocation _camera))
  (bind (_x _y _z) (Math|Vector|BreakVector _relativelocation))
  ;[1 1 1] ZOOM in and out controls
  (:Pressed
    (Transformation|SetRelativeLocation _camera (Math|Vector|MakeVector (Math|Float|Clamp(Float) (* _x (/ 1.0 (Variables|Zoom|GetZoomSpeed))) (Variables|Zoom|GetZoomMax) (Variables|Zoom|GetZoomMin)) _y _z) false false)))

(event Input|ActionEvents|InputActionBuildZoomOut
  (params (Key :type Key%20Structure :default "None"))
  (bind _playerpawn (Variables|Default|GetPlayerPawn))
  (bind _camera (Variables|/Game/Blueprints/ShipBuilder/BP_ShipBuilderPawn.BP_ShipBuilderPawn_C|GetCamera _playerpawn))
  (bind _relativelocation (Variables|/Script/Engine.SceneComponent|GetRelativeLocation _camera))
  (bind (_x _y _z) (Math|Vector|BreakVector _relativelocation))
  ;[1 1 1] ZOOM in and out controls
  (:Pressed
    (Transformation|SetRelativeLocation _camera (Math|Vector|MakeVector (Math|Float|Clamp(Float) (* _x (Variables|Zoom|GetZoomSpeed)) (Variables|Zoom|GetZoomMax) (Variables|Zoom|GetZoomMin)) _y _z) false false)))

(event Input|ActionEvents|InputActionBuildCycleBuildSlotForward
  (params (Key :type Key%20Structure :default "None"))
  (bind _buildgamemode (Variables|Default|GetBuildGameMode))
  (bind _selected_ship_part (Variables|/Game/Blueprints/ShipBuilder/BP_ShipBuilderGameMode.BP_ShipBuilderGameMode_C|GetSelected%20Ship%20Part _buildgamemode))
  ;[1 1 1] CYCLE through connection slots
  (:Pressed
    (Default|CycleThroughBuildSlots _selected_ship_part "NewEnumerator0" 1)
    (Default|CycleThroughBuildSlots _selected_ship_part "NewEnumerator1" 1)
    (Default|UpdateSelectedShipPartConnectionSlot _buildgamemode)
    (Default|SetShipPartLocation _buildgamemode)
    (Default|CheckforOverlap _selected_ship_part)))

(event Input|ActionEvents|InputActionBuildCycleBuildSlotBackward
  (params (Key :type Key%20Structure :default "None"))
  (bind _buildgamemode (Variables|Default|GetBuildGameMode))
  (bind _selected_ship_part (Variables|/Game/Blueprints/ShipBuilder/BP_ShipBuilderGameMode.BP_ShipBuilderGameMode_C|GetSelected%20Ship%20Part _buildgamemode))
  ;[1 1 1] CYCLE through connection slots
  (:Pressed
    (Default|CycleThroughBuildSlots _selected_ship_part "NewEnumerator0" -1)
    (Default|CycleThroughBuildSlots _selected_ship_part "NewEnumerator1" -1)
    (Default|UpdateSelectedShipPartConnectionSlot _buildgamemode)
    (Default|SetShipPartLocation _buildgamemode)
    (Default|CheckforOverlap _selected_ship_part)))

(event Input|ActionEvents|InputActionToggleMoveMode
  (params (Key :type Key%20Structure :default "None"))
  (bind _buildgamemode (Variables|Default|GetBuildGameMode))
  (bind _selected_ship_part (Variables|/Game/Blueprints/ShipBuilder/BP_ShipBuilderGameMode.BP_ShipBuilderGameMode_C|GetSelected%20Ship%20Part _buildgamemode))
  ;[1 1 1] ENTER move mode of currently selected piece
  (:Pressed
    (if (not (Utilities|Enum|Equal(Enum) (Variables|/Game/Blueprints/ShipBuilder/BP_ShipBuilderGameMode.BP_ShipBuilderGameMode_C|Get2DCursorMode _buildgamemode) "NewEnumerator1"))
      (Utilities|IsValid _selected_ship_part
        (:Is%20Valid
          (Default|GMAttempttoRemoveCurrentPartfromShip (Variables|Default|GetBuildGameMode))
          (Default|SetIsMoving _selected_ship_part true)
          (Default|UnsetAllConnectionSlots _selected_ship_part)
          (Default|GMSet2DCursor (Variables|Default|GetBuildGameMode) "NewEnumerator1"))))))

(event Input|ActionEvents|InputActionBuildDelete
  (params (Key :type Key%20Structure :default "None"))
  (bind _buildgamemode (Variables|Default|GetBuildGameMode))
  ;[1 1 1] DELETE ship part
  (:Pressed
    (Utilities|IsValid _buildgamemode
      (:Is%20Valid
        (Utilities|IsValid (Variables|/Game/Blueprints/ShipBuilder/BP_ShipBuilderGameMode.BP_ShipBuilderGameMode_C|GetSelected%20Ship%20Part _buildgamemode)
          (:Is%20Valid
            (Default|GMAttempttoRemoveCurrentPartfromShip _buildgamemode)
            (Default|RemoveCurrentPartfromEditor _buildgamemode)))))))

(event Input|AxisEvents|InputAxisBuildCameraUp
  (params (AxisValue :type Float%20%28single-precision%29))
  ;[1 1 1] WASD Camera Buttons
  (Transformation|AddActorLocalRotation (Game|Player|GetPlayerPawn 0) (Math|Rotator|MakeRotator 0.0 AxisValue 0.0) false false))

(event Input|AxisEvents|InputAxisBuildCameraDown
  (params (AxisValue :type Float%20%28single-precision%29))
  ;[1 1 1] WASD Camera Buttons
  (Transformation|AddActorLocalRotation (Game|Player|GetPlayerPawn 0) (Math|Rotator|MakeRotator 0.0 AxisValue 0.0) false false))

(event Input|AxisEvents|InputAxisBuildCameraLeft
  (params (AxisValue :type Float%20%28single-precision%29))
  ;[1 1 1] WASD Camera Buttons
  (Class|Actor|AddActorWorldRotation (Game|Player|GetPlayerPawn 0) (Math|Rotator|MakeRotator 0.0 0.0 AxisValue)))

(event Input|AxisEvents|InputAxisBuildCameraRight
  (params (AxisValue :type Float%20%28single-precision%29))
  ;[1 1 1] WASD Camera Buttons
  (Class|Actor|AddActorWorldRotation (Game|Player|GetPlayerPawn 0) (Math|Rotator|MakeRotator 0.0 0.0 AxisValue)))

(event Input|MouseEvents|LeftMouseButton
  (params (Key :type Key%20Structure :default "None"))
  (bind _buildgamemode (Variables|Default|GetBuildGameMode))
  ;[1 1 1] Left Mouse Click
  (:Pressed
    (switch Utilities|FlowControl|Switch|SwitchonBP_CursorModeEnum (Variables|/Game/Blueprints/ShipBuilder/BP_ShipBuilderGameMode.BP_ShipBuilderGameMode_C|Get2DCursorMode _buildgamemode)
      (:NewEnumerator1
        (Default|AddParttoShip _buildgamemode)))))

(event Input|MouseEvents|RightMouseButton
  (params (Key :type Key%20Structure :default "None"))
  ;[1 1 1] Right Mouse Click
  (:Pressed
    (Default|RotateBuildingPiece (Variables|Default|GetBuildGameMode) (Math|Rotator|MakeRotator 0.0 0.0 (Variables|Default|GetRotationAmount)))))

(fn ConstructionScript)

(fn SetMouseCursor
  (params (Cursor%20Mode :type BP_CursorModeEnum%20Enum :default "NewEnumerator2"))
  (switch Utilities|FlowControl|Switch|SwitchonBP_CursorModeEnum Cursor%20Mode
    (:NewEnumerator2
      (Variables|Default|SetCurrentMouseCursor "Hand"))
    (:NewEnumerator0
      (Variables|Default|SetCurrentMouseCursor "GrabHand"))
    (:NewEnumerator1
      (Variables|Default|SetCurrentMouseCursor "GrabHandClosed"))))