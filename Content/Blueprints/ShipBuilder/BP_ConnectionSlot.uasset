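; Ship builder connection slot Blueprint that tracks whether it is linked to another slot.
; Construction sizes its collision sphere as a small fraction of the GameInstance's BuildDistanceX.
; Set and Unset functions mirror each change onto the partner slot, using the IsConnected check to end the mutual recursion.
; It has no active event logic.
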(event EventBeginPlay)

(event Collision|EventActorBeginOverlap
  (params (OtherActor :type Actor%20Object%20Reference)))

(event EventTick
  (params (DeltaSeconds :type Float%20%28single-precision%29)))

(fn ConstructionScript
  (bind _asbp_game_instance (Utilities|Casting|CastToBP_GameInstance (Game|GetGameInstance)))
  (Variables|Default|SetGameInstance _asbp_game_instance)
  (Components|Sphere|SetSphereRadius (Variables|Default|GetCollision%20Sphere) (* (Variables|/Game/Blueprints/AllLevels/BP_GameInstance.BP_GameInstance_C|GetBuild%20Distance%20X (Variables|Default|GetGameInstance)) 0.01) true))

(fn SetConnectionSlot
  (params (Connected%20To%20Slot :type BP%20Connection%20Slot%20Object%20Reference))
  (if (not (Variables|Default|GetIsConnected))
    (Variables|Default|SetIsConnected true)
    (Utilities|IsValid Connected%20To%20Slot
      (:Is%20Valid
        (CallFunction|SetConnectionSlot Connected%20To%20Slot self)
        (Variables|Default|SetConnectedToSlot Connected%20To%20Slot)))))

(fn UnsetConnectionSlot
  (if (Variables|Default|GetIsConnected)
    (Variables|Default|SetIsConnected false)
    (Utilities|IsValid (Variables|Default|GetConnectedToSlot)
      (:Is%20Valid
        (CallFunction|UnsetConnectionSlot (Variables|Default|GetConnectedToSlot))
        (Variables|Default|SetConnectedToSlot 0)))))