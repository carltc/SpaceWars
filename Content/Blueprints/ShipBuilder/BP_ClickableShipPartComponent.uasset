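; Actor component that makes its owning BP_ShipPart clickable and hoverable in the ship builder.
; When IsClickable is set, at BeginPlay or later through SetIsClickable, it binds the owner's click and cursor-over events.
; Clicks in the Selecting or Hovering cursor modes set the part as selected in the ship builder game mode.
; Cursor enter and exit pass the hover state to the part.
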(event Custom|OnMouseClick
  (params (TouchedActor :type Actor%20Object%20Reference) (ButtonPressed :type Key%20Structure))
  (bind _shippartref (Variables|Default|GetShipPartRef))
  (bind _shippartref_2 (Variables|Default|GetShipPartRef))
  (bind _shipbuildergamemode (Variables|/Game/Blueprints/Ship/ShipPart/BP_ShipPart.BP_ShipPart_C|GetShipBuilderGameMode _shippartref))
  ;[1 1 1] On Mouse Click
  (Utilities|IsValid _shippartref_2
    (:Is%20Valid
      (switch Utilities|FlowControl|Switch|SwitchonBP_CursorModeEnum (Variables|/Game/Blueprints/ShipBuilder/BP_ShipBuilderGameMode.BP_ShipBuilderGameMode_C|Get2DCursorMode (Variables|/Game/Blueprints/Ship/ShipPart/BP_ShipPart.BP_ShipPart_C|GetShipBuilderGameMode _shippartref_2))
        (:NewEnumerator2
          _)
        (:NewEnumerator0
          _))
      (Utilities|IsValid _shipbuildergamemode
        (:Is%20Valid
          (Default|GMSetSelectedShipPart _shipbuildergamemode _shippartref))))))

(event Custom|OnMouseHoverBegin
  (params (TouchedActor :type Actor%20Object%20Reference))
  ;[1 1 1] On Mouse Hover
  (Variables|Default|SetIsHovered true)
  (Utilities|IsValid (Variables|Default|GetShipPartRef)
    (:Is%20Valid
      (Default|SetHovered (Variables|Default|GetShipPartRef) (Variables|Default|GetIsHovered)))))

(event Custom|OnMouseHoverEnd
  (params (TouchedActor :type Actor%20Object%20Reference))
  ;[1 1 1] On Mouse Hover
  (Variables|Default|SetIsHovered false)
  (Utilities|IsValid (Variables|Default|GetShipPartRef)
    (:Is%20Valid
      (Default|SetHovered (Variables|Default|GetShipPartRef) (Variables|Default|GetIsHovered)))))

(event Custom|Initialise%20Clickableness
  (bind _returnvalue (Components|GetOwner))
  (if (Variables|Default|GetIsClickable)
    (bind _asbp_ship_part (Utilities|Casting|CastToBP_ShipPart _returnvalue))
    (Variables|Default|SetShipPartRef _asbp_ship_part)
    (Utilities|FlowControl|Sequence
      (:then_0
        ;[1 1 1] On Mouse Click
        (EventDispatchers|BindEventtoOnClicked _returnvalue (delegate Custom|OnMouseClick)))
      (:then_1
        ;[1 1 1] On Mouse Hover
        (EventDispatchers|BindEventtoOnBeginCursorOver _returnvalue (delegate Custom|OnMouseHoverBegin)))
      (:then_2
        (EventDispatchers|BindEventtoOnEndCursorOver _returnvalue (delegate Custom|OnMouseHoverEnd))))))

(event EventBeginPlay
  (CallFunction|InitialiseClickableness))

(fn SetIsClickable
  (Variables|Default|SetIsClickable true)
  (CallFunction|InitialiseClickableness))