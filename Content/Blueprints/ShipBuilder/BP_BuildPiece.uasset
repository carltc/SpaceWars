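; BP_BuildPiece is a grid-sized ship-builder piece that builds its collision and connection slots on BeginPlay.
; Slot counts, plate height and GameInstance build distances size a slightly inset, query-only box offset from a computed origin.
; The same grid places one slot type at plate-height Z and the other at base Z.
; Tick draws color-coded debug circles at each slot, and clicking prints the actor's name.
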(event EventBeginPlay
  ;[1 1 1] Set the Slots Origin
  (CallFunction|SetupSlotsOrigin (Variables|SlotOrigin|GetRelative%20Slots%20Origin))
  ;[1 1 1] Generate collision box
  (CallFunction|GenerateBoxCollision)
  ;[1 1 1] Generate Build Piece Connection Slots
  (CallFunction|GenerateBuildSlots))

(event Collision|EventActorBeginOverlap
  (params (OtherActor :type Actor%20Object%20Reference)))

(event EventTick
  (params (DeltaSeconds :type Float%20%28single-precision%29))
  (for _array_element (Actor|GetComponentsByClass "/Game/Blueprints/ShipBuilder/BuildPieceConnectionSlot.BuildPieceConnectionSlot_C")
    (if (Utilities|Enum|Equal(Enum) (Variables|/Game/Blueprints/ShipBuilder/BuildPieceConnectionSlot.BuildPieceConnectionSlot_C|GetSlotType _array_element) "NewEnumerator0")
      (Rendering|Debug|DrawDebugCircle (+ (Transformation|GetWorldLocation _array_element) "0, 0,1.000000") 4.0 20 "(R=1.000000,G=0.030067,B=0.000000,A=1.000000)" 0.0 0.2 "0.000000,1.000000,0.000000" "1.000000,0.000000,0.000000")
      (else
        (Rendering|Debug|DrawDebugCircle (+ (Transformation|GetWorldLocation _array_element) "0, 0,0.000000") 4.0 20 "(R=0.028321,G=0.000000,B=1.000000,A=1.000000)" 0.0 0.2 "0.000000,1.000000,0.000000" "1.000000,0.000000,0.000000")))))

(event MouseInput|EventActorOnClicked
  (params (ButtonPressed :type Key%20Structure :default "None"))
  (Development|PrintString (Utilities|GetDisplayName self)))

(fn ConstructionScript)

(fn SetupSlotsOrigin
  (params (Slots%20Origin :type Vector))
  (bind _returnvalue (Game|GetGameInstance))
  (bind (_x _y _z) (Math|Vector|BreakVector Slots%20Origin))
  (bind _asbp_game_instance (Utilities|Casting|CastToBP_GameInstance _returnvalue))
  (Variables|Default|SetRelative%20Euclidean%20Origin (Math|Vector|MakeVector (* (Variables|/Game/Blueprints/AllLevels/BP_GameInstance.BP_GameInstance_C|GetBuild%20Distance%20X _asbp_game_instance) _x) (* (Variables|/Game/Blueprints/AllLevels/BP_GameInstance.BP_GameInstance_C|GetBuild%20Distance%20Y _asbp_game_instance) _y) (* (Variables|/Game/Blueprints/AllLevels/BP_GameInstance.BP_GameInstance_C|GetBuild%20Distance%20Z _asbp_game_instance) _z))))

(fn GenerateBoxCollision
  (bind _asbp_game_instance (Utilities|Casting|CastToBP_GameInstance (Game|GetGameInstance))
    (:then
      (bind _returnvalue (AddComponent|AddBoxComponent true (Math|Transform|MakeTransform "0, 0, 0")))
      (Development|SetHiddeninGame _returnvalue false true)
      (Transformation|AttachComponentToComponent _returnvalue (Variables|Default|GetStaticMesh) "None" "KeepRelative" "KeepRelative" "KeepRelative" true)
      (Transformation|SetRelativeLocation _returnvalue (- (Variables|Default|GetRelative%20Euclidean%20Origin) (Math|Vector|MakeVector (* (Variables|/Game/Blueprints/AllLevels/BP_GameInstance.BP_GameInstance_C|GetBuild%20Distance%20X _asbp_game_instance) (/ (Math|Conversions|ToFloat(Integer) (- (Variables|SlotOrigin|GetSlots%20X) 1)) 2.0)) (* (Variables|/Game/Blueprints/AllLevels/BP_GameInstance.BP_GameInstance_C|GetBuild%20Distance%20Y _asbp_game_instance) (/ (Math|Conversions|ToFloat(Integer) (- (Variables|SlotOrigin|GetSlots%20Y) 1)) 2.0)) (* (Variables|/Game/Blueprints/AllLevels/BP_GameInstance.BP_GameInstance_C|GetBuild%20Distance%20Z _asbp_game_instance) (/ (Math|Conversions|ToFloat(Integer) (Variables|SlotOrigin|GetPlate%20Height)) -2.0)))) false false)
      (Components|Box|SetBoxExtent _returnvalue (* (Math|Vector|MakeVector (* (Variables|SlotOrigin|GetSlots%20X) (Variables|/Game/Blueprints/AllLevels/BP_GameInstance.BP_GameInstance_C|GetBuild%20Distance%20X _asbp_game_instance)) (* (Variables|SlotOrigin|GetSlots%20Y) (Variables|/Game/Blueprints/AllLevels/BP_GameInstance.BP_GameInstance_C|GetBuild%20Distance%20Y _asbp_game_instance)) (* (Variables|SlotOrigin|GetPlate%20Height) (Variables|/Game/Blueprints/AllLevels/BP_GameInstance.BP_GameInstance_C|GetBuild%20Distance%20Z _asbp_game_instance))) 0.49) true)
      (Collision|SetCollisionEnabled _returnvalue "QueryOnly")
      (return true))
    (:CastFailed
      (return false))))

(fn AddBuildSlots
  (params (Build%20Slot%20Type :type BuildSlotType%20Enum :default "NewEnumerator0"))
  (bind _returnvalue (Game|GetGameInstance))
  (bind _returnvalue_2 (Game|GetGameInstance))
  (bind _visualisation_scale (Variables|Default|GetVisualisation%20Scale))
  (bind _visualisation_scale_2 (Variables|Default|GetVisualisation%20Scale))
  (bind _asbp_game_instance (Utilities|Casting|CastToBP_GameInstance _returnvalue))
  (bind _asbp_game_instance_2 (Utilities|Casting|CastToBP_GameInstance _returnvalue_2))
  (for _index (range 0 (- (Variables|SlotOrigin|GetSlots%20X) 1))
    (for _index_2 (range 0 (- (Variables|SlotOrigin|GetSlots%20Y) 1))
      (if (Utilities|Enum|Equal(Enum) Build%20Slot%20Type "NewEnumerator0")
        (AddComponent|AddBuildPieceConnectionSlot false (Math|Transform|MakeTransform (- (Variables|Default|GetRelative%20Euclidean%20Origin) (Math|Vector|MakeVector (* _index (Variables|/Game/Blueprints/AllLevels/BP_GameInstance.BP_GameInstance_C|GetBuild%20Distance%20X _asbp_game_instance_2)) (* _index_2 (Variables|/Game/Blueprints/AllLevels/BP_GameInstance.BP_GameInstance_C|GetBuild%20Distance%20Y _asbp_game_instance_2)) (* (Variables|SlotOrigin|GetPlate%20Height) (* (Variables|/Game/Blueprints/AllLevels/BP_GameInstance.BP_GameInstance_C|GetBuild%20Distance%20Z _asbp_game_instance_2) -1.0)))) "0, 0, 0" (Math|Vector|MakeVector _visualisation_scale _visualisation_scale _visualisation_scale)) "NewEnumerator0")
        (else
          (AddComponent|AddBuildPieceConnectionSlot false (Math|Transform|MakeTransform (- (Variables|Default|GetRelative%20Euclidean%20Origin) (Math|Vector|MakeVector (* _index (Variables|/Game/Blueprints/AllLevels/BP_GameInstance.BP_GameInstance_C|GetBuild%20Distance%20X _asbp_game_instance)) (* _index_2 (Variables|/Game/Blueprints/AllLevels/BP_GameInstance.BP_GameInstance_C|GetBuild%20Distance%20Y _asbp_game_instance)) 0.0)) "0, 0, 0" (Math|Vector|MakeVector _visualisation_scale_2 _visualisation_scale_2 _visualisation_scale_2)) "NewEnumerator1"))))))

(fn GenerateBuildSlots
  (CallFunction|AddBuildSlots "NewEnumerator0")
  (CallFunction|AddBuildSlots "NewEnumerator1"))