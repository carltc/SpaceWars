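; BP_RepairPickup is a pickup that restores one missing part on the ship of the player who collects it.
; Its OnPickup override scans the ship's ShipParts for the first invalid entry and respawns that part from the matching ShipInfo data via CLIENTSSpawnPartOnShip.
; It sets PickedUp and stops after that single repair, returning PickedUp as the result.
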(event EventBeginPlay
  (|CallParentFunction) ; This node is disabled and will not be called.\nDrag off pins to build functionality.
)

(event Collision|EventActorBeginOverlap
  (params (OtherActor :type Actor%20Object%20Reference))
  (|CallParentFunction OtherActor) ; This node is disabled and will not be called.\nDrag off pins to build functionality.
)

(event EventTick
  (params (DeltaSeconds :type Float%20%28single-precision%29))
  (|CallParentFunction DeltaSeconds) ; This node is disabled and will not be called.\nDrag off pins to build functionality.
)

(fn ConstructionScript
  (|CallParentFunction))

(fn OnPickup
  (params (Player%20Who%20Picked%20Up :type BP%20Match%20Player%20Pawn%20Object%20Reference))
  (bind _customshipref (Variables|/Game/Blueprints/Match/BP_MatchPlayerPawn.BP_MatchPlayerPawn_C|GetCustomShipRef Player%20Who%20Picked%20Up))
  (bind (_array_element _array_index) (Utilities|Array|ForEachLoopwithBreak (Variables|/Game/Blueprints/Ship/BP_CustomShip.BP_CustomShip_C|GetShipParts _customshipref) :!label _label)
    (:LoopBody
      (Utilities|IsValid _array_element
        (:Is%20Not%20Valid
          (Default|CLIENTSSpawnPartonShip _customshipref (Utilities|Array|Get(acopy) (.ShipParts (Utilities|Struct|BreakShipInfo (Variables|/Game/Blueprints/Ship/BP_CustomShip.BP_CustomShip_C|GetShipInfo _customshipref))) _array_index) _array_index)
          (LocalVariables|SetPickedUp true)
          (goto _label Break))))
    (:Completed
      (return (LocalVariables|GetPickedUp)))))