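; BP_Pickup is a base pickup actor that is collected when a ship part touches its sphere.
; On overlap it follows the ship part's parent ship to the owning pawn and proceeds only if that is a BP_MatchPlayerPawn.
; It passes that pawn to OnPickup, which is an empty hook here, then destroys the PickupActor child actor and itself.
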(event OnComponentBeginOverlap(Sphere)
  (params (OverlappedComponent :type Primitive%20Component%20Object%20Reference) (OtherActor :type Actor%20Object%20Reference) (OtherComp :type Primitive%20Component%20Object%20Reference) (OtherBodyIndex :type Integer) (bFromSweep :type Boolean) (SweepResult :type Hit%20Result%20Structure%20%28by%20ref%29))
  ;[1 1 1] CHECK if this is a valid pickup by a pawn
  (bind _asbp_ship_part (Utilities|Casting|CastToBP_ShipPart OtherActor))
  (Utilities|IsValid (Variables|/Game/Blueprints/Ship/ShipPart/BP_ShipPart.BP_ShipPart_C|GetParentShipRef _asbp_ship_part)
    (:Is%20Valid
      (Utilities|IsValid (Variables|/Game/Blueprints/Ship/BP_Ship.BP_Ship_C|GetParentPawnRef (Variables|/Game/Blueprints/Ship/ShipPart/BP_ShipPart.BP_ShipPart_C|GetParentShipRef _asbp_ship_part))
        (:Is%20Valid
          (bind _asbp_match_player_pawn (Utilities|Casting|CastToBP_MatchPlayerPawn (Variables|/Game/Blueprints/Ship/BP_Ship.BP_Ship_C|GetParentPawnRef (Variables|/Game/Blueprints/Ship/ShipPart/BP_ShipPart.BP_ShipPart_C|GetParentShipRef _asbp_ship_part))))
          ;[1 1 1] RUN pickup logic
          (CallFunction|OnPickup _asbp_match_player_pawn)
          ;[1 1 1] DESTROY pickup after it has been picked up
          (Actor|DestroyActor (Variables|/Script/Engine.ChildActorComponent|GetChildActor (Variables|Default|GetPickupActor)))
          (Actor|DestroyActor))))))

(event EventBeginPlay)

(event Collision|EventActorBeginOverlap
  (params (OtherActor :type Actor%20Object%20Reference)))

(event EventTick
  (params (DeltaSeconds :type Float%20%28single-precision%29)))

(fn ConstructionScript)

(fn OnPickup
  (params (Player%20Who%20Picked%20Up :type BP%20Match%20Player%20Pawn%20Object%20Reference)))