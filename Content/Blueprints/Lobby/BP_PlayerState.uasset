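; Lobby player state Blueprint that respawns the player through its RespawnPlayer event.
; After a short delay it spawns a BP_Pawn_Base at a random PlayerStart, prints its name and has player controller 0 possess it.
; The random index is bounded by the array length minus one, so the last PlayerStart found is never picked.
; An unconnected slow-motion time dilation node never runs.
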(event Custom|RespawnPlayer
  (Utilities|FlowControl|Delay 0.2)
  (bind _outactors (Actor|GetAllActorsOfClass "/Script/Engine.PlayerStart"))
  (bind _returnvalue (Game|SpawnActorfromClass "/Game/Deprecated/BP_Pawn_Base.BP_Pawn_Base_C" (Transformation|GetActorTransform (Utilities|Array|Get(acopy) _outactors (Math|Random|RandomInteger (- (Utilities|Array|Length _outactors) 1)))) "Undefined" 0 0))
  (Development|PrintString (Utilities|String|Append "Spawned new: " (Utilities|GetDisplayName _returnvalue)))
  (Pawn|Possess (Game|GetPlayerController 0) _returnvalue))

(event EventBeginPlay)

(event EventTick
  (params (DeltaSeconds :type Float%20%28single-precision%29)))

(fn ConstructionScript)