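; BP_Projectile is a projectile that damages or notifies ship parts it overlaps and expires after a maximum range.
; Tick estimates distance from max speed and, if nothing was hit, requests destruction through a server event relayed to a clients event.
; On authority, capsule overlaps pass the projectile to the hit BP_ShipPart, ignoring the owning player's own ship.
; ProjectileHitSomething sets the flag that suppresses range-based destruction.
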(event OnComponentBeginOverlap(Capsule)
  (params (OverlappedComponent :type Primitive%20Component%20Object%20Reference) (OtherActor :type Actor%20Object%20Reference) (OtherComp :type Primitive%20Component%20Object%20Reference) (OtherBodyIndex :type Integer) (bFromSweep :type Boolean) (SweepResult :type Hit%20Result%20Structure%20%28by%20ref%29))
  ;[1 1 1] HIT
  (Networking|SwitchHasAuthority
    (:Authority
      (bind _asbp_ship_part (Utilities|Casting|CastToBP_ShipPart OtherActor))
      (if (not (== (Variables|/Game/Blueprints/Ship/BP_Ship.BP_Ship_C|GetParentPawnRef (Variables|/Game/Blueprints/Ship/ShipPart/BP_ShipPart.BP_ShipPart_C|GetParentShipRef _asbp_ship_part)) (Variables|/Script/Engine.PlayerState|GetPawnPrivate (Variables|Default|GetOwningPlayerStateRef))))
        (Default|SERVERHitbyProjectile _asbp_ship_part self)))))

(event Custom|SERVER_DestroyProjectile
  ;[1 1 1] SERVER destroy projectile
  (CallFunction|CLIENTSDestroyProjectile))

(event Custom|CLIENTS_DestroyProjectile
  ;[1 1 1] SERVER destroy projectile
  (Variables|Default|SetDestroyed true)
  ;;[1 1 1] DESTROY actor
  (Actor|DestroyActor))

(event EventTick
  (params (DeltaSeconds :type Float%20%28single-precision%29))
  ;[1 1 1] TICK
  ;;[1 1 1] UPDATE distance travelled of projectile
  (bind _output_get (Variables|Default|SetDistanceTravelled (+ (Variables|Default|GetDistanceTravelled) (* DeltaSeconds (Class|MovementComponent|GetMaxSpeed (Variables|Default|GetProjectileMovement))))))
  ;;[1 1 1] CHECK if projectile has reached max distance and has not yet hit anything
  (if (Math|Boolean|ANDBoolean (>= _output_get (Variables|Default|GetMaxDistanceToTravel)) (not (Variables|Default|GetHitSomething)) (not (Variables|Default|GetDestroyed)))
    (CallFunction|SERVERDestroyProjectile)))

(event EventDestroyed
  (Development|PrintString "I was destroyed"))

(fn ConstructionScript)

(fn ProjectileHitSomething
  (Variables|Default|SetHitSomething true))