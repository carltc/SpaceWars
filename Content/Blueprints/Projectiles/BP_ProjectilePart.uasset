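; BP_ProjectilePart is a projectile that knocks parts off enemy custom ships.
; On the authority, its capsule overlap finds the hit BP_ShipPart's parent ship and ignores hits on the owning ship.
; A hit on another ship enables physics on the part's mesh and flags both part and projectile destroyed.
; Tick then destroys the projectile after a delay, with debug prints reporting overlap results.
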(event OnComponentBeginOverlap(Capsule)
  (params (OverlappedComponent :type Primitive%20Component%20Object%20Reference) (OtherActor :type Actor%20Object%20Reference) (OtherComp :type Primitive%20Component%20Object%20Reference) (OtherBodyIndex :type Integer) (bFromSweep :type Boolean) (SweepResult :type Hit%20Result%20Structure%20%28by%20ref%29))
  (Networking|SwitchHasAuthority
    (:Authority
      (bind _asbp_ship_part (Utilities|Casting|CastToBP_ShipPart OtherActor))
      ;[1 1 1] Check if same part was hit
      (bind _asbp_custom_ship (Utilities|Casting|CastToBP_CustomShip (Actor|GetParentActor _asbp_ship_part)))
      (bind _asbp_custom_ship_2 (Utilities|Casting|CastToBP_CustomShip (Components|GetOwner))
        (:then
          (if (== _asbp_custom_ship_2 _asbp_custom_ship)
            (Development|PrintString "HIT same ship")
            (else
              (Development|PrintString (Utilities|String|Append "HIT: " (Utilities|GetDisplayName _asbp_custom_ship)))
              (Physics|SetSimulatePhysics (Variables|/Game/Blueprints/ShipBuilder/BP_ShipPart.BP_ShipPart_C|GetStaticMesh _asbp_ship_part) true)
              (Variables|Default|SetIsDestroyed true)
              (Variables|/Game/Blueprints/ShipBuilder/BP_ShipPart.BP_ShipPart_C|SetIsDestroyed _asbp_ship_part true))))
        (:CastFailed
          (Development|PrintString "FAILED to cast"))))))

(event EventTick
  (params (DeltaSeconds :type Float%20%28single-precision%29))
  ;[1 1 1] EVENT tick
  (if (Variables|Default|GetIsDestroyed)
    (if (< (Variables|Default|GetDestroyedTimer) (Variables|Default|GetDestroyDelayTime))
      (Variables|Default|SetDestroyedTimer (+ (Variables|Default|GetDestroyedTimer) DeltaSeconds))
      (else
        (Actor|DestroyActor)))))

(fn ConstructionScript)