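; Match game mode that registers joining players, starts their controller setup and handles respawns.
; Respawning destroys the current pawn and restarts the player at a PlayerStart from GetAPlayerStart, which also serves ChoosePlayerStart.
; Each call spawns a new PlayerStart at a random location and yaw; the tag-based search for free existing starts is disconnected.
; It also relays player score additions to client HUDs through BP_MatchGameState and looks up controllers by PlayerID.
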(event Custom|GM_Respawn
  (params (Player%20Controller :type Player%20Controller%20Object%20Reference))
  (bind _returnvalue (Pawn|GetControlledPawn Player%20Controller))
  ;[1 1 1] RESPAWN Player
  (Utilities|IsValid _returnvalue
    (:Is%20Valid
      (Actor|DestroyActor _returnvalue))
    (:Is%20Not%20Valid
      _))
  (bind _chosen_player_start (CallFunction|GetAPlayerStart))
  (Class|GameModeBase|RestartPlayeratPlayerStart Player%20Controller _chosen_player_start))

(event Custom|GM_AddPlayerScoreToAllClientHUDs
  (params (PlayerState :type BP%20Match%20Player%20State%20Object%20Reference))
  ;[1 1 1] ADD player score to all clients
  (bind _asbp_match_game_state (Utilities|Casting|CastToBP_MatchGameState (Game|GetGameState)))
  (Default|GSAddPlayerScoretoAllClients _asbp_match_game_state PlayerState))

(event EventPostLogin
  (params (NewPlayer :type Player%20Controller%20Object%20Reference))
  ;[1 1 1] ADD PLAYER when they login
  (Utilities|Array|Add (Variables|Default|GetAllPlayerControllers) NewPlayer)
  (bind _asbp_match_player_controller (Utilities|Casting|CastToBP_MatchPlayerController NewPlayer))
  (Default|PCInitialSetup _asbp_match_player_controller))

(fn ConstructionScript)

(fn ChoosePlayerStart
  (params (Player :type Controller%20Object%20Reference))
  (bind _chosen_player_start (CallFunction|GetAPlayerStart))
  (return _chosen_player_start))

(fn GetAPlayerStart
  (bind _returnvalue (Math|Random|RandomFloat))
  ;[1 1 1] RANDOM player start position
  (bind _returnvalue_2 (Game|SpawnActorfromClass "/Script/Engine.PlayerStart" (Math|Transform|MakeTransform (Math|Vector|MakeVector (* 2000 _returnvalue) (* 2000 _returnvalue) 5e+02) (Math|Rotator|MakeRotator 0.0 0.0 (* 360 (Math|Random|RandomFloat)))) "Undefined" 0 0))
  (LocalVariables|SetPlayerStart _returnvalue_2)
  (return (LocalVariables|GetPlayerStart)))

(fn GetPlayerController
  (params (Player%20ID :type Guid%20Structure))
  (bind _array_element (Utilities|Array|ForEachLoopwithBreak (Variables|Default|GetAllPlayerControllers))
    (:LoopBody
      (bind _asbp_match_player_controller (Utilities|Casting|CastToBP_MatchPlayerController _array_element))
      (if (== (Variables|/Game/Blueprints/Match/BP_MatchPlayerController.BP_MatchPlayerController_C|GetPlayer%20ID _asbp_match_player_controller) Player%20ID)
        (return _asbp_match_player_controller)))
    (:Completed
      (return 0))))