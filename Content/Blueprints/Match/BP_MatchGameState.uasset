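; Game state for a ship match that times the round, opens the end map when match length elapses, and assigns a GUID match ID on construction.
; BeginPlay caches the game mode, player count and game instance, and sets a test match name.
; A score event rebuilds the first local player's ship HUD score panel from PlayerArray.
; A helper function increments a player controller's ships-destroyed count in its match result struct.
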(event Custom|GS_AddPlayerScoreToAllClients
  (params (PlayerState :type BP%20Match%20Player%20State%20Object%20Reference))
  (bind _returnvalue (Game|GetPlayerController 0))
  (bind _returnvalue_2 (HUD|GetHUD _returnvalue))
  ;[1 1 1] ADD player score to all clients
  (Utilities|IsValid _returnvalue_2
    (:Is%20Valid
      (bind _asbp_ship_hud (Utilities|Casting|CastToBP_ShipHUD _returnvalue_2))
      (Utilities|IsValid (Variables|/Game/UI/Match/BP_ShipHUD.BP_ShipHUD_C|GetShipHUDWidgetRef _asbp_ship_hud)
        (:Is%20Valid
          (Default|ClearPlayerScoreEntries (Variables|/Game/UI/Match/BP_ShipHUD.BP_ShipHUD_C|GetShipHUDWidgetRef _asbp_ship_hud))
          (for _array_element (Variables|Default|GetPlayerArray)
            (bind _asbp_match_player_state (Utilities|Casting|CastToBP_MatchPlayerState _array_element))
            (Default|AddPlayerScoretoPanel (Variables|/Game/UI/Match/BP_ShipHUD.BP_ShipHUD_C|GetShipHUDWidgetRef _asbp_ship_hud) _asbp_match_player_state)))))))

(event EventBeginPlay
  ;[1 1 1] Begin
  (Utilities|FlowControl|Sequence
    (:then_0
      (bind _asbp_match_game_mode (Utilities|Casting|CastToBP_MatchGameMode (Game|GetGameMode)))
      (bind _output_get (Variables|Default|SetMatchGameMode _asbp_match_game_mode))
      (bind _returnvalue (Class|GameModeBase|GetNumPlayers _output_get))
      (Variables|Default|SetNumPlayers _returnvalue))
    (:then_1
      (bind _asbp_game_instance (Utilities|Casting|CastToBP_GameInstance (Game|GetGameInstance)))
      (Variables|Default|SetGameInstance _asbp_game_instance))
    (:then_2
      (bind _output_get_2 (Variables|Default|SetMatch%20Name "TestMatch"))
      (Development|PrintString (Utilities|String|Append "New match started: " _output_get_2)))))

(event EventTick
  (params (DeltaSeconds :type Float%20%28single-precision%29))
  ;[1 1 1] Tick
  (Variables|Default|SetElapsedTime (+ (Variables|Default|GetElapsedTime) DeltaSeconds))
  (if (>= (Variables|Default|GetElapsedTime) (Math|Conversions|ToFloat(Integer) (Variables|Default|GetMatchLength)))
    (Utilities|FlowControl|Delay 0.2)
    (Game|OpenLevel(byName) (Variables|Default|GetEndMapName))))

(fn ConstructionScript
  (Variables|Default|SetMatch_ID (Guid|NewGuid)))

(fn UpdatePlayerShipDestroyed
  (params (Player%20Controller :type BP%20Match%20Player%20Controller%20Object%20Reference))
  (bind _currentmatchstate (Variables|/Game/Blueprints/Match/BP_MatchPlayerController.BP_MatchPlayerController_C|GetCurrentMatchState Player%20Controller))
  (Utilities|Struct|SetmembersinMatchPlayerResult _currentmatchstate (+ (.ShipsDestroyed (Utilities|Struct|BreakMatchPlayerResult _currentmatchstate)) 1)))