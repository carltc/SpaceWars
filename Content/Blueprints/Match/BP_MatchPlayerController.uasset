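; Player controller for a match that loads the player's saved profile and ship info and sets up the possessed ship pawn.
; On BeginPlay it loads the profile save slot, writes it back if one existed, caches the game state and records a match result entry with zero ships destroyed.
; On possess it links the match pawn, runs its custom ship setup and has the game mode update all ships through a server event.
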(event Custom|PC_InitialSetup
  (CallFunction|SetupPlayerControllerforMatch))

(event Custom|SERVER_UpdateAllShips
  (bind _matchgamemode (Variables|Default|GetMatchGameMode))
  (Utilities|IsValid _matchgamemode
    (:Is%20Valid
      (Default|SERVERUpdateAllShips _matchgamemode))
    (:Is%20Not%20Valid
      (Development|PrintString "MatchPlayerController: Match Game Mode invalid." true true "(R=0.000000,G=0.660000,B=1.000000,A=1.000000)" 3e+01))))

(event EventBeginPlay
  (CallFunction|SetupPlayerControllerforMatch))

(event EventPossess
  (params (PossessedPawn :type Pawn%20Object%20Reference))
  (bind _asbp_match_player_pawn (Utilities|Casting|CastToBP_MatchPlayerPawn PossessedPawn)
    (:then
      (bind _output_get (Variables|Default|SetMatchPawnRef _asbp_match_player_pawn))
      (Variables|/Game/Blueprints/Match/BP_MatchPlayerPawn.BP_MatchPlayerPawn_C|SetMatchPlayerControllerRef _output_get self)
      (Default|SetupCustomShipforMatch _output_get))
    (:CastFailed
      _))
  (CallFunction|SERVERUpdateAllShips))

(fn ConstructionScript
  (Utilities|FlowControl|Sequence
    (:then_0
      (bind _asbp_match_game_mode (Utilities|Casting|CastToBP_MatchGameMode (Game|GetGameMode)))
      (Variables|Default|SetMatchGameMode _asbp_match_game_mode))
    (:then_1
      (bind _asbp_game_instance (Utilities|Casting|CastToBP_GameInstance (Game|GetGameInstance)))
      (Variables|Default|SetGameInstance _asbp_game_instance))))

(fn SetupPlayerControllerforMatch
  (Utilities|FlowControl|Sequence
    (:then_0
      (CallFunction|SaveGameCheck))
    (:then_1
      (bind _asbp_match_game_state (Utilities|Casting|CastToBP_MatchGameState (Game|GetGameState)))
      (Variables|Default|SetCurrentGameState _asbp_match_game_state))
    (:then_2
      (bind _returnvalue (Utilities|Array|Add (Variables|Default|GetPlayerMatchStates) (Utilities|Struct|MakeMatchPlayerResult (Variables|/Game/Blueprints/Match/BP_MatchGameState.BP_MatchGameState_C|GetMatch_ID (Variables|Default|GetCurrentGameState)) (Utilities|String|ToString(Text) (.MyPlayerName (Utilities|Struct|BreakPlayerInfo (Variables|Default|GetPlayerSettings)))))))
      (Variables|Default|SetCurrentMatchState (Utilities|Array|Get(acopy) (Variables|Default|GetPlayerMatchStates) _returnvalue)))))

(fn SaveGameCheck
  (bind _returnvalue (SaveGame|DoesSaveGameExist (Variables|Default|GetPlayerSettingsSave)))
  (if _returnvalue
    (CallFunction|LoadGame)
    (CallFunction|SaveGame)
    (else
      (CallFunction|LoadGame))))

(fn LoadGame
  (bind _returnvalue (SaveGame|LoadGamefromSlot (Variables|Default|GetPlayerSettingsSave)))
  (bind _asbp_profile_save_game (Utilities|Casting|CastToBP_ProfileSaveGame _returnvalue))
  (Utilities|Struct|SetmembersinPlayerInfo (Variables|Default|GetPlayerSettings) (.MyPlayerName (Utilities|Struct|BreakPlayerInfo (Variables|/Game/Blueprints/AllLevels/BP_ProfileSaveGame.BP_ProfileSaveGame_C|GetS_PlayerInfo _asbp_profile_save_game))) (.MyPlayerImage (Utilities|Struct|BreakPlayerInfo (Variables|/Game/Blueprints/AllLevels/BP_ProfileSaveGame.BP_ProfileSaveGame_C|GetS_PlayerInfo _asbp_profile_save_game))) 0 "/Game/Textures/DefaultShip.DefaultShip" "Not Ready!" (.CustomShipSaveGames (Utilities|Struct|BreakPlayerInfo (Variables|/Game/Blueprints/AllLevels/BP_ProfileSaveGame.BP_ProfileSaveGame_C|GetS_PlayerInfo _asbp_profile_save_game))))
  (Variables|Default|SetShipInfo (Variables|/Game/Blueprints/AllLevels/BP_ProfileSaveGame.BP_ProfileSaveGame_C|GetS_ShipInfo _asbp_profile_save_game))
  (Variables|Default|SetPlayerPawnClass "/Game/Blueprints/Match/BP_MatchPlayerPawn.BP_MatchPlayerPawn_C"))

(fn SaveGame
  (Utilities|IsValid (Variables|Default|GetPlayerSaveGame)
    (:Is%20Valid
      _)
    (:Is%20Not%20Valid
      (bind _returnvalue (SaveGame|CreateSaveGameObject "/Game/Blueprints/AllLevels/BP_ProfileSaveGame.BP_ProfileSaveGame_C"))
      (Variables|Default|SetPlayerSaveGame _returnvalue)))
  (Variables|/Game/Blueprints/AllLevels/BP_ProfileSaveGame.BP_ProfileSaveGame_C|SetS_PlayerInfo (Variables|Default|GetPlayerSaveGame) (Variables|Default|GetPlayerSettings))
  (Variables|/Game/Blueprints/AllLevels/BP_ProfileSaveGame.BP_ProfileSaveGame_C|SetS_PlayerPawn (Variables|Default|GetPlayerSaveGame) (Variables|Default|GetPlayerPawnClass))
  (Variables|/Game/Blueprints/AllLevels/BP_ProfileSaveGame.BP_ProfileSaveGame_C|SetS_ShipInfo (Variables|Default|GetPlayerSaveGame) (Variables|Default|GetShipInfo))
  (SaveGame|SaveGametoSlot (Variables|Default|GetPlayerSaveGame) (Variables|Default|GetPlayerSettingsSave)))