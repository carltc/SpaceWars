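; Multiplayer match pawn for a player's modular custom ship, handling flight, shooting, part damage, destruction and respawn.
; Ship stats drive maneuverability, fire rate and FloatingPawnMovement tuning, with roll inducing yaw and self-levelling without input.
; Authority tick calls an owner update that moves the pawn and pushes its transform to the server.
; Server events handle firing and respawn via the game mode; client events sync ship loadout, engine flames and part damage by index.
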(event Custom|Server_UpdatePawn
  (params (Location :type Vector) (Rotation :type Rotator))
  ;[1 1 1] UPDATE server
  (Transformation|SetActorTransform (Math|Transform|MakeTransform Location Rotation)))

(event Custom|SERVER_SpawnProjectiles
  (params (Owning%20Player%20State%20Ref :type BP%20Match%20Player%20State%20Object%20Reference))
  ;[1 1 1] SHOOT
  (Networking|SwitchHasAuthority
    (:Authority
      (for _array_element (Variables|/Game/Blueprints/Ship/BP_CustomShip.BP_CustomShip_C|GetWeaponParts (Variables|Ship|GetCustomShipRef))
        (Default|FireWeaponSlots _array_element Owning%20Player%20State%20Ref self)))))

(event Custom|SERVER_Respawn
  (params (PlayerController :type Player%20Controller%20Object%20Reference))
  ;[1 1 1] RESPAWN
  (CallFunction|CLIENTSSetPawnDestroyed)
  (Utilities|FlowControl|Delay 3.0)
  (Networking|SwitchHasAuthority
    (:Authority
      (Utilities|IsValid (Variables|Game|GetMatchGameMode)
        (:Is%20Valid
          (Default|GMRespawn (Variables|Game|GetMatchGameMode) PlayerController))
        (:Is%20Not%20Valid
          (bind _asbp_match_game_mode (Utilities|Casting|CastToBP_MatchGameMode (Game|GetGameMode)))
          (Default|GMRespawn _asbp_match_game_mode PlayerController))))))

(event Custom|CLIENTS_SetPawnDestroyed
  ;[1 1 1] CLIENTS Set pawn destroyed
  (CallFunction|SetPawnDestroyed))

(event Custom|CLIENTS_SetShipPartDestroyed
  (params (Ship%20Part%20Name :type String) (ShipPartIndex :type Integer))
  ;[1 1 1] CLIENTS set ship part destroyed
  (bind (_found _ship_part_ref) (CallFunction|GetShipPartfromIndex ShipPartIndex))
  (if _found
    (Default|SetShipPartDestroyed _ship_part_ref (Variables|SelfHit|GetLastHitVector))
    (Default|CSCalculateVehicleStats (Variables|Ship|GetCustomShipRef))
    (else
      (Development|PrintString "Part not found"))))

(event Custom|CLIENTS_UpdateShip
  (params (ShipInfo :type Ship%20Info%20Structure))
  (bind _customshipref (Variables|Ship|GetCustomShipRef))
  ;[1 1 1] CLIENTS swap the ship on all clients
  (bind _output_get (Variables|Default|SetShipInfo ShipInfo))
  (Utilities|IsValid _customshipref
    (:Is%20Valid
      (Variables|/Game/Blueprints/Ship/BP_CustomShip.BP_CustomShip_C|SetShipInfo _customshipref _output_get)
      (Default|LoadShip _customshipref))))

(event Custom|CLIENTS_ApplyDamage
  (params (ShipPartName :type String) (Damage :type Float%20%28single-precision%29) (ShipPartIndex :type Integer))
  ;[1 1 1] CLIENTS Set ship part colour on all clients
  (bind (_found _ship_part_ref) (CallFunction|GetShipPartfromIndex ShipPartIndex))
  (if _found
    (Default|ApplyDamage _ship_part_ref Damage)))

(event Custom|SERVER_SetEngineFlames
  (params (Engine%20On :type Boolean))
  ;[1 1 1] MOVEMENT Controls
  ;;[1 1 1] SERVER run on server to then set engine flames on clients
  (Networking|SwitchHasAuthority
    (:Authority
      (CallFunction|CLIENTSSetEngineFlames Engine%20On))))

(event Custom|CLIENTS_SetEngineFlames
  (params (Engine%20On :type Boolean))
  (bind _customshipref (Variables|Ship|GetCustomShipRef))
  ;[1 1 1] MOVEMENT Controls
  ;;[1 1 1] CLIENTS set engine flames on all clients
  (Utilities|IsValid _customshipref
    (:Is%20Valid
      (Default|SetEngineFlames _customshipref Engine%20On))))

(event Custom|OWNER_UpdatePawn
  (params (Delta%20Seconds :type Float%20%28single-precision%29))
  (bind _customshipref (Variables|Ship|GetCustomShipRef))
  ;[1 1 1] EVENT tick
  (Utilities|FlowControl|Sequence
    (:then_0
      (Utilities|IsValid _customshipref
        (:Is%20Valid
          (Pawn|Input|AddControllerYawInput (* (/ (.Roll (Math|Rotator|BreakRotator (Transformation|GetActorRotation))) 9e+01) (Variables|MovementCalibration|GetYawRate) (Variables|/Game/Blueprints/Ship/BP_ShipStats.BP_ShipStats_C|GetManeuverability (Variables|/Game/Blueprints/Ship/BP_Ship.BP_Ship_C|GetShipStats _customshipref)) Delta%20Seconds)))))
    (:then_1
      (Class|PawnMovementComponent|AddInputVector (Variables|Default|GetFloatingPawnMovement) (* (Transformation|GetActorForwardVector) (Variables|Movement|GetForwardInput)) false)
      (CallFunction|ServerUpdatePawn (Transformation|GetActorLocation) (Transformation|GetActorRotation)))
    (:then_2
      (Pawn|Input|AddControllerPitchInput (* (Variables|Movement|GetPitchInput) Delta%20Seconds))
      (Pawn|Input|AddControllerRollInput (* (Variables|Movement|GetRollInput) Delta%20Seconds)))
    (:then_3
      ;;[1 1 1] SET fire cooldown
      (if (> (Variables|Firing|GetFireCooldown) 0.0)
        (Variables|Firing|SetFireCooldown (- (Variables|Firing|GetFireCooldown) Delta%20Seconds))
        (else
          (Variables|Firing|SetFireCooldown 0.0))))))

(event EventTick
  (params (DeltaSeconds :type Float%20%28single-precision%29))
  ;[1 1 1] ONLY run TICK on owning client
  (Networking|SwitchHasAuthority
    (:Authority
      (CallFunction|OWNERUpdatePawn DeltaSeconds))))

(event Input|ActionEvents|InputActionForward
  (params (Key :type Key%20Structure :default "None"))
  ;[1 1 1] MOVEMENT Controls
  ;;[1 1 1] SET flames when movement pressed
  (:Pressed
    (CallFunction|SERVERSetEngineFlames true))
  (:Released
    (CallFunction|SERVERSetEngineFlames false)))

(event Input|ActionEvents|InputActionExitGame
  (params (Key :type Key%20Structure :default "None"))
  ;[1 1 1] EXIT back to main menu
  (:Pressed
    (Default|StartMainMenu (Variables|Game|GetGameInstance))))

(event Input|ActionEvents|InputActionRespawn
  (params (Key :type Key%20Structure :default "None"))
  ;[1 1 1] RESPAWN
  (:Pressed
    (CallFunction|SERVERRespawn (Game|GetPlayerController 0))))

(event Input|AxisEvents|InputAxisApplyPitch
  (params (AxisValue :type Float%20%28single-precision%29))
  ;[1 1 1] MOVEMENT Controls
  ;;[1 1 1] FORWARD/BACKWARDS
  (Variables|Movement|SetForwardInput AxisValue))

(event Input|AxisEvents|InputAxisShoot
  (params (AxisValue :type Float%20%28single-precision%29))
  ;[1 1 1] SHOOT
  (if (!= AxisValue 0.0)
    (if (<= (Variables|Firing|GetFireCooldown) 0.0)
      (bind _asbp_match_player_state (Utilities|Casting|CastToBP_MatchPlayerState (Variables|GetPlayerState)))
      (CallFunction|SERVERSpawnProjectiles _asbp_match_player_state)
      (Variables|Firing|SetFireCooldown (/ 3e+01 (CallFunction|GetPlayerFireRate))))))

(event Input|AxisEvents|InputAxisCameraUp
  (params (AxisValue :type Float%20%28single-precision%29))
  (bind _customshipref (Variables|Ship|GetCustomShipRef))
  ;[1 1 1] MOVEMENT Controls
  ;;[1 1 1] PITCH
  (Utilities|IsValid _customshipref
    (:Is%20Valid
      (Variables|Movement|SetPitchInput (* AxisValue (Variables|/Game/Blueprints/Ship/BP_ShipStats.BP_ShipStats_C|GetManeuverability (Variables|/Game/Blueprints/Ship/BP_Ship.BP_Ship_C|GetShipStats _customshipref)) (Variables|MovementCalibration|GetPitchRate))))))

(event Input|AxisEvents|InputAxisCameraRight
  (params (AxisValue :type Float%20%28single-precision%29))
  (bind _customshipref (Variables|Ship|GetCustomShipRef))
  ;[1 1 1] MOVEMENT Controls
  ;;[1 1 1] ROLL
  ;;;[1 1 1] CHECK if there is input
  (if (!= AxisValue 0.0)
    ;;;[1 1 1] ROLL ship based on input
    (Utilities|IsValid _customshipref
      (:Is%20Valid
        (Variables|Movement|SetRollInput (* AxisValue (Variables|MovementCalibration|GetRollRate) (Variables|/Game/Blueprints/Ship/BP_ShipStats.BP_ShipStats_C|GetManeuverability (Variables|/Game/Blueprints/Ship/BP_Ship.BP_Ship_C|GetShipStats _customshipref)) 4.0))))
    (else
      ;;;[1 1 1] RETURN ship to horizontal
      (Variables|Movement|SetRollInput (* (* (.Roll (Math|Rotator|BreakRotator (Transformation|GetActorRotation))) -1.0) (Variables|MovementCalibration|GetRollReturnRate))))))

(fn ConstructionScript
  (Utilities|FlowControl|Sequence
    (:then_0
      (bind _asbp_game_instance (Utilities|Casting|CastToBP_GameInstance (Game|GetGameInstance)))
      (Variables|Game|SetGameInstance _asbp_game_instance))
    (:then_1
      (bind _asbp_match_game_mode (Utilities|Casting|CastToBP_MatchGameMode (Game|GetGameMode)))
      (Variables|Game|SetMatchGameMode _asbp_match_game_mode))
    (:then_2
      (bind _asbp_match_player_controller (Utilities|Casting|CastToBP_MatchPlayerController (Pawn|GetController)))
      (Variables|Game|SetMatchPlayerControllerRef _asbp_match_player_controller))
    (:then_3
      (Variables|State|SetIsDestroyed false))))

(fn SetupCustomShipforMatch
  (bind _shipactor (Variables|Default|GetShipActor))
  ;[1 1 1] LOAD ship info from player controller
  (Utilities|IsValid (Variables|Game|GetMatchPlayerControllerRef)
    (:Is%20Valid
      (Variables|Default|SetShipInfo (Variables|/Game/Blueprints/Match/BP_MatchPlayerController.BP_MatchPlayerController_C|GetShipInfo (Variables|Game|GetMatchPlayerControllerRef)))
      ;[1 1 1] SET class of ship child actor
      (ChildActorComponent|SetChildActorClass _shipactor "/Game/Blueprints/Ship/BP_CustomShip.BP_CustomShip_C")
      (bind _asbp_custom_ship (Utilities|Casting|CastToBP_CustomShip (Variables|/Script/Engine.ChildActorComponent|GetChildActor _shipactor))
        (:then
          ;;[1 1 1] SET ref to ship in pawn
          (bind _output_get (Variables|Ship|SetCustomShipRef _asbp_custom_ship))
          ;;[1 1 1] SET ref to pawn in ship
          (Variables|/Game/Blueprints/Ship/BP_Ship.BP_Ship_C|SetParentPawnRef _output_get self)
          ;[1 1 1] SETUP the movement variables
          (CallFunction|SetupMovementCharacteristics))
        (:CastFailed
          (Development|PrintString "MatchPlayerPawn: FAILED to cast ship actor to custom ship." true true "(R=1.000000,G=0.000000,B=0.000000,A=1.000000)" 1e+01))))))

(fn CalculateEngineThrust
  (bind _customshipref (Variables|Ship|GetCustomShipRef))
  (bind _speedrate (Variables|MovementCalibration|GetSpeedRate))
  (bind _forwardinput (Variables|Movement|GetForwardInput))
  (bind _shipstats (Variables|/Game/Blueprints/Ship/BP_Ship.BP_Ship_C|GetShipStats _customshipref))
  (bind _speed (Variables|/Game/Blueprints/Ship/BP_ShipStats.BP_ShipStats_C|GetSpeed _shipstats))
  (bind _returnvalue (* _speed _speedrate _forwardinput))
  (if (== (Variables|Movement|GetForwardInput) 0.0)
    (Variables|Movement|SetEngineThrust (- (Variables|Movement|GetEngineThrust) _returnvalue))
    (if (or (< (Variables|Movement|GetEngineThrust) 0.1) (> (Variables|Movement|GetEngineThrust) -0.1))
      (Variables|Movement|SetEngineThrust 0.0))
    (else
      (Variables|Movement|SetEngineThrust (+ _returnvalue (Variables|Movement|GetEngineThrust))))))

(fn CalculateForwardSpeed
  (Variables|Movement|SetForwardSpeed (+ (Variables|Movement|GetForwardSpeed) (- (Variables|Movement|GetEngineThrust) (Variables|Movement|GetAirResistance)))))

(fn CalculateAirResistance
  (Variables|Movement|SetAirResistance (* (Variables|Movement|GetForwardSpeed) (Variables|MovementCalibration|GetAirResistanceRatio))))

(fn SetupMovementCharacteristics
  (bind _defaultacceleration (Variables|MovementCalibration|GetDefaultAcceleration))
  (bind _floatingpawnmovement (Variables|Default|GetFloatingPawnMovement))
  (bind _customshipref (Variables|Ship|GetCustomShipRef))
  (bind _customshipref_2 (Variables|Ship|GetCustomShipRef))
  (bind _shipstats (Variables|/Game/Blueprints/Ship/BP_Ship.BP_Ship_C|GetShipStats _customshipref))
  (bind _shipstats_2 (Variables|/Game/Blueprints/Ship/BP_Ship.BP_Ship_C|GetShipStats _customshipref_2))
  (bind _weight (Variables|/Game/Blueprints/Ship/BP_ShipStats.BP_ShipStats_C|GetWeight _shipstats))
  (bind _thrust (Variables|/Game/Blueprints/Ship/BP_ShipStats.BP_ShipStats_C|GetThrust _shipstats))
  (bind _returnvalue (- _thrust _weight))
  (bind _returnvalue_2 (* _returnvalue 2e+01))
  (bind _returnvalue_3 (+ _defaultacceleration _returnvalue_2))
  (Variables|/Script/Engine.FloatingPawnMovement|SetMaxSpeed (Variables|Default|GetFloatingPawnMovement) (+ (Variables|ShipCharacteristics|GetDefaultMaxSpeed) (* (- (Variables|/Game/Blueprints/Ship/BP_ShipStats.BP_ShipStats_C|GetThrust _shipstats_2) (Variables|/Game/Blueprints/Ship/BP_ShipStats.BP_ShipStats_C|GetResistance _shipstats_2)) 1e+02)))
  (Variables|/Script/Engine.FloatingPawnMovement|SetAcceleration _floatingpawnmovement _returnvalue_3)
  (Variables|/Script/Engine.FloatingPawnMovement|SetDeceleration _floatingpawnmovement (* _returnvalue_3 -1.0)))

(fn GetPlayerFireRate
  (return (* (Variables|/Game/Blueprints/Ship/BP_ShipStats.BP_ShipStats_C|GetFire%20Rate (Variables|/Game/Blueprints/Ship/BP_Ship.BP_Ship_C|GetShipStats (Variables|Ship|GetCustomShipRef))) (Variables|Firing|GetFireRateModifier))))

(fn SetPawnDestroyed
  (bind _customshipref (Variables|Ship|GetCustomShipRef))
  (Variables|State|SetIsDestroyed true)
  (Utilities|IsValid _customshipref
    (:Is%20Valid
      (Default|SetShiptoDestroyed _customshipref))))

(fn GetShipPartfromName
  (params (Ship%20Part%20Name :type String))
  (for _array_element (Actor|GetAllChildActors (Variables|Ship|GetCustomShipRef) false)
    (bind _asbp_ship_part (Utilities|Casting|CastToBP_ShipPart _array_element))
    (if (Game|IsActorBeingDestroyed _asbp_ship_part)
      (if (Utilities|Enum|Equal(Enum) (Variables|/Game/Blueprints/Ship/ShipPart/BP_ShipPart.BP_ShipPart_C|GetPartName _asbp_ship_part) Ship%20Part%20Name)
        (return true _asbp_ship_part))))
  (return false 0))

(fn GetShipPartfromIndex
  (params (Ship%20Part%20Index :type Integer))
  (for (_array_element _array_index) (Variables|/Game/Blueprints/Ship/BP_CustomShip.BP_CustomShip_C|GetShipParts (Variables|Ship|GetCustomShipRef))
    (if (== _array_index Ship%20Part%20Index)
      (Utilities|IsValid _array_element
        (:Is%20Valid
          (return true _array_element))
        (:Is%20Not%20Valid
          (return false 0)))))
  (return false 0))