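; Match player state that tracks a player's ship combat score: opponent ships destroyed and own ship losses.
; On BeginPlay it calls a SERVER-prefixed event that asks BP_MatchGameMode to add this player's score to all client HUDs.
; Two functions increment the respective counters by one, without triggering any HUD update themselves.
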(event Custom|SERVER_UpdateAllPlayerScorePanels
  (bind _asbp_match_game_mode (Utilities|Casting|CastToBP_MatchGameMode (Game|GetGameMode)))
  (Default|GMAddPlayerScoretoAllClientHUDs _asbp_match_game_mode self))

(event EventBeginPlay
  (CallFunction|SERVERUpdateAllPlayerScorePanels))

(fn ConstructionScript)

(fn PSOpponentShipWasDestroyed
  (Variables|Default|SetOpponentShipsDestroyed (+ (Variables|Default|GetOpponentShipsDestroyed) 1)))

(fn PSOwnShipWasDestroyed
  (Variables|Default|SetOwnShipDestroyed (+ (Variables|Default|GetOwnShipDestroyed) 1)))