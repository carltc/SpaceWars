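; Match game state that ends a timed match by loading the end map.
; On BeginPlay it caches the game mode, player count and game instance, then sets a hardcoded test match ID and prints it.
; Tick compares ElapsedTime plus the frame delta to MatchLength and opens the end map after a short delay.
; ShipDestroyed is an empty stub, and a music playback node is left unconnected.
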(event Custom|ShipDestroyed)

(event EventBeginPlay
  ;[1 1 1] Begin
  (Utilities|FlowControl|Sequence
    (:then_0
      (bind _asbp_game_mode (Utilities|Casting|CastToBP_GameMode (Game|GetGameMode)))
      (bind _output_get (Variables|Default|SetGameMode _asbp_game_mode))
      (bind _returnvalue (Class|GameModeBase|GetNumPlayers _output_get))
      (Variables|Default|SetNumPlayers _returnvalue))
    (:then_1
      (bind _asbp_game_instance (Utilities|Casting|CastToBP_GameInstance (Game|GetGameInstance)))
      (Variables|Default|SetGameInstance _asbp_game_instance))
    (:then_2
      (bind _output_get_2 (Variables|Default|SetMatchID "TestMatch"))
      (Development|PrintString (Utilities|String|Append "New match started: " _output_get_2)))))

(event EventTick
  (params (DeltaSeconds :type Float%20%28single-precision%29))
  ;[1 1 1] Tick
  (if (>= (+ (Variables|Default|GetElapsedTime) DeltaSeconds) (Math|Conversions|ToFloat(Integer) (Variables|Default|GetMatchLength)))
    (Utilities|FlowControl|Delay 0.2)
    (Game|OpenLevel(byName) (Variables|Default|GetEndMapName))))

(fn ConstructionScript)