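; BP_EnemySpawner is an actor that repeatedly spawns enemy ship pawns at its own location.
; A looping timer started on BeginPlay spawns a BP_Pawn_Enemy with SpawnAIFromClass at a fixed interval, first firing after one interval.
; Each spawned pawn is added to the EnemyPawns array on BP_GameState, with no cap or stop condition in this Blueprint.
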(event Custom|Spawn%20Enemy
  ;[1 1 1] SPAWN Enemy Ship
  (bind _returnvalue (AI|SpawnAIFromClass "/Game/Blueprints/Enemies/BP_Pawn_Enemy.BP_Pawn_Enemy_C" 0 (Transformation|GetActorLocation) "0, 0, 0" false 0))
  (bind _asbp_pawn_enemy (Utilities|Casting|CastToBP_Pawn_Enemy _returnvalue))
  (bind _asbp_game_state (Utilities|Casting|CastToBP_GameState (Game|GetGameState)))
  (Utilities|Array|Add (Variables|/Game/Blueprints/BP_GameState.BP_GameState_C|GetEnemyPawns _asbp_game_state) _asbp_pawn_enemy))

(event Custom|Enemy%20Spawner
  (CallFunction|SpawnEnemy))

(event EventBeginPlay
  (Utilities|Time|SetTimerbyEvent (delegate Custom|Enemy%20Spawner) 5.0 true))

(event Collision|EventActorBeginOverlap
  (params (OtherActor :type Actor%20Object%20Reference)))

(event EventTick
  (params (DeltaSeconds :type Float%20%28single-precision%29)))

(fn ConstructionScript)