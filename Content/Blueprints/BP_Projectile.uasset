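; BP_Projectile is a Lego projectile that scores hits for its firing BP_Pawn and breaks apart the ships it strikes.
; Its sphere ignores the instigator when moving, and hits on other actors besides the shooter's ship add impulse magnitude to score.
; Impulses above a threshold set the struck component simulating physics, or all static meshes for a "ShipCore" with an attached BP_Pawn.
; Tick destroys it on lifetime expiry or once it slows after a short grace period.
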(event EventBeginPlay
  ;[1 1 1] Begin
  (Collision|IgnoreActorwhenMoving (Variables|Default|GetSphereCollision) (Game|GetInstigator) true))

(event Collision|EventHit
  (params (MyComp :type Primitive%20Component%20Object%20Reference) (Other :type Actor%20Object%20Reference) (OtherComp :type Primitive%20Component%20Object%20Reference) (bSelfMoved :type Boolean) (HitLocation :type Vector :default "0, 0, 0") (HitNormal :type Vector :default "0, 0, 0") (NormalImpulse :type Vector :default "0, 0, 0") (Hit :type Hit%20Result%20Structure%20%28by%20ref%29))
  (bind _returnvalue (Math|Vector|VectorLength NormalImpulse))
  (bind _outactors (Actor|GetAttachedActors Other true))
  (bind _returnvalue_2 (Game|GetInstigator))
  (bind _output (Utilities|Array|Get(acopy) _outactors))
  ;[1 1 1] Hit
  (bind _asbp_pawn (Utilities|Casting|CastToBP_Pawn _returnvalue_2))
  (if (or (== Other (Variables|/Game/Blueprints/BP_Pawn.BP_Pawn_C|GetCurrentShip _asbp_pawn)) (== Other _returnvalue_2))
    (Development|PrintString "Parent Hit" false)
    (else
      (Development|PrintString (Utilities|String|Append "Hit:" (Utilities|GetDisplayName Other) (Utilities|String|ToString(Float) _returnvalue)) false)
      (Variables|/Game/Blueprints/BP_Pawn.BP_Pawn_C|SetScore _asbp_pawn (+ (Variables|/Game/Blueprints/BP_Pawn.BP_Pawn_C|GetScore _asbp_pawn) _returnvalue))
      (if (> _returnvalue (Variables|Default|GetHitDamageThreshold))
        (if (Components|ComponentHasTag OtherComp "ShipCore")
          (Development|PrintString "Ship Destroyed" true true "(R=0.000000,G=0.660000,B=1.000000,A=1.000000)" 2e+01)
          (bind _asbp_pawn_2 (Utilities|Casting|CastToBP_Pawn _output)
            (:then
              (for _array_element (Actor|GetComponentsByClass Other "/Script/Engine.StaticMeshComponent")
                (bind _asstatic_mesh_component (Utilities|Casting|CastToStaticMeshComponent _array_element)
                  (:then
                    (Physics|SetSimulatePhysics _asstatic_mesh_component true))
                  (:CastFailed
                    (Development|PrintString "Can't Get Static Meshes" true true "(R=0.000000,G=0.660000,B=1.000000,A=1.000000)" 2e+01)))))
            (:CastFailed
              (Development|PrintString (Utilities|String|Append "Can't convert: " (Utilities|GetDisplayName _output) " to BP_Pawn") true true "(R=0.000000,G=0.660000,B=1.000000,A=1.000000)" 2e+01)))
          (else
            (Physics|SetSimulatePhysics OtherComp true)))))))

(event EventTick
  (params (DeltaSeconds :type Float%20%28single-precision%29))
  ;[1 1 1] Tick
  (bind _output_get (Variables|Default|SetLifetimeSeconds (+ DeltaSeconds (Variables|Default|GetLifetimeSeconds))))
  (if (or (> _output_get (Variables|Default|GetMaxLifetimeSeconds)) (and (> _output_get 1.0) (< (Math|Vector|VectorLength (Transformation|GetComponentVelocity (Variables|Default|GetLegoProjectile))) 2e+02)))
    (Actor|DestroyActor)
    (Development|PrintString (Utilities|String|Append (Utilities|GetDisplayName self) " died"))))

(fn ConstructionScript)