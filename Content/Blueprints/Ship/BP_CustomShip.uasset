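; Player-customizable ship actor assembled from modular BP_ShipPart child actors, tracked in a ShipParts array.
; Construction seeds an empty ship with a CoreBrick from the parts data table; BeginPlay sums part bonuses into ShipStats.
; SaveShip captures part transforms and materials into a BP_CustomShipSaveGame slot, appending numeric suffixes to avoid collisions for new ships.
; LoadShip respawns parts from the ShipParts array, without reading the save itself.
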(event EventBeginPlay
  (CallFunction|CalculateVehicleStats))

(event Collision|EventActorBeginOverlap
  (params (OtherActor :type Actor%20Object%20Reference)))

(event EventTick
  (params (DeltaSeconds :type Float%20%28single-precision%29)))

(fn ConstructionScript
  (|CallParentFunction)
  (Utilities|FlowControl|Sequence
    (:then_0
      ;[1 1 1] ADD core block to custom ship
      ;;[1 1 1] ONLY add core block if no other parts exist
      (if (<= (Utilities|Array|Length (Variables|Default|GetShipParts)) 0)
        (bind _returnvalue (Utilities|GetDataTableRow "/Game/Blueprints/ShipBuilder/ShipParts_DataTable.ShipParts_DataTable" "CoreBrick")
          (:then
            (bind _returnvalue_2 (AddComponent|AddChildActorComponent false))
            (ChildActorComponent|SetChildActorClass _returnvalue_2 (.Class (Utilities|Struct|BreakShipPartInfo _returnvalue)))
            (bind _asbp_ship_part (Utilities|Casting|CastToBP_ShipPart (Variables|/Script/Engine.ChildActorComponent|GetChildActor _returnvalue_2)))
            (Variables|/Game/Blueprints/ShipBuilder/BP_ShipPart.BP_ShipPart_C|SetShipPartInfo _asbp_ship_part _returnvalue)
            (Utilities|Array|Add (Variables|/Script/Engine.Actor|GetTags _asbp_ship_part) "ShipPart")
            (Default|SetPieceMaterial _asbp_ship_part (.DefaultMaterial (Utilities|Struct|BreakShipPartInfo _returnvalue)) false)
            (Utilities|Array|Add (Variables|Default|GetShipParts) (Utilities|Struct|MakeShipPart _returnvalue _asbp_ship_part "0.000000,0.000000,0.000000|0.000000,0.000000,0.000000|1.000000,1.000000,1.000000" (.DefaultMaterial (Utilities|Struct|BreakShipPartInfo _returnvalue))))))))))

(fn CalculateVehicleStats
  ;[1 1 1] RESET stats
  (Default|ResetStats (Variables|Default|GetShipStats))
  (for _array_element (Variables|Default|GetShipParts)
    (Default|AddStats (Variables|Default|GetShipStats) (.SpeedAddition (Utilities|Struct|BreakShipPartInfo (.ShipPartInfo (Utilities|Struct|BreakShipPart _array_element)))) (.ManueverabilityAddition (Utilities|Struct|BreakShipPartInfo (.ShipPartInfo (Utilities|Struct|BreakShipPart _array_element)))) (.ArmourAddition (Utilities|Struct|BreakShipPartInfo (.ShipPartInfo (Utilities|Struct|BreakShipPart _array_element)))) (.FireRateAddition (Utilities|Struct|BreakShipPartInfo (.ShipPartInfo (Utilities|Struct|BreakShipPart _array_element)))) (.FireSpeedAddition (Utilities|Struct|BreakShipPartInfo (.ShipPartInfo (Utilities|Struct|BreakShipPart _array_element)))))))

(fn AddParttoShip
  (params (Ship%20Part :type Ship%20Part%20Structure))
  (Utilities|Array|Add (Variables|Default|GetShipParts) Ship%20Part))

(fn SaveShip
  (params (PlayerName :type String) (CreateNewShip :type Boolean))
  (for (_ _array_index) (Variables|Default|GetShipParts)
    ;[1 1 1] SET the transform of this part
    (Utilities|IsValid (.Actor (Utilities|Struct|BreakShipPart (Utilities|Array|Get(acopy) (Variables|Default|GetShipParts) _array_index)))
      (:Is%20Valid
        (Utilities|Array|SetArrayElem (Variables|Default|GetShipParts) _array_index (Utilities|Struct|MakeShipPart (.ShipPartInfo (Utilities|Struct|BreakShipPart (Utilities|Array|Get(acopy) (Variables|Default|GetShipParts) _array_index))) 0 (Transformation|GetRelativeTransform (Variables|/Game/Blueprints/ShipBuilder/BP_ShipPart.BP_ShipPart_C|GetStaticMesh (.Actor (Utilities|Struct|BreakShipPart (Utilities|Array|Get(acopy) (Variables|Default|GetShipParts) _array_index))))) (.Material (Utilities|Struct|BreakShipPart (Utilities|Array|Get(acopy) (Variables|Default|GetShipParts) _array_index))))))))
  ;[1 1 1] CREATE a save game
  (Variables|Default|SetSaveGameSlotName (Utilities|String|Append PlayerName "-CustomShip-" (Variables|Default|GetShipName)))
  (bind _returnvalue (SaveGame|CreateSaveGameObject "/Game/Blueprints/ShipBuilder/BP_CustomShipSaveGame.BP_CustomShipSaveGame_C"))
  (Variables|Default|SetSaveGameRef _returnvalue)
  (Variables|/Game/Blueprints/ShipBuilder/BP_CustomShipSaveGame.BP_CustomShipSaveGame_C|SetShipInfo _returnvalue (Utilities|Struct|MakeShipInfo (Utilities|Text|ToText(String) (Variables|Default|GetShipName)) (Variables|Default|GetShipParts) (Variables|Default|GetSaveGameSlotName)))
  ;[1 1 1] Check if a new Ship should be created, if not then check for unique save game name
  (if CreateNewShip
    (bind _returnvalue_2 (SaveGame|DoesSaveGameExist (Variables|Default|GetSaveGameSlotName)))
    (Variables|Default|SetSaveGameAlreadyExists _returnvalue_2)
    ;[1 1 1] LOOP through to find a valid save game name and append a number if none found
    (while (Variables|Default|GetSaveGameAlreadyExists)
      (Variables|Default|SetSaveGameSlotInteger (+ (Variables|Default|GetSaveGameSlotInteger) 1))
      (bind _output_get (Variables|Default|SetSaveGameSlotName (Utilities|String|Append (Variables|Default|GetSaveGameSlotName) "_" (Utilities|String|ToString(Integer) (Variables|Default|GetSaveGameSlotInteger)))))
      (bind _returnvalue_3 (SaveGame|DoesSaveGameExist _output_get))
      (Variables|Default|SetSaveGameAlreadyExists _returnvalue_3)
      (Variables|/Game/Blueprints/ShipBuilder/BP_CustomShipSaveGame.BP_CustomShipSaveGame_C|SetShipInfo (Variables|Default|GetSaveGameRef) (Utilities|Struct|MakeShipInfo (Utilities|Text|ToText(String) (Variables|Default|GetShipName)) (Variables|Default|GetShipParts) (Variables|Default|GetSaveGameSlotName)))))
  ;[1 1 1] SAVE the ship
  (bind _returnvalue_4 (SaveGame|SaveGametoSlot (Variables|Default|GetSaveGameRef) (Variables|Default|GetSaveGameSlotName)))
  (if _returnvalue_4
    (Development|PrintString (Utilities|String|Append "Ship '" (Variables|Default|GetSaveGameSlotName) "' saved successfully!") true true "(R=0.000000,G=0.660000,B=1.000000,A=1.000000)" 1e+01)
    (else
      (Development|PrintString (Utilities|String|Append "Ship '" (Variables|Default|GetSaveGameSlotName) "' did NOT save successfully!") true true "(R=0.000000,G=0.660000,B=1.000000,A=1.000000)" 1e+01)))
  (return (Variables|Default|GetSaveGameSlotName)))

(fn LoadShip
  (for _array_element (Variables|Default|GetShipParts)
    (bind _returnvalue (AddComponent|AddChildActorComponent false (.Transform (Utilities|Struct|BreakShipPart _array_element))))
    (ChildActorComponent|SetChildActorClass _returnvalue (.Class (Utilities|Struct|BreakShipPartInfo (.ShipPartInfo (Utilities|Struct|BreakShipPart _array_element)))))
    (bind _asbp_ship_part (Utilities|Casting|CastToBP_ShipPart (Variables|/Script/Engine.ChildActorComponent|GetChildActor _returnvalue)))
    (Variables|/Game/Blueprints/ShipBuilder/BP_ShipPart.BP_ShipPart_C|SetShipPartInfo _asbp_ship_part (.ShipPartInfo (Utilities|Struct|BreakShipPart _array_element)))
    (Default|SetPieceMaterial _asbp_ship_part (.Material (Utilities|Struct|BreakShipPart _array_element)) false)
    (bind _structout (Utilities|Struct|SetmembersinShipPart _array_element _asbp_ship_part))
    (|SetBy-RefVar _array_element _structout))
  (return))