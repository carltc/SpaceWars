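; Base ship pawn for a multiplayer game, handling replicated flight movement and projectile fire.
; Each tick applies roll, pitch, yaw and forward deltas locally, then relays them through server and multicast events to non-controlling copies, without frame-time scaling.
; The server spawns projectiles and multicasts their launch impulse.
; Ship destruction gathers mesh parts into the child ship actor's list, while unpossess and respawn logic is left disconnected.
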(event Custom|UnpossessPawn
  ;[1 1 1] Unpossess Pawn
  (bind _asbp_player_state (Utilities|Casting|CastToBP_PlayerState (Variables|GetPlayerState))))

(event Custom|ShipDestroyed
  ;[1 1 1] Ship Destroyed
  (bind _asfbx_scene_basic_ship (Utilities|Casting|CastToFbxScene_BasicShip (Variables|/Script/Engine.ChildActorComponent|GetChildActor (Variables|Default|GetShip))))
  (for _array_element (Actor|GetComponentsByClass _asfbx_scene_basic_ship "/Script/Engine.StaticMeshComponent")
    (bind _asstatic_mesh_component (Utilities|Casting|CastToStaticMeshComponent _array_element)
      (:then
        (Utilities|Array|Add (Variables|/Game/Models/BasicShip/FbxScene_BasicShip.FbxScene_BasicShip_C|GetDestroyedPartReferences _asfbx_scene_basic_ship) _asstatic_mesh_component))
      (:CastFailed
        (Development|PrintString (Utilities|String|Append "Failed to cast Static Mesh Component: " (Utilities|GetDisplayName _asstatic_mesh_component)) true true "(R=0.000000,G=0.660000,B=1.000000,A=1.000000)" 2e+01)))))

(event Custom|Server_SetPawnMovement
  (params (DeltaRotation :type Rotator) (DeltaLocation :type Vector) (ScaleValue :type Float%20%28single-precision%29) (Target2 :type Pawn%20Object%20Reference))
  ;[1 1 1] Cast movement to server
  (CallFunction|MulticastEvent 0 DeltaRotation DeltaLocation ScaleValue Target2))

(event Custom|MulticastEvent
  (params (Target :type Actor%20Object%20Reference) (DeltaRotation :type Rotator) (DeltaLocation :type Vector) (ScaleValue :type Float%20%28single-precision%29) (Target2 :type Pawn%20Object%20Reference))
  ;[1 1 1] Multicast Actor Position
  (if (Pawn|IsLocallyControlled)
    (Development|PrintString (Utilities|String|Append "Network:" (Utilities|GetObjectName Target2)))
    (else
      (Transformation|AddActorLocalRotation DeltaRotation true false)
      (Transformation|AddActorLocalOffset DeltaLocation true false))))

(event Custom|Client_SetPawnMovement
  (bind _self self)
  (bind _currentforwardspeed (Variables|Default|GetCurrentForwardSpeed))
  (bind _currentrollspeed (Variables|Default|GetCurrentRollSpeed))
  (bind _currentpitchspeed (Variables|Default|GetCurrentPitchSpeed))
  (bind _currentyawspeed (Variables|Default|GetCurrentYawSpeed))
  (bind _returnvalue (Math|Rotator|MakeRotator _currentrollspeed _currentpitchspeed _currentyawspeed))
  (bind _returnvalue_2 (Math|Vector|MakeVector _currentforwardspeed 0.0 0.0))
  ;[1 1 1] Cleint Pawn Movement
  (if (Math|Boolean|ORBoolean (!= _currentrollspeed 0.0) (!= _currentpitchspeed 0.0) (!= _currentyawspeed 0.0) (!= 0.0 _currentforwardspeed))
    (Transformation|AddActorLocalRotation _returnvalue true false)
    (Transformation|AddActorLocalOffset _returnvalue_2 true false)
    (Development|PrintString (Utilities|String|Append "Locally: " (Utilities|String|ToString(Float) _currentforwardspeed)))
    (Networking|SwitchHasAuthority
      (:Authority
        (CallFunction|MulticastEvent 0 _returnvalue _returnvalue_2 _currentforwardspeed _self))
      (:Remote
        (CallFunction|ServerSetPawnMovement _returnvalue _returnvalue_2 _currentforwardspeed _self)))))

(event Custom|Server_ProjectileShot
  (params (SpawnTransform :type Transform) (Impulse :type Vector))
  ;[1 1 1] Server Projectile Shot
  (Networking|SwitchHasAuthority
    (:Authority
      (bind _returnvalue (Game|SpawnActorfromClass "/Game/Blueprints/Ship/BP_Projectile.BP_Projectile_C" SpawnTransform "AlwaysSpawn" 0 0))
      (CallFunction|MulticastProjectileShot Impulse _returnvalue))))

(event Custom|Multicast_ProjectileShot
  (params (InputPin :type Vector) (Target :type BP%20Projectile%20Object%20Reference))
  ;[1 1 1] Multicast Projectile Shot
  (Utilities|IsValid Target
    (:Is%20Valid
      (Physics|AddImpulse (Variables|/Game/Blueprints/Ship/BP_Projectile.BP_Projectile_C|GetLegoProjectile Target) InputPin "None" false)
      (Variables|Default|SetShotsFired (+ (Variables|Default|GetShotsFired) 1)))))

(event EventBeginPlay
  ;[1 1 1] Start of game
  (Utilities|FlowControl|Sequence
    (:then_0
      (bind _asbp_game_instance (Utilities|Casting|CastToBP_GameInstance (Game|GetGameInstance)))
      (Variables|Default|SetGameInstance _asbp_game_instance))
    (:then_1
      (bind _asbp_player_controller_base (Utilities|Casting|CastToBP_PlayerController_Base (Game|GetPlayerController 0)))
      (Variables|Default|SetPlayerController _asbp_player_controller_base))))

(event EventDestroyed
  ;[1 1 1] Destroyed
  (Development|PrintString (Utilities|String|Append "Died: " (Utilities|GetDisplayName self))))

(event EventTick
  (params (DeltaSeconds :type Float%20%28single-precision%29))
  ;[1 1 1] Tick
  (CallFunction|ClientSetPawnMovement))

(event EventEndPlay
  (params (EndPlayReason :type EEndPlayReason%20Enum :default "Destroyed"))
  ;[1 1 1] End of game
)

(fn ConstructionScript)