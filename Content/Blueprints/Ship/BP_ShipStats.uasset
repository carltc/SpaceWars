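; Actor that holds a ship's stats, such as speed, armour, fire rate and thrust, and totals the bonuses from its parts.
; CalculateStats looks up each part's row in the ShipParts data table and feeds its additions to AddStats, without resetting first.
; ResetStats returns every stat to a baseline of one.
; AddStat and GetStat modify or read a single stat selected by a type enum.
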(event EventBeginPlay)

(event Collision|EventActorBeginOverlap
  (params (OtherActor :type Actor%20Object%20Reference)))

(event EventTick
  (params (DeltaSeconds :type Float%20%28single-precision%29)))

(fn ConstructionScript)

(fn AddStat
  (params (Stat%20Type :type ShipStatTypes%20Enum :default "ShipStatTypes_MAX") (Stat%20Value%20To%20Add :type Float%20%28single-precision%29))
  (switch Utilities|FlowControl|Switch|SwitchonShipStatTypes Stat%20Type
    (:NewEnumerator0
      (Variables|Default|SetSpeed (+ Stat%20Value%20To%20Add (Variables|Default|GetSpeed))))
    (:NewEnumerator1
      (Variables|Default|SetManeuverability (+ Stat%20Value%20To%20Add (Variables|Default|GetManeuverability))))
    (:NewEnumerator2
      (Variables|Default|SetArmour (+ Stat%20Value%20To%20Add (Variables|Default|GetArmour))))
    (:NewEnumerator3
      (Variables|Default|SetFire%20Rate (+ Stat%20Value%20To%20Add (Variables|Default|GetFire%20Rate))))
    (:NewEnumerator4
      (Variables|Default|SetFire%20Speed (+ Stat%20Value%20To%20Add (Variables|Default|GetFire%20Speed))))
    (:NewEnumerator5
      (Variables|Default|SetWeight (+ Stat%20Value%20To%20Add (Variables|Default|GetWeight))))
    (:NewEnumerator6
      (Variables|Default|SetResistance (+ Stat%20Value%20To%20Add (Variables|Default|GetResistance))))
    (:NewEnumerator7
      (Variables|Default|SetThrust (+ Stat%20Value%20To%20Add (Variables|Default|GetThrust))))))

(fn ResetStats
  (bind _output_get (Variables|Default|SetSpeed 1.0))
  (bind _output_get_2 (Variables|Default|SetManeuverability _output_get))
  (bind _output_get_3 (Variables|Default|SetArmour _output_get_2))
  (bind _output_get_4 (Variables|Default|SetFire%20Rate _output_get_3))
  (bind _output_get_5 (Variables|Default|SetFire%20Speed _output_get_4))
  (bind _output_get_6 (Variables|Default|SetWeight _output_get_5))
  (bind _output_get_7 (Variables|Default|SetResistance _output_get_6))
  (Variables|Default|SetThrust _output_get_7))

(fn GetStat
  (params (Stat%20Type :type ShipStatTypes%20Enum :default "NewEnumerator0"))
  (switch Utilities|FlowControl|Switch|SwitchonShipStatTypes Stat%20Type
    (:NewEnumerator0
      (return (Variables|Default|GetSpeed)))
    (:NewEnumerator1
      (return (Variables|Default|GetManeuverability)))
    (:NewEnumerator2
      (return (Variables|Default|GetArmour)))
    (:NewEnumerator3
      (return (Variables|Default|GetFire%20Rate)))
    (:NewEnumerator4
      (return (Variables|Default|GetFire%20Speed)))
    (:NewEnumerator5
      (return (Variables|Default|GetWeight)))
    (:NewEnumerator6
      (return (Variables|Default|GetResistance)))
    (:NewEnumerator7
      (return (Variables|Default|GetThrust)))))

(fn AddStats
  (params (Speed :type Float%20%28single-precision%29) (Manueverability :type Float%20%28single-precision%29) (Armour :type Float%20%28single-precision%29) (Fire%20Rate :type Float%20%28single-precision%29) (Fire%20Speed :type Float%20%28single-precision%29) (Weight :type Float%20%28single-precision%29) (Resistance :type Float%20%28single-precision%29) (Thrust :type Float%20%28single-precision%29))
  (Utilities|FlowControl|Sequence
    (:then_0
      (Variables|Default|SetSpeed (+ Speed (Variables|Default|GetSpeed))))
    (:then_1
      (Variables|Default|SetManeuverability (+ Manueverability (Variables|Default|GetManeuverability))))
    (:then_2
      (Variables|Default|SetArmour (+ Armour (Variables|Default|GetArmour))))
    (:then_3
      (Variables|Default|SetFire%20Rate (+ Fire%20Rate (Variables|Default|GetFire%20Rate))))
    (:then_4
      (Variables|Default|SetFire%20Speed (+ Fire%20Speed (Variables|Default|GetFire%20Speed))))
    (:then_5
      (Variables|Default|SetWeight (+ Weight (Variables|Default|GetWeight))))
    (:then_6
      (Variables|Default|SetResistance (+ Resistance (Variables|Default|GetResistance))))
    (:then_7
      (Variables|Default|SetThrust (+ Thrust (Variables|Default|GetThrust))))))

(fn CalculateStats
  (params (ShipParts :type Array%20of%20Ship%20Part%20Structures))
  (for _array_element ShipParts
    (bind _returnvalue (Utilities|GetDataTableRow "/Game/Blueprints/Ship/ShipPart/ShipParts_DataTable.ShipParts_DataTable" (.ShipPartRowName (Utilities|Struct|BreakShipPart _array_element)))
      (:then
        (CallFunction|AddStats (.SpeedAddition (Utilities|Struct|BreakShipPartInfo _returnvalue)) (.ManueverabilityAddition (Utilities|Struct|BreakShipPartInfo _returnvalue)) (.ArmourAddition (Utilities|Struct|BreakShipPartInfo _returnvalue)) (.FireRateAddition (Utilities|Struct|BreakShipPartInfo _returnvalue)) (.FireSpeedAddition (Utilities|Struct|BreakShipPartInfo _returnvalue)) (.WeightAddition (Utilities|Struct|BreakShipPartInfo _returnvalue)) (.ResistanceAddition (Utilities|Struct|BreakShipPartInfo _returnvalue)) (.ThrustAddition (Utilities|Struct|BreakShipPartInfo _returnvalue)))))))