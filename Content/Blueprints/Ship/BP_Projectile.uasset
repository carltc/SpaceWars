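; Ship projectile that damages modular ships, ignores its instigator pawn and destroys itself when too old or too slow.
; Hits go to a server event that adds impulse magnitude to the shooter's score.
; Above a damage threshold, ShipCore-tagged components trigger ShipDestroyed on the hit actor's parent pawn.
; Other components go through a multicast that records them as destroyed on their Ship_Base and attaches an explosion effect.
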(event Custom|Server_ProjectileHit
  (params (Other%20Comp :type Primitive%20Component%20Object%20Reference) (Other :type Actor%20Object%20Reference) (PlayerPawn :type BP%20Pawn%20Base%20Object%20Reference) (Hit%20Normal :type Vector))
  (bind _returnvalue (Math|Vector|VectorLength Hit%20Normal))
  (bind _returnvalue_2 (Actor|GetParentActor Other))
  ;[1 1 1] Hit
  (Development|PrintString (Utilities|String|Append (Utilities|GetDisplayName self) " hit " (Utilities|GetDisplayName Other) " on " (Utilities|GetDisplayName Other%20Comp)) false)
  (Variables|/Game/Blueprints/Ship/BP_Pawn_Base.BP_Pawn_Base_C|SetScore PlayerPawn (+ (Variables|/Game/Blueprints/Ship/BP_Pawn_Base.BP_Pawn_Base_C|GetScore PlayerPawn) _returnvalue))
  (if (> _returnvalue (Variables|Default|GetHitDamageThreshold))
    (if (Components|ComponentHasTag Other%20Comp "ShipCore")
      (Development|PrintString "Ship Destroyed" false true "(R=0.000000,G=0.660000,B=1.000000,A=1.000000)" 2e+01)
      (bind _asship_base (Utilities|Casting|CastToShip_Base (Components|GetOwner Other%20Comp)))
      (Development|PrintString (Utilities|String|Append "Owner of hit components: " (Utilities|GetDisplayName _asship_base)) true true "(R=0.000000,G=0.660000,B=1.000000,A=1.000000)" 2e+01)
      (bind _asbp_pawn_base (Utilities|Casting|CastToBP_Pawn_Base _returnvalue_2)
        (:then
          (Default|ShipDestroyed _asbp_pawn_base)
          (Development|PrintString (Utilities|String|Append "Actor Destroy: " (Utilities|GetObjectName _asbp_pawn_base)) true true "(R=0.000000,G=0.660000,B=1.000000,A=1.000000)" 2e+01))
        (:CastFailed
          (Development|PrintString (Utilities|String|Append "Failed to cast to BP_Pawn_Base: " (Utilities|GetDisplayName _returnvalue_2)))))
      (else
        (CallFunction|MulticastComponentDestroyed Other%20Comp)))))

(event Custom|Multicast_ComponentDestroyed
  (params (Component :type Primitive%20Component%20Object%20Reference))
  ;[1 1 1] Multicast Destroyed Ship Part
  (bind _asship_base (Utilities|Casting|CastToShip_Base (Components|GetOwner Component))
    (:then
      (bind _asstatic_mesh_component (Utilities|Casting|CastToStaticMeshComponent Component))
      (Utilities|Array|Add (Variables|/Game/Models/Ship_Base.Ship_Base_C|GetDestroyedPartReferences _asship_base) _asstatic_mesh_component)
      (Effects|SpawnEmitterAttached "/Game/ParticleSystems/PS_Explosion.PS_Explosion" _asstatic_mesh_component "None"))
    (:CastFailed
      (Development|PrintString (Utilities|String|Append "Failed to cast to FbxScene_BasicShip: " (Utilities|GetDisplayName Component)) true true "(R=0.000000,G=0.660000,B=1.000000,A=1.000000)" 2e+01))))

(event EventBeginPlay
  ;[1 1 1] Begin
  (bind _asbp_pawn_base (Utilities|Casting|CastToBP_Pawn_Base (Game|GetInstigator)))
  (bind _output_get (Variables|Default|SetPlayerPawn _asbp_pawn_base))
  (Collision|IgnoreActorwhenMoving (Variables|Default|GetLegoProjectile) _output_get true))

(event Collision|EventHit
  (params (MyComp :type Primitive%20Component%20Object%20Reference) (Other :type Actor%20Object%20Reference) (OtherComp :type Primitive%20Component%20Object%20Reference) (bSelfMoved :type Boolean) (HitLocation :type Vector :default "0, 0, 0") (HitNormal :type Vector :default "0, 0, 0") (NormalImpulse :type Vector :default "0, 0, 0") (Hit :type Hit%20Result%20Structure%20%28by%20ref%29))
  ;[1 1 1] Hit
  (CallFunction|ServerProjectileHit OtherComp Other (Variables|Default|GetPlayerPawn) NormalImpulse))

(event EventTick
  (params (DeltaSeconds :type Float%20%28single-precision%29))
  ;[1 1 1] Tick
  (bind _output_get (Variables|Default|SetLifetimeSeconds (+ DeltaSeconds (Variables|Default|GetLifetimeSeconds))))
  (if (or (> _output_get (Variables|Default|GetMaxLifetimeSeconds)) (and (> _output_get 1.0) (< (Math|Vector|VectorLength (Transformation|GetComponentVelocity (Variables|Default|GetLegoProjectile))) 2e+02)))
    (Actor|DestroyActor)
    (Development|PrintString (Utilities|String|Append (Utilities|GetDisplayName self) " died") false)))

(fn ConstructionScript)