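; BP_Brick_1x2_5_On_Side_Gun is a ship part brick with five side connection slots and a front gun slot.
; Its construction script runs the parent script, then casts each connector's child actor to BP_ConnectionSlot.
; PositionCustomConnectionSlot gives each slot a fixed relative location and rotation: two pairs on opposite sides, one on an end, and the gun slot beyond the other end.
; The event graph holds only disabled default events.
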(event EventBeginPlay
  (|CallParentFunction) ; This node is disabled and will not be called.\nDrag off pins to build functionality.
)

(event Collision|EventActorBeginOverlap
  (params (OtherActor :type Actor%20Object%20Reference))
  (|CallParentFunction OtherActor) ; This node is disabled and will not be called.\nDrag off pins to build functionality.
)

(event EventTick
  (params (DeltaSeconds :type Float%20%28single-precision%29))
  (|CallParentFunction DeltaSeconds) ; This node is disabled and will not be called.\nDrag off pins to build functionality.
)

(fn ConstructionScript
  (|CallParentFunction)
  (Utilities|FlowControl|Sequence
    (:then_0
      ;[1 1 1] Side Connection 1
      (CallFunction|PositionCustomConnectionSlot (.AsBP%20Connection%20Slot (Utilities|Casting|CastToBP_ConnectionSlot (Variables|/Script/Engine.ChildActorComponent|GetChildActor (Variables|Default|GetSide%20Connector%201)))) "0.500000,0.500000,0.770000" "-90.000000, 0,0.000000"))
    (:then_1
      ;[1 1 1] Side Connection 2
      (CallFunction|PositionCustomConnectionSlot (.AsBP%20Connection%20Slot (Utilities|Casting|CastToBP_ConnectionSlot (Variables|/Script/Engine.ChildActorComponent|GetChildActor (Variables|Default|GetSide%20Connector%202)))) "0.500000,-0.500000,0.770000" "-90.000000, 0,0.000000"))
    (:then_2
      ;[1 1 1] Side Connection 3
      (CallFunction|PositionCustomConnectionSlot (.AsBP%20Connection%20Slot (Utilities|Casting|CastToBP_ConnectionSlot (Variables|/Script/Engine.ChildActorComponent|GetChildActor (Variables|Default|GetSide%20Connector%203)))) "-0.500000,0.500000,0.770000" "90.000000, 0,0.000000"))
    (:then_3
      ;[1 1 1] Side Connection 4
      (CallFunction|PositionCustomConnectionSlot (.AsBP%20Connection%20Slot (Utilities|Casting|CastToBP_ConnectionSlot (Variables|/Script/Engine.ChildActorComponent|GetChildActor (Variables|Default|GetSide%20Connector%204)))) "-0.500000,-0.500000,0.770000" "90.000000, 0,0.000000"))
    (:then_4
      ;[1 1 1] Side Connection 5
      (CallFunction|PositionCustomConnectionSlot (.AsBP%20Connection%20Slot (Utilities|Casting|CastToBP_ConnectionSlot (Variables|/Script/Engine.ChildActorComponent|GetChildActor (Variables|Default|GetSide%20Connector%205)))) "0,-1.000000,0.770000" "0, 0,-90.000000"))
    (:then_5
      ;[1 1 1] Front Gun Slot
      (CallFunction|PositionCustomConnectionSlot (.AsBP%20Connection%20Slot (Utilities|Casting|CastToBP_ConnectionSlot (Variables|/Script/Engine.ChildActorComponent|GetChildActor (Variables|Default|GetFront%20Connector)))) "0,1.800000,0.770000" "0, 0,-90.000000"))))