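; Ship part Blueprint for an 8x3 angled plate that defines where other parts can connect to it.
; The construction script runs the parent's, then builds an irregular slot footprint: four centered top-row cells, a full middle row and the two bottom-row end cells.
; Each cell gets two 1x1 horizontal slots offset from RelativeSlotsOrigin, one default type at plate height 1 and one of a second build slot type.
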(event EventBeginPlay
  (|CallParentFunction) ; This node is disabled and will not be called.\nDrag off pins to build functionality.
)

(event Collision|EventActorBeginOverlap
  (params (OtherActor :type Actor%20Object%20Reference))
  (|CallParentFunction OtherActor) ; This node is disabled and will not be called.\nDrag off pins to build functionality.
)

(event EventTick
  (params (DeltaSeconds :type Float%20%28single-precision%29))
  (|CallParentFunction DeltaSeconds) ; This node is disabled and will not be called.\nDrag off pins to build functionality.
)

(fn ConstructionScript
  (bind _returnvalue (Math|Vector|MakeVector 0.0 2.0 0.0))
  (bind _returnvalue_2 (Math|Vector|MakeVector 7.0 2.0 0.0))
  (bind _relative_slots_origin (Variables|Default|GetRelative%20Slots%20Origin))
  (bind _relative_slots_origin_2 (Variables|Default|GetRelative%20Slots%20Origin))
  (bind _returnvalue_3 (- _relative_slots_origin _returnvalue_2))
  (bind _returnvalue_4 (- _relative_slots_origin_2 _returnvalue))
  (|CallParentFunction)
  (Utilities|FlowControl|Sequence
    (:then_0
      ;[1 1 1] ADD top row of slots
      (for _index (range 2 5)
        (CallFunction|AddCustomConnectionSlotsHorizontal "NewEnumerator0" 1 1 1 (- (Variables|Default|GetRelative%20Slots%20Origin) (Math|Vector|MakeVector (Math|Conversions|ToFloat(Integer) _index) 0.0 0.0)) false "NewEnumerator0")
        (CallFunction|AddCustomConnectionSlotsHorizontal "NewEnumerator1" 1 1 0 (- (Variables|Default|GetRelative%20Slots%20Origin) (Math|Vector|MakeVector (Math|Conversions|ToFloat(Integer) _index) 0.0 0.0)) false "NewEnumerator0")))
    (:then_1
      ;[1 1 1] ADD middle row of slots
      (for _index_2 (range 0 7)
        (CallFunction|AddCustomConnectionSlotsHorizontal "NewEnumerator0" 1 1 1 (- (Variables|Default|GetRelative%20Slots%20Origin) (Math|Vector|MakeVector (Math|Conversions|ToFloat(Integer) _index_2) 1.0 0.0)) false "NewEnumerator0")
        (CallFunction|AddCustomConnectionSlotsHorizontal "NewEnumerator1" 1 1 0 (- (Variables|Default|GetRelative%20Slots%20Origin) (Math|Vector|MakeVector (Math|Conversions|ToFloat(Integer) _index_2) 1.0 0.0)) false "NewEnumerator0")))
    (:then_2
      ;[1 1 1] ADD bottom row slot 1
      (CallFunction|AddCustomConnectionSlotsHorizontal "NewEnumerator0" 1 1 1 _returnvalue_4 false "NewEnumerator0")
      (CallFunction|AddCustomConnectionSlotsHorizontal "NewEnumerator1" 1 1 0 _returnvalue_4 false "NewEnumerator0"))
    (:then_3
      ;[1 1 1] ADD bottom row slot 2
      (CallFunction|AddCustomConnectionSlotsHorizontal "NewEnumerator0" 1 1 1 _returnvalue_3 false "NewEnumerator0")
      (CallFunction|AddCustomConnectionSlotsHorizontal "NewEnumerator1" 1 1 0 _returnvalue_3 false "NewEnumerator0"))))