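; Ship part Blueprint for a 4x4 angled plate, defining where other parts can connect to it.
; After the parent construction script runs, a nested loop lays out a triangular staircase of single-cell horizontal connection slots relative to the slot origin.
; Each cell gets two slots: one of the default type with a plate height set, and one of a second build slot type.
; The event graph holds no active logic.
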(event EventBeginPlay
  (|CallParentFunction) ; This node is disabled and will not be called.\nDrag off pins to build functionality.
)

(event Collision|EventActorBeginOverlap
  (params (OtherActor :type Actor%20Object%20Reference))
  (|CallParentFunction OtherActor) ; This node is disabled and will not be called.\nDrag off pins to build functionality.
)

(event EventTick
  (params (DeltaSeconds :type Float%20%28single-precision%29))
  (|CallParentFunction DeltaSeconds) ; This node is disabled and will not be called.\nDrag off pins to build functionality.
)

(fn ConstructionScript
  (bind _relative_slots_origin (Variables|Default|GetRelative%20Slots%20Origin))
  (bind (_x _y) (Math|Vector|BreakVector _relative_slots_origin))
  (|CallParentFunction)
  ;[1 1 1] Y
  (for _index (range 0 3)
    ;[1 1 1] X
    (for _index_2 (range 0 _index)
      (CallFunction|AddCustomConnectionSlotsHorizontal "NewEnumerator0" 1 1 1 (Math|Vector|MakeVector (- _x (Math|Conversions|ToFloat(Integer) (- 3 _index_2))) (- _y (Math|Conversions|ToFloat(Integer) _index)) 0.0) false "NewEnumerator0")
      (CallFunction|AddCustomConnectionSlotsHorizontal "NewEnumerator1" 1 1 0 (Math|Vector|MakeVector (- _x (Math|Conversions|ToFloat(Integer) (- 3 _index_2))) (- _y (Math|Conversions|ToFloat(Integer) _index)) 0.0) false "NewEnumerator0"))))