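; BP_Sloping_1x2 is a ship part Blueprint, by its name a sloping 1x2 piece.
; Its construction script runs the parent's, then casts the TopConnector child actor to BP_ConnectionSlot and passes it to PositionCustomConnectionSlot with a fixed, unrotated offset for this shape.
; The event graph holds only disabled placeholder events, so the Blueprint adds no runtime logic of its own.
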(event EventBeginPlay
  (|CallParentFunction) ; This node is disabled and will not be called.\nDrag off pins to build functionality.
)

(event Collision|EventActorBeginOverlap
  (params (OtherActor :type Actor%20Object%20Reference))
  (|CallParentFunction OtherActor) ; This node is disabled and will not be called.\nDrag off pins to build functionality.
)

(event EventTick
  (params (DeltaSeconds :type Float%20%28single-precision%29))
  (|CallParentFunction DeltaSeconds) ; This node is disabled and will not be called.\nDrag off pins to build functionality.
)

(fn ConstructionScript
  (|CallParentFunction)
  (bind _asbp_connection_slot (Utilities|Casting|CastToBP_ConnectionSlot (Variables|/Script/Engine.ChildActorComponent|GetChildActor (Variables|Default|GetTop%20Connector))))
  (CallFunction|PositionCustomConnectionSlot _asbp_connection_slot (Math|Vector|MakeVector 0.0 -0.5 3.0) "0, 0, 0"))