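; Ship building part Blueprint for a 1x2 plate with a single connection slot on top.
; Its construction script runs the parent's, then adds a two-by-one horizontal set of custom connection slots, one plate high, with an offset origin.
; It then positions the TopConnector child actor, cast to BP_ConnectionSlot, one unit up on the local Z axis.
; The event graph holds only disabled default events.
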(event EventBeginPlay
  (|CallParentFunction) ; This node is disabled and will not be called.\nDrag off pins to build functionality.
)

(event Collision|EventActorBeginOverlap
  (params (OtherActor :type Actor%20Object%20Reference))
  (|CallParentFunction OtherActor) ; This node is disabled and will not be called.\nDrag off pins to build functionality.
)

(event EventTick
  (params (DeltaSeconds :type Float%20%28single-precision%29))
  (|CallParentFunction DeltaSeconds) ; This node is disabled and will not be called.\nDrag off pins to build functionality.
)

(fn ConstructionScript
  (|CallParentFunction)
  (CallFunction|AddCustomConnectionSlotsHorizontal "NewEnumerator1" 2 1 1 "0.500000, 0, 0")
  (CallFunction|PositionCustomConnectionSlot (.AsBP%20Connection%20Slot (Utilities|Casting|CastToBP_ConnectionSlot (Variables|/Script/Engine.ChildActorComponent|GetChildActor (Variables|Default|GetTop%20Connector)))) "0.000000,0.000000,1.000000" "0, 0, 0"))