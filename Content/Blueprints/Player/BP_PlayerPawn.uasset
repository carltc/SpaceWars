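; Player-controlled ship pawn that flies a BP_CustomShip child actor built from the parts and name stored in the game instance.
; Each tick, roll angle drives yaw, while forward input, engine thrust and proportional air resistance set forward speed for the FloatingPawnMovement.
; Pitch scales with ship maneuverability, roll self-levels without input, and strafing is disconnected.
; Transform is sent through a server update event every tick; actions handle shooting, respawn and menu exit.
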(event Custom|Server_UpdatePawn
  (params (Location :type Vector) (Rotation :type Rotator))
  ;[1 1 1] MOVEMENT Controls
  ;;[1 1 1] UPDATE server
  (Transformation|SetActorTransform (Math|Transform|MakeTransform Location Rotation)))

(event EventTick
  (params (DeltaSeconds :type Float%20%28single-precision%29))
  ;[1 1 1] EVENT tick
  (Utilities|FlowControl|Sequence
    (:then_0
      (Pawn|Input|AddControllerYawInput (* (/ (.Roll (Math|Rotator|BreakRotator (Transformation|GetActorRotation))) 9e+01) (Variables|MovementCalibration|GetYawRate))))
    (:then_1
      (CallFunction|CalculateForwardSpeed)
      (CallFunction|CalculateAirResistance)
      (CallFunction|CalculateEngineThrust)
      (Class|PawnMovementComponent|AddInputVector (Variables|Default|GetFloatingPawnMovement) (* (Transformation|GetActorForwardVector) (Variables|Movement|GetForwardSpeed)) false)
      ;[1 1 1] MOVEMENT Controls
      (CallFunction|ServerUpdatePawn (Transformation|GetActorLocation) (Transformation|GetActorRotation)))))

(event Input|ActionEvents|InputActionShoot
  (params (Key :type Key%20Structure))
  (:Pressed
    (Default|CSShoot (Variables|Default|GetCustomShipRef))))

(event Input|ActionEvents|InputActionExitGame
  (params (Key :type Key%20Structure))
  ;[1 1 1] EXIT back to main menu
  (:Pressed
    (Default|StartMainMenu (Variables|Default|GetGameInstance))))

(event Input|ActionEvents|InputActionRespawn
  (params (Key :type Key%20Structure))
  (:Pressed
    (Default|GMRespawn (Variables|Default|GetGameMode) (Game|GetPlayerController 0))))

(event Input|AxisEvents|InputAxisApplyPitch
  (params (AxisValue :type Float%20%28single-precision%29))
  ;[1 1 1] MOVEMENT Controls
  ;;[1 1 1] FORWARD/BACKWARDS
  (Variables|Movement|SetForwardInput AxisValue))

(event Input|AxisEvents|InputAxisApplyRoll
  (params (AxisValue :type Float%20%28single-precision%29))
  ;[1 1 1] MOVEMENT Controls
  ;;[1 1 1] STRAFE
)

(event Input|AxisEvents|InputAxisCameraUp
  (params (AxisValue :type Float%20%28single-precision%29))
  ;[1 1 1] MOVEMENT Controls
  ;;[1 1 1] PITCH
  (Pawn|Input|AddControllerPitchInput (* AxisValue (Variables|/Game/Blueprints/Ship/BP_ShipStats.BP_ShipStats_C|GetManeuverability (Variables|/Game/Blueprints/Ship/BP_Ship.BP_Ship_C|GetShipStats (Variables|Default|GetCustomShipRef))) (Variables|MovementCalibration|GetPitchRate))))

(event Input|AxisEvents|InputAxisCameraRight
  (params (AxisValue :type Float%20%28single-precision%29))
  ;[1 1 1] MOVEMENT Controls
  ;;[1 1 1] ROLL
  (if (!= AxisValue 0.0)
    (Pawn|Input|AddControllerRollInput (* AxisValue (Variables|MovementCalibration|GetRollRate)))
    (else
      (Pawn|Input|AddControllerRollInput (* (* (.Roll (Math|Rotator|BreakRotator (Transformation|GetActorRotation))) -1.0) (Variables|MovementCalibration|GetRollReturnRate))))))

(fn ConstructionScript
  (Utilities|FlowControl|Sequence
    (:then_0
      (bind _asbp_game_instance (Utilities|Casting|CastToBP_GameInstance (Game|GetGameInstance)))
      (Variables|Default|SetGameInstance _asbp_game_instance))
    (:then_1
      (bind _asbp_pawn_game_mode (Utilities|Casting|CastToBP_PawnGameMode (Game|GetGameMode)))
      (Variables|Default|SetGameMode _asbp_pawn_game_mode))
    (:then_2
      (CallFunction|SetupCustomShip))))

(fn SetupCustomShip
  (bind _gameinstance (Variables|Default|GetGameInstance))
  (bind _shipactor (Variables|Default|GetShipActor))
  (bind _shipinfo (Variables|/Game/Blueprints/AllLevels/BP_GameInstance.BP_GameInstance_C|GetShipInfo _gameinstance))
  (bind (_shipname _shipparts) (Utilities|Struct|BreakShipInfo _shipinfo))
  (ChildActorComponent|SetChildActorClass _shipactor "/Game/Blueprints/Ship/BP_CustomShip.BP_CustomShip_C")
  (bind _asbp_custom_ship (Utilities|Casting|CastToBP_CustomShip (Variables|/Script/Engine.ChildActorComponent|GetChildActor _shipactor)))
  (Variables|/Game/Blueprints/Ship/BP_CustomShip.BP_CustomShip_C|SetShipParts _asbp_custom_ship _shipparts)
  (Variables|/Game/Blueprints/Ship/BP_CustomShip.BP_CustomShip_C|SetShipName _asbp_custom_ship (Utilities|String|ToString(Text) _shipname))
  (Default|LoadShip _asbp_custom_ship)
  (Variables|Default|SetCustomShipRef _asbp_custom_ship))

(fn CalculateEngineThrust
  (bind _customshipref (Variables|Default|GetCustomShipRef))
  (bind _speedrate (Variables|MovementCalibration|GetSpeedRate))
  (bind _forwardinput (Variables|Movement|GetForwardInput))
  (bind _shipstats (Variables|/Game/Blueprints/Ship/BP_Ship.BP_Ship_C|GetShipStats _customshipref))
  (bind _speed (Variables|/Game/Blueprints/Ship/BP_ShipStats.BP_ShipStats_C|GetSpeed _shipstats))
  (bind _returnvalue (* _speed _speedrate _forwardinput))
  (if (== (Variables|Movement|GetForwardInput) 0.0)
    (Variables|Movement|SetEngineThrust (- (Variables|Movement|GetEngineThrust) _returnvalue))
    (if (or (< (Variables|Movement|GetEngineThrust) 0.1) (> (Variables|Movement|GetEngineThrust) -0.1))
      (Variables|Movement|SetEngineThrust 0.0))
    (else
      (Variables|Movement|SetEngineThrust (+ _returnvalue (Variables|Movement|GetEngineThrust))))))

(fn CalculateForwardSpeed
  (Variables|Movement|SetForwardSpeed (+ (Variables|Movement|GetForwardSpeed) (- (Variables|Movement|GetEngineThrust) (Variables|Movement|GetAirResistance)))))

(fn CalculateAirResistance
  (Variables|Movement|SetAirResistance (* (Variables|Movement|GetForwardSpeed) (Variables|MovementCalibration|GetAirResistanceRatio))))