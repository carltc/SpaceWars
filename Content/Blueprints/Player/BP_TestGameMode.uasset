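; Test game mode that assigns player starts and respawns players as basic ship pawns.
; ChoosePlayerStart claims an untagged start from a cached list, tags it full and stores it on the BP_PlayerController.
; RespawnPlayer destroys the current pawn, then spawns and possesses a new ship at that stored start.
; If no valid start is held, a new one spawns near the origin at random, though that branch returns nothing.
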(event Custom|RespawnPlayer
  (params (PlayerController :type BP%20Player%20Controller%20Object%20Reference))
  (bind _returnvalue (Pawn|GetControlledPawn PlayerController))
  (Utilities|IsValid _returnvalue
    (:Is%20Valid
      (Actor|DestroyActor _returnvalue))
    (:Is%20Not%20Valid
      _))
  (bind _returnvalue_2 (Game|SpawnActorfromClass "/Game/Blueprints/Ship/BP_Pawn_BasicShip.BP_Pawn_BasicShip_C" (Transformation|GetActorTransform (Variables|/Game/Blueprints/Player/BP_PlayerController.BP_PlayerController_C|GetPlayerStart PlayerController)) "Undefined" 0 0))
  (Pawn|Possess PlayerController _returnvalue_2))

(fn ConstructionScript)

(fn ChoosePlayerStart
  (params (Player :type Controller%20Object%20Reference))
  (bind _chosen_player_start (CallFunction|GetAPlayerStart))
  (bind _asbp_player_controller (Utilities|Casting|CastToBP_PlayerController Player))
  (bind _output_get (Variables|/Game/Blueprints/Player/BP_PlayerController.BP_PlayerController_C|SetPlayerStart _asbp_player_controller _chosen_player_start))
  (return _output_get))

(fn GetAPlayerStart
  (bind _returnvalue (Math|Random|RandomFloat))
  (bind _spawnfulltag (LocalVariables|GetSpawnFullTag))
  (bind _outactors (Actor|GetAllActorsOfClass "/Script/Engine.PlayerStart"))
  (if (> (Utilities|Array|Length (Variables|Default|GetPlayerStarts)) 0)
    _
    (else
      (Variables|Default|SetPlayerStarts _outactors)))
  (bind _array_element (Utilities|Array|ForEachLoopwithBreak (Variables|Default|GetPlayerStarts) :!label _label)
    (:LoopBody
      (if (not (Utilities|Name|Equal(Name) _spawnfulltag (Variables|/Script/Engine.PlayerStart|GetPlayerStartTag _array_element)))
        (LocalVariables|SetPlayerStart _array_element)
        (Variables|/Script/Engine.PlayerStart|SetPlayerStartTag _array_element _spawnfulltag)
        (goto _label Break)))
    (:Completed
      (Utilities|IsValid (LocalVariables|GetPlayerStart)
        (:Is%20Valid
          (return (LocalVariables|GetPlayerStart)))
        (:Is%20Not%20Valid
          (bind _returnvalue_2 (Game|SpawnActorfromClass "/Script/Engine.PlayerStart" (Math|Transform|MakeTransform (Math|Vector|MakeVector (* 500 _returnvalue) (* 500 _returnvalue) 0.0)) "Undefined" 0 0))
          (LocalVariables|SetPlayerStart _returnvalue_2))))))