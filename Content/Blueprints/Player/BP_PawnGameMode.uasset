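; Game mode that places players at random positions and handles respawning them.
; GetAPlayerStart spawns a new PlayerStart actor on each call, with random XY within a square, fixed height and random yaw.
; ChoosePlayerStart returns that start, and GM_Respawn destroys the controller's current pawn before restarting it at one.
; Older logic that picks an unoccupied placed PlayerStart by tag remains but is disconnected.
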(event Custom|GM_Respawn
  (params (Player%20Controller :type Player%20Controller%20Object%20Reference))
  (bind _returnvalue (Pawn|GetControlledPawn Player%20Controller))
  (Utilities|IsValid _returnvalue
    (:Is%20Valid
      (Actor|DestroyActor _returnvalue))
    (:Is%20Not%20Valid
      _))
  (bind _chosen_player_start (CallFunction|GetAPlayerStart))
  (Class|GameModeBase|RestartPlayeratPlayerStart Player%20Controller _chosen_player_start))

(event EventBeginPlay)

(event EventTick
  (params (DeltaSeconds :type Float%20%28single-precision%29)))

(fn ConstructionScript)

(fn ChoosePlayerStart
  (params (Player :type Controller%20Object%20Reference))
  (bind _chosen_player_start (CallFunction|GetAPlayerStart))
  (return _chosen_player_start))

(fn GetAPlayerStart
  (bind _returnvalue (Math|Random|RandomFloat))
  ;[1 1 1] RANDOM player start position
  (bind _returnvalue_2 (Game|SpawnActorfromClass "/Script/Engine.PlayerStart" (Math|Transform|MakeTransform (Math|Vector|MakeVector (* 2000 _returnvalue) (* 2000 _returnvalue) 5e+02) (Math|Rotator|MakeRotator 0.0 0.0 (* 360 (Math|Random|RandomFloat)))) "Undefined" 0 0))
  (LocalVariables|SetPlayerStart _returnvalue_2)
  (return (LocalVariables|GetPlayerStart)))