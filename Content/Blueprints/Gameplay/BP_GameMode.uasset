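; Game mode that overrides ChoosePlayerStart to hand out a separate PlayerStart to joining players.
; It fills a cached list of the level's PlayerStarts when empty, then takes the first not yet tagged as done and tags it as used.
; If no valid start is selected, it spawns a new PlayerStart at a random spot near the world origin and returns that.
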(event EventBeginPlay)

(event EventTick
  (params (DeltaSeconds :type Float%20%28single-precision%29)))

(fn ConstructionScript)

(fn ChoosePlayerStart
  (params (Player :type Controller%20Object%20Reference))
  (bind _returnvalue (Math|Random|RandomFloat))
  (bind _actordonetag (LocalVariables|GetActorDoneTag))
  (bind _outactors (Actor|GetAllActorsOfClass "/Script/Engine.PlayerStart"))
  (if (> (Utilities|Array|Length (Variables|Default|GetPlayerStarts)) 0)
    _
    (else
      (Variables|Default|SetPlayerStarts _outactors)))
  (bind _array_element (Utilities|Array|ForEachLoopwithBreak (Variables|Default|GetPlayerStarts) :!label _label)
    (:LoopBody
      (if (not (Utilities|Name|Equal(Name) _actordonetag (Variables|/Script/Engine.PlayerStart|GetPlayerStartTag _array_element)))
        (LocalVariables|SetSelectedPlayerStart _array_element)
        (Variables|/Script/Engine.PlayerStart|SetPlayerStartTag _array_element _actordonetag)
        (goto _label Break)))
    (:Completed
      (Utilities|IsValid (LocalVariables|GetSelectedPlayerStart)
        (:Is%20Valid
          _)
        (:Is%20Not%20Valid
          (bind _returnvalue_2 (Game|SpawnActorfromClass "/Script/Engine.PlayerStart" (Math|Transform|MakeTransform (Math|Vector|MakeVector (* 500 _returnvalue) (* 500 _returnvalue) 0.0)) "Undefined" 0 0))
          (LocalVariables|SetSelectedPlayerStart _returnvalue_2)))
      (return (LocalVariables|GetSelectedPlayerStart)))))