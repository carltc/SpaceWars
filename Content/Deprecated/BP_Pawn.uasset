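; BP_Pawn, kept in the Deprecated folder, is a pawn that gets its own ship in the game.
; On BeginPlay it calls a run-on-server event that spawns CurrentShipClass at the pawn's transform, stores it as CurrentShip and attaches the pawn to it.
; EndPlay destroys that ship, and Destroyed prints a death message with the pawn's name.
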(event Custom|Run%20on%20Server%20-%20Spawn%20Ship
  ;[1 1 1] Start of game
  (bind _returnvalue (Game|SpawnActorfromClass (Variables|Default|GetCurrentShipClass) (Transformation|GetActorTransform) "Undefined" 0 0))
  (bind _output_get (Variables|Default|SetCurrentShip _returnvalue))
  (Transformation|AttachActorToActor _output_get "None" "KeepWorld" "KeepWorld" "KeepWorld" false))

(event EventBeginPlay
  ;[1 1 1] Start of game
  (CallFunction|RunonServer-SpawnShip))

(event EventDestroyed
  ;[1 1 1] Destroyed
  (Development|PrintString (Utilities|String|Append "Died: " (Utilities|GetDisplayName self))))

(event EventEndPlay
  (params (EndPlayReason :type EEndPlayReason%20Enum :default "Destroyed"))
  ;[1 1 1] End of game
  (Actor|DestroyActor (Variables|Default|GetCurrentShip)))

(fn ConstructionScript)