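; Base pawn for a flyable multiplayer ship, kept in the Deprecated folder, covering movement, shooting and death.
; Tick moves it client-side from PlayerController speeds, with a FreeMovement drift mode; the server/multicast transform replication in MovePawn is disconnected.
; Shooting sends each ProjectileSource mesh socket to a server event that spawns BP_Projectile.
; Death records ship parts, removes enemies from match state and requests a GameMode respawn on authority.
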(event Custom|UnpossessPawn
  ;[1 1 1] Unpossess Pawn
  (bind _asbp_match_player_state (Utilities|Casting|CastToBP_MatchPlayerState (Variables|GetPlayerState))))

(event Custom|ShipDestroyed
  ;[1 1 1] Ship Destroyed
  (bind _asship_base (Utilities|Casting|CastToShip_Base (Variables|/Script/Engine.ChildActorComponent|GetChildActor (Variables|Default|GetShip))))
  (Utilities|FlowControl|Sequence
    (:then_0
      ;[1 1 1] ADD all parts to the destroyed parts list
      (for _array_element (Actor|GetComponentsByClass _asship_base "/Script/Engine.StaticMeshComponent")
        (bind _asstatic_mesh_component (Utilities|Casting|CastToStaticMeshComponent _array_element)
          (:then
            (Utilities|Array|Add (Variables|/Game/Models/Ship_Base.Ship_Base_C|GetDestroyedPartReferences _asship_base) _asstatic_mesh_component))
          (:CastFailed
            (Development|PrintString (Utilities|String|Append "Failed to cast Static Mesh Component: " (Utilities|GetDisplayName _asstatic_mesh_component)) true true "(R=0.000000,G=0.660000,B=1.000000,A=1.000000)" 2e+01)))))
    (:then_1
      ;[1 1 1] REMOVE this pawn from the Enemy Pawns
      (bind _asbp_match_game_state (Utilities|Casting|CastToBP_MatchGameState (Game|GetGameState))
        (:then
          (bind _asbp_pawn_enemy (Utilities|Casting|CastToBP_Pawn_Enemy self)
            (:then
              (Utilities|Array|RemoveItem (Variables|/Game/Blueprints/Match/BP_MatchGameState.BP_MatchGameState_C|GetEnemyPawns _asbp_match_game_state) _asbp_pawn_enemy))
            (:CastFailed
              (Development|PrintString "Failed to CAST to BP_Pawn_enemy" true true "(R=0.000000,G=0.660000,B=1.000000,A=1.000000)" 1e+01))))
        (:CastFailed
          (Development|PrintString "Failed to CAST to BP_GameState" true true "(R=0.000000,G=0.660000,B=1.000000,A=1.000000)" 1e+01))))
    (:then_2
      ;[1 1 1] DESTROY ship on Server
      (CallFunction|ShipDestroyedServer))))

(event Custom|Server_SetPawnMovement
  (params (DeltaRotation :type Rotator) (DeltaLocation :type Vector))
  ;[1 1 1] Cast movement to server
  (CallFunction|MulticastEvent DeltaRotation DeltaLocation))

(event Custom|MulticastEvent
  (params (DeltaRotation :type Rotator) (DeltaLocation :type Vector))
  ;[1 1 1] Multicast Actor Position
  (if (not (Variables|Default|GetIsDestroyed))
    (if (not (Pawn|IsLocallyControlled))
      (Transformation|SetActorLocationAndRotation DeltaLocation DeltaRotation true))))

(event Custom|Client_SetPawnMovement
  (params (DeltaSeconds :type Float%20%28single-precision%29))
  (bind _playercontroller (Variables|Default|GetPlayerController))
  ;[1 1 1] Client Pawn Movement
  (if (not (Variables|Default|GetIsDestroyed))
    (Utilities|IsValid _playercontroller
      (:Is%20Valid
        (CallFunction|MovePawn DeltaSeconds (Variables|/Game/Deprecated/Gameplay/BP_PlayerController_Base.BP_PlayerController_Base_C|GetRollSpeed _playercontroller) (Variables|/Game/Deprecated/Gameplay/BP_PlayerController_Base.BP_PlayerController_Base_C|GetPitchSpeed _playercontroller) (Variables|/Game/Deprecated/Gameplay/BP_PlayerController_Base.BP_PlayerController_Base_C|GetYawSpeed _playercontroller) (Variables|/Game/Deprecated/Gameplay/BP_PlayerController_Base.BP_PlayerController_Base_C|GetForwardSpeed _playercontroller))))))

(event Custom|Server_ProjectileShot
  (params (SpawnTransform :type Transform) (Impulse :type Vector))
  ;[1 1 1] Server Projectile Shot
  ;[1 1 1] Multicast Projectile Shot
  (Game|SpawnActorfromClass "/Game/Deprecated/BP_Projectile.BP_Projectile_C" SpawnTransform "AlwaysSpawn" (Variables|Default|GetPlayerController) self))

(event Custom|ShipDestructionSequence)

(event Custom|Multicast_ProjectileShot
  (params (Spawn%20Transform :type Transform))
  ;[1 1 1] Multicast Projectile Shot
  (Game|SpawnActorfromClass "/Game/Deprecated/BP_Projectile.BP_Projectile_C" (stale Custom|Server_ProjectileShot SpawnTransform) "AlwaysSpawn" (Variables|Default|GetPlayerController) self))

(event Custom|Shoot!
  (bind _ship (Variables|Default|GetShip))
  (bind _childactor (Variables|/Script/Engine.ChildActorComponent|GetChildActor _ship))
  ;[1 1 1] SHOOT
  (Utilities|IsValid _childactor
    (:Is%20Valid
      (for _array_element (Actor|GetComponentsbyTag _childactor "/Script/Engine.StaticMeshComponent" "ProjectileSource")
        (for _array_element_2 (Transformation|GetAllSocketNames _array_element)
          (CallFunction|ServerProjectileShot (Transformation|GetSocketTransform _array_element _array_element_2 "RTS_World") (* (Math|Vector|GetRightVector (.Rotation (Math|Transform|BreakTransform (Transformation|GetSocketTransform _array_element _array_element_2 "RTS_World")))) (* 0.0 -1.0))))))
    (:Is%20Not%20Valid
      (Development|PrintString "Current Ship not valid. Not shooting..."))))

(event Custom|ShipDestroyed_Server
  ;[1 1 1] BEGIN destruction event
  (bind _asbp_game_mode (Utilities|Casting|CastToBP_GameMode (Game|GetGameMode)))
  (Networking|SwitchHasAuthority
    (:Authority
      (Default|RespawnPlayer _asbp_game_mode self (Variables|Default|GetPlayerController)))))

(event EventBeginPlay
  ;[1 1 1] Start of game
  (Utilities|FlowControl|Sequence
    (:then_0
      (bind _asbp_game_instance (Utilities|Casting|CastToBP_GameInstance (Game|GetGameInstance)))
      (Variables|Default|SetGameInstance _asbp_game_instance))
    (:then_1
      (bind _asbp_player_controller_base (Utilities|Casting|CastToBP_PlayerController_Base (Game|GetPlayerController 0))
        (:then
          (Variables|Default|SetPlayerController _asbp_player_controller_base))
        (:CastFailed
          (Development|PrintString "BP_Pawn_Base: Startup cast to BP_PlayerController_Base failed." true true "(R=0.000000,G=0.660000,B=1.000000,A=1.000000)" 1e+01))))))

(event EventDestroyed
  ;[1 1 1] Destroyed
  (Development|PrintString (Utilities|String|Append "Died: " (Utilities|GetDisplayName self))))

(event EventTick
  (params (DeltaSeconds :type Float%20%28single-precision%29))
  ;[1 1 1] Tick
  (CallFunction|ClientSetPawnMovement DeltaSeconds))

(event EventEndPlay
  (params (EndPlayReason :type EEndPlayReason%20Enum :default "Destroyed"))
  ;[1 1 1] End of game
)

(fn ConstructionScript)

(fn MoveTowards
  (params (DesiredVector :type Vector) (CurrentVector :type Vector) (Difference :type Float%20%28single-precision%29))
  (bind (_x _y _z) (Math|Vector|BreakVector CurrentVector))
  (bind (_x_2 _y_2 _z_2) (Math|Vector|BreakVector DesiredVector))
  (return (Math|Vector|MakeVector (CallFunction|AddPartDifference _x_2 _x Difference) (CallFunction|AddPartDifference _y_2 _y Difference) (CallFunction|AddPartDifference _z_2 _z Difference))))

(fn AddPartDifference
  (params (Float1 :type Float%20%28single-precision%29) (Float2 :type Float%20%28single-precision%29) (Difference :type Float%20%28single-precision%29))
  (return (+ Float2 (* (- Float1 Float2) Difference))))

(fn MovePawn
  (params (DeltaSeconds :type Float%20%28single-precision%29) (Roll :type Float%20%28single-precision%29) (Pitch :type Float%20%28single-precision%29) (Yaw :type Float%20%28single-precision%29) (Forward%20Speed :type Float%20%28single-precision%29))
  ;[1 1 1] CHECK if any movement should be made
  (if (Math|Boolean|ORBoolean (!= Roll 0.0) (!= Pitch 0.0) (!= Yaw 0.0) (!= 0.0 Forward%20Speed))
    ;[1 1 1] ADD rotation
    (Transformation|AddActorLocalRotation (Math|Rotator|MakeRotator Roll Pitch Yaw) true false)
    ;[1 1 1] CHECK if free movement is ON
    (if (Variables|Default|GetFreeMovement?)
      _
      (else
        ;[1 1 1] SET forward vector
        (Variables|Default|SetLastActorForward (* (* (Math|Vector|GetForwardVector (.Rotation (Math|Transform|BreakTransform (Transformation|GetWorldTransform (Variables|Default|GetShip))))) Forward%20Speed) (* DeltaSeconds 5e+02)))))
    ;[1 1 1] SET actor location
    (Transformation|SetActorLocation (+ (Variables|Default|GetLastActorForward) (Transformation|GetActorLocation)) true false)))