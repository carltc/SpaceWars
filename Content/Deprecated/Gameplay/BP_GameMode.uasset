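; Deprecated game mode that assigns player starts and respawns players in a basic ship.
; ChoosePlayerStart claims an untagged start from a cached list by setting its tag to SpawnFullTag, or spawns one at a random location if none remain, then stores it on the player controller.
; RespawnPlayer flags the old pawn as destroyed, spawns a BP_Pawn_BasicShip at that stored start and possesses it.
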(event Custom|RespawnPlayer
  (params (DestroyedPawn :type BP%20Pawn%20Base%20Object%20Reference) (PlayerController :type BP%20Player%20Controller%20Base%20Object%20Reference))
  (Variables|/Game/Deprecated/BP_Pawn_Base.BP_Pawn_Base_C|SetIsDestroyed DestroyedPawn true)
  (bind _returnvalue (Game|SpawnActorfromClass "/Game/Deprecated/BP_Pawn_BasicShip.BP_Pawn_BasicShip_C" (Transformation|GetActorTransform (Variables|/Game/Deprecated/Gameplay/BP_PlayerController_Base.BP_PlayerController_Base_C|GetPlayerStart PlayerController)) "Undefined" 0 0))
  (bind _asbp_pawn_base (Utilities|Casting|CastToBP_Pawn_Base _returnvalue))
  (bind _asbp_player_controller_base (Utilities|Casting|CastToBP_PlayerController_Base PlayerController))
  (Pawn|Possess _asbp_player_controller_base _asbp_pawn_base))

(event EventBeginPlay)

(event EventTick
  (params (DeltaSeconds :type Float%20%28single-precision%29)))

(fn ConstructionScript)

(fn ChoosePlayerStart
  (params (Player :type Controller%20Object%20Reference))
  (bind _chosenplayerstart (CallFunction|GetAPlayerStart))
  (bind _asbp_player_controller_base (Utilities|Casting|CastToBP_PlayerController_Base Player))
  (Variables|/Game/Deprecated/Gameplay/BP_PlayerController_Base.BP_PlayerController_Base_C|SetPlayerStart _asbp_player_controller_base _chosenplayerstart)
  (return _chosenplayerstart))

(fn GetAPlayerStart
  (bind _returnvalue (Math|Random|RandomFloat))
  (bind _spawnfulltag (LocalVariables|GetSpawnFullTag))
  (bind _outactors (Actor|GetAllActorsOfClass "/Script/Engine.PlayerStart"))
  (if (> (Utilities|Array|Length (Variables|Default|GetPlayerStarts)) 0)
    _
    (else
      (Variables|Default|SetPlayerStarts _outactors)))
  (bind _array_element (Utilities|Array|ForEachLoopwithBreak (Variables|Default|GetPlayerStarts) :!label _label)
    (:LoopBody
      (if (not (Utilities|Name|Equal(Name) _spawnfulltag (Variables|/Script/Engine.PlayerStart|GetPlayerStartTag _array_element)))
        (LocalVariables|SetPlayerStart _array_element)
        (Variables|/Script/Engine.PlayerStart|SetPlayerStartTag _array_element _spawnfulltag)
        (goto _label Break)))
    (:Completed
      (Utilities|IsValid (LocalVariables|GetPlayerStart)
        (:Is%20Valid
          _)
        (:Is%20Not%20Valid
          (bind _returnvalue_2 (Game|SpawnActorfromClass "/Script/Engine.PlayerStart" (Math|Transform|MakeTransform (Math|Vector|MakeVector (* 500 _returnvalue) (* 500 _returnvalue) 0.0)) "Undefined" 0 0))
          (LocalVariables|SetPlayerStart _returnvalue_2)))
      (return (LocalVariables|GetPlayerStart)))))