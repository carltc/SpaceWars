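; Deprecated player character Blueprint that fires projectiles from the ship held in its Ship child actor component.
; Shoot finds the ship's static mesh components tagged ProjectileSource and treats every socket on them as a muzzle.
; Each socket's world transform goes to a server-named shot event, which spawns BP_Projectile_old with the character as owner and instigator.
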(event Custom|Shoot
  (bind _ship (Variables|Default|GetShip))
  (bind _childactor (Variables|/Script/Engine.ChildActorComponent|GetChildActor _ship))
  ;[1 1 1] SHOOT
  (Utilities|IsValid _childactor
    (:Is%20Valid
      (for _array_element (Actor|GetComponentsbyTag _childactor "/Script/Engine.StaticMeshComponent" "ProjectileSource")
        (for _array_element_2 (Transformation|GetAllSocketNames _array_element)
          (CallFunction|PlayerServerProjectileShot (Transformation|GetSocketTransform _array_element _array_element_2 "RTS_World")))))
    (:Is%20Not%20Valid
      (Development|PrintString "Current Ship not valid. Not shooting..."))))

(event Custom|Player_Server_ProjectileShot
  (params (Spawn%20Transform :type Transform))
  ;[1 1 1] SHOOT
  ;;[1 1 1] Server Projectile Shot
  (Game|SpawnActorfromClass "/Game/Deprecated/BP_Projectile_old.BP_Projectile_old_C" Spawn%20Transform "AlwaysSpawn" self self))

(fn ConstructionScript)