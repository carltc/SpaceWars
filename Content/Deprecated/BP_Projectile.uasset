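; Deprecated ship-weapon projectile that moves manually along its negative right vector, counts shots fired on the player controller, and expires after a maximum lifetime.
; Each tick, a server-only capsule trace sweeps from previous to next position, ignoring same-class projectiles and the instigator's ship.
; Hits spawn an explosion and destroy the projectile; ShipCore-tagged components destroy the ship, others are multicast into its destroyed-part list.
; Damage-threshold, scoring and relative-speed logic are disconnected.
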(event Custom|Multicast_ComponentDestroyed
  (params (Component :type Primitive%20Component%20Object%20Reference))
  ;[1 1 1] Multicast Destroyed Ship Part
  (bind _asship_base (Utilities|Casting|CastToShip_Base (Components|GetOwner Component))
    (:then
      (bind _asstatic_mesh_component (Utilities|Casting|CastToStaticMeshComponent Component))
      (Utilities|Array|Add (Variables|/Game/Models/Ship_Base.Ship_Base_C|GetDestroyedPartReferences _asship_base) _asstatic_mesh_component))
    (:CastFailed
      (Development|PrintString (Utilities|String|Append "Failed to cast to FbxScene_BasicShip: " (Utilities|GetDisplayName Component)) true true "(R=0.000000,G=0.660000,B=1.000000,A=1.000000)" 2e+01))))

(event EventBeginPlay
  (bind _returnvalue (Game|GetPlayerController 0))
  ;[1 1 1] Begin
  (Variables|Default|SetVelocity (* (Transformation|GetActorRightVector) (* (Utilities|GetRelativeProjectileSpeed) -1.0)))
  (Utilities|IsValid _returnvalue
    (:Is%20Valid
      (bind _asbp_player_controller_base (Utilities|Casting|CastToBP_PlayerController_Base _returnvalue))
      (Variables|/Game/Deprecated/Gameplay/BP_PlayerController_Base.BP_PlayerController_Base_C|SetShotsFired _asbp_player_controller_base (+ (Variables|/Game/Deprecated/Gameplay/BP_PlayerController_Base.BP_PlayerController_Base_C|GetShotsFired _asbp_player_controller_base) 1)))))

(event EventTick
  (params (DeltaSeconds :type Float%20%28single-precision%29))
  ;[1 1 1] MOVE Projectile
  ;;[1 1 1] SET previous location
  (Variables|Default|SetPreviousPosition (Transformation|GetActorLocation))
  ;;[1 1 1] SET new location
  (Variables|Default|SetNextPosition (+ (* (Variables|Default|GetVelocity) DeltaSeconds) (Transformation|GetActorLocation)))
  ;;[1 1 1] DETECT hit (and destroy projectile on hit)
  (bind _hit (CallFunction|DetectHit))
  (if _hit
    (Actor|DestroyActor)
    (else
      ;;[1 1 1] MOVE Projectile
      (Transformation|SetActorLocation (Variables|Default|GetNextPosition) false false)
      ;;[1 1 1] DESTROY actor if it has lived longer than allowed
      (bind _output_get (Variables|Default|SetLifetimeSeconds (+ (Variables|Default|GetLifetimeSeconds) DeltaSeconds)))
      (if (> _output_get (Variables|Default|GetMaxLifetimeSeconds))
        (Actor|DestroyActor)))))

(fn ConstructionScript)

(fn DetectHit
  (bind _capsule (Variables|Default|GetCapsule))
  (bind (_outradius _outhalfheight) (Components|Capsule|GetScaledCapsuleSize _capsule))
  ;[1 1 1] ONLY execute on server
  (Networking|SwitchHasAuthority
    (:Authority
      ;[1 1 1] CHECK for hit
      (bind (_outhit _returnvalue) (Collision|CapsuleTraceByChannel (Variables|Default|GetPreviousPosition) (Variables|Default|GetNextPosition) _outradius _outhalfheight "TraceTypeQuery1" false 0 "None"))
      (if _returnvalue
        ;[1 1 1] CHECK if valid hit
        (if (and (!= (Utilities|GetClass self) (Utilities|GetClass (.HitActor (Collision|BreakHitResult _outhit)))) (!= (Actor|GetParentActor (.HitActor (Collision|BreakHitResult _outhit))) (Game|GetInstigator)))
          ;[1 1 1] CHECK if hit damage breached threshold
          (Effects|SpawnEmitterAttached "/Game/ParticleSystems/PS_Explosion.PS_Explosion" (.HitComponent (Collision|BreakHitResult _outhit)) "None" "0, 0, 0" (Math|Conversions|RotationFromXVector (.ImpactNormal (Collision|BreakHitResult _outhit))))
          (if true
            ;[1 1 1] SET hit state
            (LocalVariables|SetWasHit true)
            ;[1 1 1] CHECK if core was hit
            (if (Components|ComponentHasTag (.HitComponent (Collision|BreakHitResult _outhit)) "ShipCore")
              ;[1 1 1] SHIP was destroyed
              (Development|PrintString "Ship Destroyed" true true "(R=0.000000,G=0.660000,B=1.000000,A=1.000000)" 2e+01)
              (bind _asship_base (Utilities|Casting|CastToShip_Base (Components|GetOwner (.HitComponent (Collision|BreakHitResult _outhit))))
                (:then
                  (Development|PrintString (Utilities|String|Append "Owner of hit components: " (Utilities|GetDisplayName _asship_base)) true true "(R=0.000000,G=0.660000,B=1.000000,A=1.000000)" 2e+01)
                  (Default|ShipDestroyed _asship_base)
                  (Development|PrintString (Utilities|String|Append "Actor Destroy: " (Utilities|GetObjectName _asship_base)) true true "(R=0.000000,G=0.660000,B=1.000000,A=1.000000)" 2e+01))
                (:CastFailed
                  _))
              (else
                ;[1 1 1] PART was destroyed
                (CallFunction|MulticastComponentDestroyed (.HitComponent (Collision|BreakHitResult _outhit)))))
            (else
              (LocalVariables|SetWasHit true)))
          (else
            (LocalVariables|SetWasHit false :!label _label)))
        (else
          (goto _label))))
    (:Remote
      (goto _label)))
  (return (LocalVariables|GetWasHit)))